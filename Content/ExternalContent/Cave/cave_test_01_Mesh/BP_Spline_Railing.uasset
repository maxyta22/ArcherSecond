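; Spline-driven railing Blueprint that builds a run of deformed mesh sections along a spline in the construction script.
; It divides the spline by a section length derived from the actor's Z scale and adds a collidable, Z-forward spline mesh component per section.
; Each section takes its endpoints from the spline, with tangents clamped to the section length.
; An alternative instanced static mesh placement using bounds-based spacing is present but never runs.
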(event EventBeginPlay)

(event Collision|EventActorBeginOverlap
  (params (OtherActor :type Actor%20Object%20Reference)))

(event EventTick
  (params (DeltaSeconds :type Float%20%28single-precision%29)))

(fn ConstructionScript
  (bind _spline (Variables|Default|GetSpline))
  (bind _spline_2 (Variables|Default|GetSpline))
  (Variables|Default|SetSection_Lengt (* (.z (Transformation|GetActorScale3D)) 209.0))
  (for _index (range 0 (Math|Float|Truncate (/ (Spline|GetSplineLength (Variables|Default|GetSpline)) (Variables|Default|GetSection_Lengt))))
    (bind _returnvalue (AddComponent|AddSplineMeshComponent false))
    (SplineMesh|SetForwardAxis _returnvalue "Z" true)
    (Collision|SetCollisionEnabled _returnvalue "QueryAndPhysics")
    (SplineMesh|SetStartandEnd _returnvalue (Spline|GetLocationatDistanceAlongSpline _spline_2 (* (Variables|Default|GetSection_Lengt) _index) "Local") (Math|Vector|ClampVectorSize (Spline|GetTangentatDistanceAlongSpline _spline_2 (* (Variables|Default|GetSection_Lengt) _index) "Local") 0.0 (Variables|Default|GetSection_Lengt)) (Spline|GetLocationatDistanceAlongSpline _spline (* (Variables|Default|GetSection_Lengt) (+ _index 1)) "Local") (Math|Vector|ClampVectorSize (Spline|GetTangentatDistanceAlongSpline _spline (* (Variables|Default|GetSection_Lengt) (+ _index 1)) "Local") 0.0 (Variables|Default|GetSection_Lengt)) true :!class /Script/Engine.SplineMeshComponent)))

(fn GetLocationIndex
  (params (A :type Integer))
  (return (Spline|GetLocationatDistanceAlongSpline (Variables|Default|GetSpline) (* A (Variables|Default|GetSpacing)) "Local")))