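; Boss launch platform actor that launches the player character on contact while it is active.
; Activate and deactivate events set a CanLaunch flag and switch the Niagara effect, audio and point light on or off to match.
; When something overlaps the box while the flag is set, it casts to PlayerCharacter_BP and calls LaunchPlatform, leaving the launch itself to the character.
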(event OnComponentBeginOverlap(Box)
  (params (OverlappedComponent :type Primitive%20Component%20Object%20Reference) (OtherActor :type Actor%20Object%20Reference) (OtherComp :type Primitive%20Component%20Object%20Reference) (OtherBodyIndex :type Integer) (bFromSweep :type Boolean) (SweepResult :type Hit%20Result%20Structure%20%28by%20ref%29))
  (if (Variables|Default|Getcan_launch)
    (bind _asplayer_character_bp (Utilities|Casting|CastToPlayerCharacter_BP OtherActor))
    (Default|LaunchPlatform _asplayer_character_bp)))

(event Custom|Activate_Boss_Launch
  (Variables|Default|Setcan_launch true)
  (Components|Activation|Activate (Variables|Default|GetNiagara) false)
  (Audio|Components|Audio|Play (Variables|Default|GetAudio) 0.0)
  (Rendering|Components|Light|SetIntensity (Variables|Default|GetPointLight) 5e+03))

(event Custom|Deactivate_Boss_Launch
  (Variables|Default|Setcan_launch false)
  (Components|Activation|Deactivate (Variables|Default|GetNiagara))
  (Audio|Components|Audio|Stop (Variables|Default|GetAudio))
  (Rendering|Components|Light|SetIntensity (Variables|Default|GetPointLight) 0.0))

(event EventBeginPlay
  (Audio|Components|Audio|Stop (Variables|Default|GetAudio)))

(event Collision|EventActorBeginOverlap
  (params (OtherActor :type Actor%20Object%20Reference)))

(event EventTick
  (params (DeltaSeconds :type Float%20%28single-precision%29)))

(fn ConstructionScript)