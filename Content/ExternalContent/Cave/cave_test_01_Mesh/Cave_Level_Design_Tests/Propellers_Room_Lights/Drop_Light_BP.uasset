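; Drop_Light_BP is a lighting Blueprint for the propellers room in a cave level test that switches on a group of lights.
; Its Lights_on event waits a few seconds, then raises the intensity of both propeller lights and the first white light together.
; Two more white lights follow one after another with short delays, giving a staggered power-up.
; Nothing in this Blueprint calls the event or turns the lights off.
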(event Custom|Lights_on
  (Utilities|FlowControl|Delay 3.0)
  (Utilities|FlowControl|Sequence
    (:then_0
      (Rendering|Components|Light|SetIntensity (Variables|Default|GetPropeller_Light_02) 5e+03)
      (Rendering|Components|Light|SetIntensity (Variables|Default|GetPropeller_Light_01) 5e+03)
      (Rendering|Components|Light|SetIntensity (Variables|Default|GetWhite_Light_03) 3e+03)
      (Utilities|FlowControl|Delay 0.2)
      (Rendering|Components|Light|SetIntensity (Variables|Default|GetWhite_Light_04) 3e+03)
      (Utilities|FlowControl|Delay 0.2)
      (Rendering|Components|Light|SetIntensity (Variables|Default|GetWhite_Light_05) 3e+03))))

(event EventBeginPlay)

(event Collision|EventActorBeginOverlap
  (params (OtherActor :type Actor%20Object%20Reference)))

(event EventTick
  (params (DeltaSeconds :type Float%20%28single-precision%29)))

(fn ConstructionScript)