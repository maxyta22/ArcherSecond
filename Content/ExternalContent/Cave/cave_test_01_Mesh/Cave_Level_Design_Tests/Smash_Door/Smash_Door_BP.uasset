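; Smashable bunker door that breaks open when it receives a charged glove hit; uncharged hits and shots have no effect here.
; A charged hit hides the static mesh and reveals a skeletal crash mesh, then a DoOnce plays its crash montage and smash sound a single time.
; Damaged-stage and material flip-flop logic is left disconnected and never runs.
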(event EventAfterShotHit
  (params (HitResult :type Hit%20Result%20Structure%20%28by%20ref%29) (Causer :type Actor%20Object%20Reference)))

(event EventBeginPlay)

(event EventAfterGloveHit
  (params (Charged :type Boolean) (HitResult :type Hit%20Result%20Structure%20%28by%20ref%29) (Causer :type Actor%20Object%20Reference))
  (if Charged
    (Rendering|SetVisibility (Variables|Default|GetStaticMeshComponent) false false)
    (Rendering|SetVisibility (Variables|Default|GetBunker_door_crash_Anim) true false)
    (Utilities|FlowControl|DoOnce false
      (:Completed
        (Animation|Montage|PlayMontage (Variables|Default|GetBunker_door_crash_Anim) "/Game/ExternalContent/Cave/cave_test_01_Mesh/Cave_Level_Design_Tests/Smash_Door/Bunker_door_crash_Anim_Anim_Montage.Bunker_door_crash_Anim_Anim_Montage"
          (:then
            (Audio|Components|Audio|Play (Variables|Default|GetDoor_Smash_Cue) 0.0)))))))

(fn ConstructionScript
  (|CallParentFunction))