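; AI character Blueprint for the Walking House enemy, adding combat reactions through server-played lizard montages on its CustomAction component.
; Being aimed at triggers a random left or right side dodge.
; After a hit reaction, it plays a forward charge if the AI controller's enemy is at or beyond a minimum distance.
; Tick runs a downward visibility trace from high above the mesh with persistent debug drawing, leaving the result unused.
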(event EventAfterReactiontoAiming
  (Class|CustomAction|TryPerformPlayAnimMontageServer (Variables|Default|GetCustomAction) (select (Math|Random|RandomBool) "/Game/ExternalContent/Lizard/Lizard_Side_Right_Dodge_AM.Lizard_Side_Right_Dodge_AM" "/Game/ExternalContent/Lizard/Lizard_Side_Left_Dodge_AM.Lizard_Side_Left_Dodge_AM") false))

(event EventAfterCustomAction
  (bind _returnvalue (Pawn|GetController))
  (bind _asaicontroller_bp (Utilities|Casting|CastToAIController_BP _returnvalue))
  (bind _returnvalue_2 (Class|PRTAIController|GetEnemy _asaicontroller_bp))
  (Utilities|IsValid _asaicontroller_bp
    (:Is%20Valid
      (Utilities|IsValid _returnvalue_2
        (:Is%20Valid
          (if (>= (Transformation|GetDistanceTo _returnvalue_2) (Variables|Default|GetMinDistanceForAttackAfterHitReaction))
            (if (== (Class|CustomAction|GetLastAnimMontage (Variables|Default|GetCustomAction)) (Variables|Default|GetHitReaction))
              (Class|CustomAction|TryPerformPlayAnimMontageServer (Variables|Default|GetCustomAction) (select (Math|Random|RandomBool) "/Game/ExternalContent/Lizard/Lizard_charge_forward_ONSPOT_AM.Lizard_charge_forward_ONSPOT_AM" "/Game/ExternalContent/Lizard/Lizard_charge_forward_ONSPOT_AM.Lizard_charge_forward_ONSPOT_AM") false))))))))

(event EventTick
  (params (DeltaSeconds :type Float%20%28single-precision%29))
  (bind _mesh (Variables|Character|GetMesh))
  (bind _returnvalue (Transformation|GetSocketLocation _mesh "None"))
  (bind _returnvalue_2 (Transformation|GetWorldLocation _mesh))
  (bind (_x _y) (Math|Vector|BreakVector _returnvalue))
  (bind _returnvalue_3 (+ _returnvalue_2 "0, 0,3700.000000"))
  (bind _z (Math|Vector|BreakVector _returnvalue_3))
  (bind _returnvalue_4 (Math|Vector|MakeVector _x _y _z))
  (Collision|LineTraceByChannel _returnvalue_4 (- _returnvalue_4 "0, 0,3700.000000") "TraceTypeQuery1" false 0 "Persistent"))

(fn ConstructionScript
  (|CallParentFunction))