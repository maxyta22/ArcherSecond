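; Test Blueprint of a walking house that the player operates from trigger zones aboard it.
; An E-toggled oven gates forward movement, with alternating step timelines counting steps until a maximum shuts it off.
; Overlaps enable walking, rotation and strafing, with timeline-driven mesh leaning, while per-tick traces supply foot IK offsets.
; BeginPlay attaches "Floor"-tagged static meshes to the house and makes its wood and grass pickups infinite.
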(event OnComponentBeginOverlap(Tower_Moving_Forward_Collision)
  (params (OverlappedComponent :type Primitive%20Component%20Object%20Reference) (OtherActor :type Actor%20Object%20Reference) (OtherComp :type Primitive%20Component%20Object%20Reference) (OtherBodyIndex :type Integer) (bFromSweep :type Boolean) (SweepResult :type Hit%20Result%20Structure%20%28by%20ref%29)))

(event OnComponentBeginOverlap(Left_Right_Move)
  (params (OverlappedComponent :type Primitive%20Component%20Object%20Reference) (OtherActor :type Actor%20Object%20Reference) (OtherComp :type Primitive%20Component%20Object%20Reference) (OtherBodyIndex :type Integer) (bFromSweep :type Boolean) (SweepResult :type Hit%20Result%20Structure%20%28by%20ref%29))
  (bind _returnvalue (Actor|GetActorOfClass "/Game/Blueprint/Player/PlayerCharacter_BP.PlayerCharacter_BP_C"))
  (if (== _returnvalue OtherActor)
    (Variables|Default|SetHouse_Can_move true)))

(event OnComponentEndOverlap(Oven_Collision)
  (params (OverlappedComponent :type Primitive%20Component%20Object%20Reference) (OtherActor :type Actor%20Object%20Reference) (OtherComp :type Primitive%20Component%20Object%20Reference) (OtherBodyIndex :type Integer))
  (bind _returnvalue (Actor|GetActorOfClass "/Game/Blueprint/Player/PlayerCharacter_BP.PlayerCharacter_BP_C"))
  (if (== _returnvalue OtherActor)
    (Variables|Default|SetPlayer_In_Oven false)))

(event OnComponentBeginOverlap(Turn_Left_END_Collision)
  (params (OverlappedComponent :type Primitive%20Component%20Object%20Reference) (OtherActor :type Actor%20Object%20Reference) (OtherComp :type Primitive%20Component%20Object%20Reference) (OtherBodyIndex :type Integer) (bFromSweep :type Boolean) (SweepResult :type Hit%20Result%20Structure%20%28by%20ref%29))
  (bind _mesh (Variables|Character|GetMesh))
  (bind _mesh_2 (Variables|Character|GetMesh))
  ;[1 1 1] LEAN LEFT RIGHT
  (bind _returnvalue (Actor|GetActorOfClass "/Game/Blueprint/Player/PlayerCharacter_BP.PlayerCharacter_BP_C"))
  (if (== _returnvalue OtherActor)
    (Variables|Default|SetCapsule_Left_Strafe false)
    (Utilities|FlowControl|Sequence
      (:then_0
        (Variables|Default|SetRelative%20Rotation (Variables|/Script/Engine.SceneComponent|GetRelativeRotation _mesh_2))
        (bind _newtrack_0 (Timeline|Timeline_3 PlayFromStart)
          (:Update
            (Transformation|SetRelativeRotation _mesh_2 (Math|Rotator|Lerp(Rotator) (Math|Rotator|MakeRotator (.roll (Variables|Default|GetRelative%20Rotation)) (.pitch (Variables|Default|GetRelative%20Rotation)) (.yaw (Variables|Default|GetRelative%20Rotation))) (Math|Rotator|MakeRotator 0.0 0.0 0.0) _newtrack_0) false false))
          (:Finished
            (Utilities|FlowControl|DoOnce false) ; enters at Reset
          )))
      (:then_1
        (bind _newtrack_0_2 (Timeline|Timeline_2 Stop)
          (:Update
            (Transformation|SetRelativeRotation _mesh (Math|Rotator|Lerp(Rotator) (Math|Rotator|MakeRotator (.roll (Variables|Default|GetRelative%20Rotation)) (.pitch (Variables|Default|GetRelative%20Rotation)) (.yaw (Variables|Default|GetRelative%20Rotation))) (Math|Rotator|MakeRotator (+ (.roll (Variables|Default|GetRelative%20Rotation)) -1e+01) (.pitch (Variables|Default|GetRelative%20Rotation)) (.yaw (Variables|Default|GetRelative%20Rotation))) _newtrack_0_2) false false)))))))

(event OnComponentBeginOverlap(Turn_Right_END_Collision)
  (params (OverlappedComponent :type Primitive%20Component%20Object%20Reference) (OtherActor :type Actor%20Object%20Reference) (OtherComp :type Primitive%20Component%20Object%20Reference) (OtherBodyIndex :type Integer) (bFromSweep :type Boolean) (SweepResult :type Hit%20Result%20Structure%20%28by%20ref%29))
  (bind _mesh (Variables|Character|GetMesh))
  (bind _mesh_2 (Variables|Character|GetMesh))
  ;[1 1 1] LEAN LEFT RIGHT
  (bind _returnvalue (Actor|GetActorOfClass "/Game/Blueprint/Player/PlayerCharacter_BP.PlayerCharacter_BP_C"))
  (if (== _returnvalue OtherActor)
    (Variables|Default|SetCapsule_Right_Strafe false)
    (Utilities|FlowControl|Sequence
      (:then_0
        (Variables|Default|SetRelative%20Rotation (Variables|/Script/Engine.SceneComponent|GetRelativeRotation _mesh))
        (bind _newtrack_0 (Timeline|Timeline_5 PlayFromStart)
          (:Update
            (Transformation|SetRelativeRotation _mesh (Math|Rotator|Lerp(Rotator) (Math|Rotator|MakeRotator (.roll (Variables|Default|GetRelative%20Rotation)) (.pitch (Variables|Default|GetRelative%20Rotation)) (.yaw (Variables|Default|GetRelative%20Rotation))) (Math|Rotator|MakeRotator 0.0 0.0 0.0) _newtrack_0) false false))
          (:Finished
            (Utilities|FlowControl|DoOnce false) ; enters at Reset
          )))
      (:then_1
        (bind _newtrack_0_2 (Timeline|Timeline_4 Stop)
          (:Update
            (Transformation|SetRelativeRotation _mesh_2 (Math|Rotator|Lerp(Rotator) (Math|Rotator|MakeRotator (.roll (Variables|Default|GetRelative%20Rotation)) (.pitch (Variables|Default|GetRelative%20Rotation)) (.yaw (Variables|Default|GetRelative%20Rotation))) (Math|Rotator|MakeRotator (+ (.roll (Variables|Default|GetRelative%20Rotation)) 1e+01) (.pitch (Variables|Default|GetRelative%20Rotation)) (.yaw (Variables|Default|GetRelative%20Rotation))) _newtrack_0_2) false false)))))))

(event OnComponentBeginOverlap(Left_Right_Rotate)
  (params (OverlappedComponent :type Primitive%20Component%20Object%20Reference) (OtherActor :type Actor%20Object%20Reference) (OtherComp :type Primitive%20Component%20Object%20Reference) (OtherBodyIndex :type Integer) (bFromSweep :type Boolean) (SweepResult :type Hit%20Result%20Structure%20%28by%20ref%29))
  ;[1 1 1] ROTATION LEFT RIGHT
  (bind _returnvalue (Actor|GetActorOfClass "/Game/Blueprint/Player/PlayerCharacter_BP.PlayerCharacter_BP_C"))
  (if (== _returnvalue OtherActor)
    (Variables|Default|SetMain_Capsule_Can_Rotate true)))

(event OnComponentEndOverlap(Left_Right_Rotate)
  (params (OverlappedComponent :type Primitive%20Component%20Object%20Reference) (OtherActor :type Actor%20Object%20Reference) (OtherComp :type Primitive%20Component%20Object%20Reference) (OtherBodyIndex :type Integer))
  ;[1 1 1] ROTATION LEFT RIGHT
  (bind _returnvalue (Actor|GetActorOfClass "/Game/Blueprint/Player/PlayerCharacter_BP.PlayerCharacter_BP_C"))
  (if (== _returnvalue OtherActor)
    (Variables|Default|SetMain_Capsule_Can_Rotate false)))

(event OnComponentHit(SphereLeft)
  (params (HitComponent :type Primitive%20Component%20Object%20Reference) (OtherActor :type Actor%20Object%20Reference) (OtherComp :type Primitive%20Component%20Object%20Reference) (NormalImpulse :type Vector :default "0, 0, 0") (Hit :type Hit%20Result%20Structure%20%28by%20ref%29))
  (Rendering|Material|SetMaterial (Variables|Character|GetMesh) 2 "/Game/Characters/Walking_House/House_Mat.House_Mat"))

(event OnComponentHit(SphereRight)
  (params (HitComponent :type Primitive%20Component%20Object%20Reference) (OtherActor :type Actor%20Object%20Reference) (OtherComp :type Primitive%20Component%20Object%20Reference) (NormalImpulse :type Vector :default "0, 0, 0") (Hit :type Hit%20Result%20Structure%20%28by%20ref%29))
  (Rendering|Material|SetMaterial (Variables|Character|GetMesh) 1 0))

(event OnComponentEndOverlap(Left_Right_Move)
  (params (OverlappedComponent :type Primitive%20Component%20Object%20Reference) (OtherActor :type Actor%20Object%20Reference) (OtherComp :type Primitive%20Component%20Object%20Reference) (OtherBodyIndex :type Integer))
  (bind _returnvalue (Actor|GetActorOfClass "/Game/Blueprint/Player/PlayerCharacter_BP.PlayerCharacter_BP_C"))
  (if (== _returnvalue OtherActor)
    (if (not (>= (Variables|Default|GetSteps_number) (Variables|Default|GetMininum_Steps_Before_Walk)))
      (Variables|Default|SetHouse_Can_move false))))

(event OnComponentBeginOverlap(Turn_Left_Collision)
  (params (OverlappedComponent :type Primitive%20Component%20Object%20Reference) (OtherActor :type Actor%20Object%20Reference) (OtherComp :type Primitive%20Component%20Object%20Reference) (OtherBodyIndex :type Integer) (bFromSweep :type Boolean) (SweepResult :type Hit%20Result%20Structure%20%28by%20ref%29))
  (bind _mesh (Variables|Character|GetMesh))
  ;[1 1 1] LEAN LEFT RIGHT
  (bind _returnvalue (Actor|GetActorOfClass "/Game/Blueprint/Player/PlayerCharacter_BP.PlayerCharacter_BP_C"))
  (if (== _returnvalue OtherActor)
    (Variables|Default|SetCapsule_Left_Strafe true)
    (Utilities|FlowControl|DoOnce false :!label _label
      (:Completed
        (Utilities|FlowControl|Sequence
          (:then_0
            (bind _newtrack_0 (Timeline|Timeline_3 Stop)
              (:Update
                (Transformation|SetRelativeRotation (Variables|Character|GetMesh) (Math|Rotator|Lerp(Rotator) (Math|Rotator|MakeRotator (.roll (Variables|Default|GetRelative%20Rotation)) (.pitch (Variables|Default|GetRelative%20Rotation)) (.yaw (Variables|Default|GetRelative%20Rotation))) (Math|Rotator|MakeRotator 0.0 0.0 0.0) _newtrack_0) false false))
              (:Finished
                (goto _label Reset))))
          (:then_1
            (Variables|Default|SetRelative%20Rotation (Variables|/Script/Engine.SceneComponent|GetRelativeRotation _mesh))
            (bind _newtrack_0_2 (Timeline|Timeline_2 PlayFromStart)
              (:Update
                (Transformation|SetRelativeRotation _mesh (Math|Rotator|Lerp(Rotator) (Math|Rotator|MakeRotator (.roll (Variables|Default|GetRelative%20Rotation)) (.pitch (Variables|Default|GetRelative%20Rotation)) (.yaw (Variables|Default|GetRelative%20Rotation))) (Math|Rotator|MakeRotator (+ (.roll (Variables|Default|GetRelative%20Rotation)) -1e+01) (.pitch (Variables|Default|GetRelative%20Rotation)) (.yaw (Variables|Default|GetRelative%20Rotation))) _newtrack_0_2) false false)))))))))

(event OnComponentBeginOverlap(Oven_Collision)
  (params (OverlappedComponent :type Primitive%20Component%20Object%20Reference) (OtherActor :type Actor%20Object%20Reference) (OtherComp :type Primitive%20Component%20Object%20Reference) (OtherBodyIndex :type Integer) (bFromSweep :type Boolean) (SweepResult :type Hit%20Result%20Structure%20%28by%20ref%29))
  (bind _returnvalue (Actor|GetActorOfClass "/Game/Blueprint/Player/PlayerCharacter_BP.PlayerCharacter_BP_C"))
  (if (== _returnvalue OtherActor)
    (Variables|Default|SetPlayer_In_Oven true)))

(event OnComponentBeginOverlap(Turn_Right_Collision)
  (params (OverlappedComponent :type Primitive%20Component%20Object%20Reference) (OtherActor :type Actor%20Object%20Reference) (OtherComp :type Primitive%20Component%20Object%20Reference) (OtherBodyIndex :type Integer) (bFromSweep :type Boolean) (SweepResult :type Hit%20Result%20Structure%20%28by%20ref%29))
  (bind _mesh (Variables|Character|GetMesh))
  ;[1 1 1] LEAN LEFT RIGHT
  (bind _returnvalue (Actor|GetActorOfClass "/Game/Blueprint/Player/PlayerCharacter_BP.PlayerCharacter_BP_C"))
  (if (== _returnvalue OtherActor)
    (Variables|Default|SetCapsule_Right_Strafe true)
    (Utilities|FlowControl|DoOnce false :!label _label
      (:Completed
        (Utilities|FlowControl|Sequence
          (:then_0
            (bind _newtrack_0 (Timeline|Timeline_5 Stop)
              (:Update
                (Transformation|SetRelativeRotation (Variables|Character|GetMesh) (Math|Rotator|Lerp(Rotator) (Math|Rotator|MakeRotator (.roll (Variables|Default|GetRelative%20Rotation)) (.pitch (Variables|Default|GetRelative%20Rotation)) (.yaw (Variables|Default|GetRelative%20Rotation))) (Math|Rotator|MakeRotator 0.0 0.0 0.0) _newtrack_0) false false))
              (:Finished
                (goto _label Reset))))
          (:then_1
            (Variables|Default|SetRelative%20Rotation (Variables|/Script/Engine.SceneComponent|GetRelativeRotation _mesh))
            (bind _newtrack_0_2 (Timeline|Timeline_4 PlayFromStart)
              (:Update
                (Transformation|SetRelativeRotation _mesh (Math|Rotator|Lerp(Rotator) (Math|Rotator|MakeRotator (.roll (Variables|Default|GetRelative%20Rotation)) (.pitch (Variables|Default|GetRelative%20Rotation)) (.yaw (Variables|Default|GetRelative%20Rotation))) (Math|Rotator|MakeRotator (+ (.roll (Variables|Default|GetRelative%20Rotation)) 1e+01) (.pitch (Variables|Default|GetRelative%20Rotation)) (.yaw (Variables|Default|GetRelative%20Rotation))) _newtrack_0_2) false false)))))))))

(event Custom|Step_Left
  (bind _arrow_direction_left (Variables|Default|GetArrow_Direction_Left))
  (if (Variables|Default|GetHouse_Can_move)
    (if (Variables|Default|GetRight_Step_Finished)
      (Variables|Default|SetRight_Step_Finished false)
      (Variables|Default|SetHouse_Moving true)
      (Variables|Default|SetSteps_number (+ (Variables|Default|GetSteps_number) 1))
      (if (not (Variables|Default|GetLeft_Right_Step))
        (Variables|Default|SetLeft_Right_Step true)
        (Timeline|Timeline_0 PlayFromStart
          (:Update
            (Rendering|Material|SetScalarParameterValueonMaterials _arrow_direction_left "Color_Lerp" 1.0))
          (:Finished
            (Variables|Default|SetHouse_Moving false)
            (Variables|Default|SetLeft_Step_Finished true)
            (Rendering|Material|SetScalarParameterValueonMaterials _arrow_direction_left "Color_Lerp" 0.0)
            (CallFunction|RepeatSteps)))))))

(event Custom|Cam_Shake_R
  (Camera|PlayWorldCameraShake "/Game/Characters/Walking_House/Walking_House_Walking_Shake.Walking_House_Walking_Shake_C" (Transformation|GetSocketLocation (Variables|Character|GetMesh) "right_foot1_jntSocket") 0.0 1e+03))

(event Custom|Strafing_Left
  (bind _capsulecomponent (Variables|Collision|GetCapsuleComponent))
  (bind _returnvalue (Transformation|GetWorldLocation _capsulecomponent))
  ;[1 1 1] STRAFE
  (if (Variables|Default|GetCapsule_Left_Strafe)
    (Variables|Default|SetWorld_Loc_Walking_House _returnvalue)
    (Transformation|SetWorldLocation _capsulecomponent (+ _returnvalue (* (Math|Vector|GetRightVector _capsulecomponent) -15.0)) false false)))

(event Custom|Strafing_Right
  (bind _capsulecomponent (Variables|Collision|GetCapsuleComponent))
  (bind _returnvalue (Transformation|GetWorldLocation _capsulecomponent))
  ;[1 1 1] STRAFE
  (if (Variables|Default|GetCapsule_Right_Strafe)
    (Variables|Default|SetWorld_Loc_Walking_House _returnvalue)
    (Transformation|SetWorldLocation _capsulecomponent (+ _returnvalue (* (Math|Vector|GetRightVector _capsulecomponent) 15.0)) false false)))

(event Custom|Steps_Moves
  ;[1 0 0] Timeline_Walk
)

(event Custom|Right_Mouse_Released
  (bind _mesh (Variables|Character|GetMesh))
  (bind _mesh_2 (Variables|Character|GetMesh))
  ;[1 1 1] LEAN LEFT RIGHT
  (if (Variables|Default|GetMain_Capsule_Can_Rotate)
    (Utilities|FlowControl|Sequence
      (:then_0
        (Variables|Default|SetRelative%20Rotation (Variables|/Script/Engine.SceneComponent|GetRelativeRotation _mesh))
        (bind _newtrack_0 (Timeline|Timeline_5 PlayFromStart)
          (:Update
            (Transformation|SetRelativeRotation _mesh (Math|Rotator|Lerp(Rotator) (Math|Rotator|MakeRotator (.roll (Variables|Default|GetRelative%20Rotation)) (.pitch (Variables|Default|GetRelative%20Rotation)) (.yaw (Variables|Default|GetRelative%20Rotation))) (Math|Rotator|MakeRotator 0.0 0.0 0.0) _newtrack_0) false false))
          (:Finished
            (Utilities|FlowControl|DoOnce false) ; enters at Reset
          )))
      (:then_1
        (bind _newtrack_0_2 (Timeline|Timeline_4 Stop)
          (:Update
            (Transformation|SetRelativeRotation _mesh_2 (Math|Rotator|Lerp(Rotator) (Math|Rotator|MakeRotator (.roll (Variables|Default|GetRelative%20Rotation)) (.pitch (Variables|Default|GetRelative%20Rotation)) (.yaw (Variables|Default|GetRelative%20Rotation))) (Math|Rotator|MakeRotator (+ (.roll (Variables|Default|GetRelative%20Rotation)) 1e+01) (.pitch (Variables|Default|GetRelative%20Rotation)) (.yaw (Variables|Default|GetRelative%20Rotation))) _newtrack_0_2) false false)))))))

(event Custom|Tower_moving
  (bind _capsulecomponent (Variables|Collision|GetCapsuleComponent))
  (if (Variables|Default|GetHouse_Oven_Active)
    (if (Variables|Default|GetHouse_Moving)
      (bind _output_get (Variables|Default|SetWaklking_House_Speed (+ (Variables|Default|GetWaklking_House_Speed) 0.08)))
      (if (>= _output_get 25.0)
        (Variables|Default|SetWaklking_House_Speed 25.0))
      (bind _output_get_2 (Variables|Default|SetWorld_Loc_Walking_House (Transformation|GetWorldLocation _capsulecomponent)))
      (Transformation|SetWorldLocation _capsulecomponent (+ _output_get_2 (* (Math|Vector|GetForwardVector _capsulecomponent) (Variables|Default|GetWaklking_House_Speed))) false false)
      (else
        (Variables|Default|SetWaklking_House_Speed 0.0)))))

(event Custom|E_Button_Released
  (Utilities|FlowControl|Sequence
    (:then_0
      (if (>= (Variables|Default|GetSteps_number) (Variables|Default|GetMininum_Steps_Before_Walk))
        (Variables|Default|SetHouse_Moving true)
        (CallFunction|RepeatSteps)
        (else
          (Variables|Default|SetHouse_Moving false)
          (CallFunction|StopMontage))))))

(event Custom|Right_Mouse_Pressed
  (bind _mesh (Variables|Character|GetMesh))
  ;[1 1 1] LEAN LEFT RIGHT
  (if (Variables|Default|GetMain_Capsule_Can_Rotate)
    (Utilities|FlowControl|DoOnce false :!label _label
      (:Completed
        (Utilities|FlowControl|Sequence
          (:then_0
            (bind _newtrack_0 (Timeline|Timeline_5 Stop)
              (:Update
                (Transformation|SetRelativeRotation (Variables|Character|GetMesh) (Math|Rotator|Lerp(Rotator) (Math|Rotator|MakeRotator (.roll (Variables|Default|GetRelative%20Rotation)) (.pitch (Variables|Default|GetRelative%20Rotation)) (.yaw (Variables|Default|GetRelative%20Rotation))) (Math|Rotator|MakeRotator 0.0 0.0 0.0) _newtrack_0) false false))
              (:Finished
                (goto _label Reset))))
          (:then_1
            (Variables|Default|SetRelative%20Rotation (Variables|/Script/Engine.SceneComponent|GetRelativeRotation _mesh))
            (bind _newtrack_0_2 (Timeline|Timeline_4 PlayFromStart)
              (:Update
                (Transformation|SetRelativeRotation _mesh (Math|Rotator|Lerp(Rotator) (Math|Rotator|MakeRotator (.roll (Variables|Default|GetRelative%20Rotation)) (.pitch (Variables|Default|GetRelative%20Rotation)) (.yaw (Variables|Default|GetRelative%20Rotation))) (Math|Rotator|MakeRotator (+ (.roll (Variables|Default|GetRelative%20Rotation)) 1e+01) (.pitch (Variables|Default|GetRelative%20Rotation)) (.yaw (Variables|Default|GetRelative%20Rotation))) _newtrack_0_2) false false)))))))))

(event Custom|Stop_Montage
  (bind _arrow_direction_left (Variables|Default|GetArrow_Direction_Left))
  (bind _arrow_direction_right (Variables|Default|GetArrow_Direction_Right))
  (Utilities|FlowControl|Sequence
    (:then_0
      (Timeline|Timeline_0 Stop
        (:Update
          (Rendering|Material|SetScalarParameterValueonMaterials _arrow_direction_left "Color_Lerp" 1.0))
        (:Finished
          (Variables|Default|SetHouse_Moving false)
          (Variables|Default|SetLeft_Step_Finished true)
          (Rendering|Material|SetScalarParameterValueonMaterials _arrow_direction_left "Color_Lerp" 0.0)
          (CallFunction|RepeatSteps))))
    (:then_1
      (Timeline|Timeline_1 Stop
        (:Update
          (Rendering|Material|SetScalarParameterValueonMaterials _arrow_direction_right "Color_Lerp" 1.0))
        (:Finished
          (Variables|Default|SetHouse_Moving false)
          (Variables|Default|SetRight_Step_Finished true)
          (Rendering|Material|SetScalarParameterValueonMaterials _arrow_direction_right "Color_Lerp" 0.0)
          (CallFunction|RepeatSteps))))
    (:then_2
      (Variables|Default|SetLeft_Step_Finished true)
      (Variables|Default|SetRight_Step_Finished true)
      (Variables|Default|SetSteps_number 0))))

(event Custom|Oven_Activate
  (if (Variables|Default|GetPlayer_In_Oven)
    (Variables|Default|SetHouse_Oven_Active true)
    (Rendering|Components|Light|SetIntensity (Variables|Default|GetOven_Pointlight) 5e+03)))

(event Custom|Oven_Deactivate
  (Variables|Default|SetHouse_Oven_Active false)
  (Rendering|Components|Light|SetIntensity (Variables|Default|GetOven_Pointlight) 0.0))

(event Custom|Cam_Shale_L
  (Camera|PlayWorldCameraShake "/Game/Characters/Walking_House/Walking_House_Walking_Shake.Walking_House_Walking_Shake_C" (Transformation|GetSocketLocation (Variables|Character|GetMesh) "left_foot1_jntSocket") 0.0 1e+03))

(event Custom|Step_Right
  (bind _arrow_direction_right (Variables|Default|GetArrow_Direction_Right))
  (if (Variables|Default|GetHouse_Can_move)
    (if (Variables|Default|GetLeft_Step_Finished)
      (Variables|Default|SetLeft_Step_Finished false)
      (Variables|Default|SetHouse_Moving true)
      (Variables|Default|SetSteps_number (+ (Variables|Default|GetSteps_number) 1))
      (if (Variables|Default|GetLeft_Right_Step)
        (Variables|Default|SetLeft_Right_Step false)
        (Timeline|Timeline_1 PlayFromStart
          (:Update
            (Rendering|Material|SetScalarParameterValueonMaterials _arrow_direction_right "Color_Lerp" 1.0))
          (:Finished
            (Variables|Default|SetHouse_Moving false)
            (Variables|Default|SetRight_Step_Finished true)
            (Rendering|Material|SetScalarParameterValueonMaterials _arrow_direction_right "Color_Lerp" 0.0)
            (CallFunction|RepeatSteps)))))))

(event Custom|Left_Mouse_Pressed
  (bind _mesh (Variables|Character|GetMesh))
  ;[1 1 1] LEAN LEFT RIGHT
  (if (Variables|Default|GetMain_Capsule_Can_Rotate)
    (Utilities|FlowControl|DoOnce false :!label _label
      (:Completed
        (Utilities|FlowControl|Sequence
          (:then_0
            (bind _newtrack_0 (Timeline|Timeline_3 Stop)
              (:Update
                (Transformation|SetRelativeRotation (Variables|Character|GetMesh) (Math|Rotator|Lerp(Rotator) (Math|Rotator|MakeRotator (.roll (Variables|Default|GetRelative%20Rotation)) (.pitch (Variables|Default|GetRelative%20Rotation)) (.yaw (Variables|Default|GetRelative%20Rotation))) (Math|Rotator|MakeRotator 0.0 0.0 0.0) _newtrack_0) false false))
              (:Finished
                (goto _label Reset))))
          (:then_1
            (Variables|Default|SetRelative%20Rotation (Variables|/Script/Engine.SceneComponent|GetRelativeRotation _mesh))
            (bind _newtrack_0_2 (Timeline|Timeline_2 PlayFromStart)
              (:Update
                (Transformation|SetRelativeRotation _mesh (Math|Rotator|Lerp(Rotator) (Math|Rotator|MakeRotator (.roll (Variables|Default|GetRelative%20Rotation)) (.pitch (Variables|Default|GetRelative%20Rotation)) (.yaw (Variables|Default|GetRelative%20Rotation))) (Math|Rotator|MakeRotator (+ (.roll (Variables|Default|GetRelative%20Rotation)) -1e+01) (.pitch (Variables|Default|GetRelative%20Rotation)) (.yaw (Variables|Default|GetRelative%20Rotation))) _newtrack_0_2) false false)))))))))

(event Custom|Left_Mouse_Released
  (bind _mesh (Variables|Character|GetMesh))
  (bind _mesh_2 (Variables|Character|GetMesh))
  ;[1 1 1] LEAN LEFT RIGHT
  (if (Variables|Default|GetMain_Capsule_Can_Rotate)
    (Utilities|FlowControl|Sequence
      (:then_0
        (Variables|Default|SetRelative%20Rotation (Variables|/Script/Engine.SceneComponent|GetRelativeRotation _mesh_2))
        (bind _newtrack_0 (Timeline|Timeline_3 PlayFromStart)
          (:Update
            (Transformation|SetRelativeRotation _mesh_2 (Math|Rotator|Lerp(Rotator) (Math|Rotator|MakeRotator (.roll (Variables|Default|GetRelative%20Rotation)) (.pitch (Variables|Default|GetRelative%20Rotation)) (.yaw (Variables|Default|GetRelative%20Rotation))) (Math|Rotator|MakeRotator 0.0 0.0 0.0) _newtrack_0) false false))
          (:Finished
            (Utilities|FlowControl|DoOnce false) ; enters at Reset
          )))
      (:then_1
        (bind _newtrack_0_2 (Timeline|Timeline_2 Stop)
          (:Update
            (Transformation|SetRelativeRotation _mesh (Math|Rotator|Lerp(Rotator) (Math|Rotator|MakeRotator (.roll (Variables|Default|GetRelative%20Rotation)) (.pitch (Variables|Default|GetRelative%20Rotation)) (.yaw (Variables|Default|GetRelative%20Rotation))) (Math|Rotator|MakeRotator (+ (.roll (Variables|Default|GetRelative%20Rotation)) -1e+01) (.pitch (Variables|Default|GetRelative%20Rotation)) (.yaw (Variables|Default|GetRelative%20Rotation))) _newtrack_0_2) false false)))))))

(event Custom|E_Button_Pressed
  (bind _arrow_direction_left (Variables|Default|GetArrow_Direction_Left))
  (bind _arrow_direction_right (Variables|Default|GetArrow_Direction_Right))
  (Utilities|FlowControl|Sequence
    (:then_0
      (if (Variables|Default|GetHouse_Can_move)
        (if (>= (Variables|Default|GetSteps_number) (Variables|Default|GetMaximum_Steps_Before_Stop))
          (Variables|Default|SetSteps_number 0)
          (Variables|Default|SetHouse_Can_move false)
          (CallFunction|OvenDeactivate)
          (elif (Variables|Default|GetLeft_Right_Step)
            (if (Variables|Default|GetLeft_Step_Finished)
              (Variables|Default|SetLeft_Step_Finished false)
              (Variables|Default|SetHouse_Moving true)
              (Variables|Default|SetSteps_number (+ (Variables|Default|GetSteps_number) 1))
              (if (Variables|Default|GetLeft_Right_Step)
                (Variables|Default|SetLeft_Right_Step false)
                (Timeline|Timeline_1 PlayFromStart
                  (:Update
                    (Rendering|Material|SetScalarParameterValueonMaterials _arrow_direction_right "Color_Lerp" 1.0))
                  (:Finished
                    (Variables|Default|SetHouse_Moving false)
                    (Variables|Default|SetRight_Step_Finished true)
                    (Rendering|Material|SetScalarParameterValueonMaterials _arrow_direction_right "Color_Lerp" 0.0)
                    (CallFunction|RepeatSteps)))))
            (elif (Variables|Default|GetRight_Step_Finished)
              (Variables|Default|SetRight_Step_Finished false)
              (Variables|Default|SetHouse_Moving true)
              (Variables|Default|SetSteps_number (+ (Variables|Default|GetSteps_number) 1))
              (if (not (Variables|Default|GetLeft_Right_Step))
                (Variables|Default|SetLeft_Right_Step true)
                (Timeline|Timeline_0 PlayFromStart
                  (:Update
                    (Rendering|Material|SetScalarParameterValueonMaterials _arrow_direction_left "Color_Lerp" 1.0))
                  (:Finished
                    (Variables|Default|SetHouse_Moving false)
                    (Variables|Default|SetLeft_Step_Finished true)
                    (Rendering|Material|SetScalarParameterValueonMaterials _arrow_direction_left "Color_Lerp" 0.0)
                    (CallFunction|RepeatSteps)))))))))
    (:then_1
      (if (Variables|Default|GetPlayer_In_Oven)
        (if (Variables|Default|GetHouse_Oven_Active)
          (Variables|Default|SetHouse_Oven_Active false)
          (CallFunction|OvenDeactivate)
          (CallFunction|StopMontage)
          (else
            (CallFunction|OvenActivate)))))))

(event Custom|Rotating_Left_Main
  (bind _capsulecomponent (Variables|Collision|GetCapsuleComponent))
  ;[1 1 1] ROTATION LEFT RIGHT
  (if (Variables|Default|GetMain_Capsule_Can_Rotate)
    (if (Variables|Default|GetCapsule_Left_Rotation)
      (Variables|Default|SetMain_Capsule_Relative%20Rotation (Variables|/Script/Engine.SceneComponent|GetRelativeRotation _capsulecomponent))
      (Transformation|SetRelativeRotation _capsulecomponent (Math|Rotator|MakeRotator (.roll (Variables|Default|GetMain_Capsule_Relative%20Rotation)) (.pitch (Variables|Default|GetMain_Capsule_Relative%20Rotation)) (+ (.yaw (Variables|Default|GetMain_Capsule_Relative%20Rotation)) -0.1)) false false)
      (Rendering|Material|SetScalarParameterValueonMaterials (Variables|Default|GetArrow_Rotator_Left) "Color_Lerp" 1.0)
      (else
        (Rendering|Material|SetScalarParameterValueonMaterials (Variables|Default|GetArrow_Rotator_Left) "Color_Lerp" 0.0)))))

(event Custom|Rotating_Right_Main
  (bind _capsulecomponent (Variables|Collision|GetCapsuleComponent))
  ;[1 1 1] ROTATION LEFT RIGHT
  (if (Variables|Default|GetMain_Capsule_Can_Rotate)
    (if (Variables|Default|GetCapsule_Right_Rotation)
      (Variables|Default|SetMain_Capsule_Relative%20Rotation (Variables|/Script/Engine.SceneComponent|GetRelativeRotation _capsulecomponent))
      (Transformation|SetRelativeRotation _capsulecomponent (Math|Rotator|MakeRotator (.roll (Variables|Default|GetMain_Capsule_Relative%20Rotation)) (.pitch (Variables|Default|GetMain_Capsule_Relative%20Rotation)) (+ (.yaw (Variables|Default|GetMain_Capsule_Relative%20Rotation)) 0.1)) false false)
      (Rendering|Material|SetScalarParameterValueonMaterials (Variables|Default|GetArrow_Rotator_Right) "Color_Lerp" 1.0)
      (else
        (Rendering|Material|SetScalarParameterValueonMaterials (Variables|Default|GetArrow_Rotator_Right) "Color_Lerp" 0.0)))))

(event Custom|Repeat_Steps
  (bind _arrow_direction_left (Variables|Default|GetArrow_Direction_Left))
  (bind _arrow_direction_right (Variables|Default|GetArrow_Direction_Right))
  (if (Variables|Default|GetHouse_Oven_Active)
    (if (>= (Variables|Default|GetSteps_number) (Variables|Default|GetMaximum_Steps_Before_Stop))
      (Variables|Default|SetSteps_number 0)
      (Variables|Default|SetHouse_Can_move false)
      (CallFunction|OvenDeactivate)
      (elif (Variables|Default|GetLeft_Right_Step)
        (if (Variables|Default|GetLeft_Step_Finished)
          (Variables|Default|SetLeft_Step_Finished false)
          (Variables|Default|SetHouse_Moving true)
          (Variables|Default|SetSteps_number (+ (Variables|Default|GetSteps_number) 1))
          (if (Variables|Default|GetLeft_Right_Step)
            (Variables|Default|SetLeft_Right_Step false)
            (Timeline|Timeline_1 PlayFromStart
              (:Update
                (Rendering|Material|SetScalarParameterValueonMaterials _arrow_direction_right "Color_Lerp" 1.0))
              (:Finished
                (Variables|Default|SetHouse_Moving false)
                (Variables|Default|SetRight_Step_Finished true)
                (Rendering|Material|SetScalarParameterValueonMaterials _arrow_direction_right "Color_Lerp" 0.0)
                (CallFunction|RepeatSteps)))))
        (elif (Variables|Default|GetRight_Step_Finished)
          (Variables|Default|SetRight_Step_Finished false)
          (Variables|Default|SetHouse_Moving true)
          (Variables|Default|SetSteps_number (+ (Variables|Default|GetSteps_number) 1))
          (if (not (Variables|Default|GetLeft_Right_Step))
            (Variables|Default|SetLeft_Right_Step true)
            (Timeline|Timeline_0 PlayFromStart
              (:Update
                (Rendering|Material|SetScalarParameterValueonMaterials _arrow_direction_left "Color_Lerp" 1.0))
              (:Finished
                (Variables|Default|SetHouse_Moving false)
                (Variables|Default|SetLeft_Step_Finished true)
                (Rendering|Material|SetScalarParameterValueonMaterials _arrow_direction_left "Color_Lerp" 0.0)
                (CallFunction|RepeatSteps)))))))))

(event EventBeginPlay
  (Utilities|FlowControl|Sequence
    (:then_0
      (Utilities|FlowControl|Delay 0.2)
      (bind _outactors (Actor|GetAllActorsOfClass "/Script/Engine.StaticMeshActor"))
      (for _array_element _outactors
        (if (Components|ComponentHasTag (Variables|/Script/Engine.StaticMeshActor|GetStaticMeshComponent _array_element) "Floor")
          (Transformation|AttachActorToActor _array_element self "None" "KeepWorld" "KeepWorld" "KeepWorld" true))))
    (:then_1
      (bind _aspickup_base (Utilities|Casting|CastToPickupBase (Variables|/Script/Engine.ChildActorComponent|GetChildActor (Variables|Default|GetChildActor_wood))))
      (Variables|/Script/ArcherPRT.PickupBase|SetbInfinity _aspickup_base true)
      (bind _aspickup_base_2 (Utilities|Casting|CastToPickupBase (Variables|/Script/Engine.ChildActorComponent|GetChildActor (Variables|Default|GetChildActor_grass))))
      (Variables|/Script/ArcherPRT.PickupBase|SetbInfinity _aspickup_base_2 true))))

(event EventTick
  (params (DeltaSeconds :type Float%20%28single-precision%29))
  (Utilities|FlowControl|Sequence
    (:then_0
      (bind _foottraceoffset (CallFunction|IKFootTrace "left_foot1_jntSocket" -2e+04))
      (Variables|Default|SetIKLeftFootOffset _foottraceoffset)
      (bind _foottraceoffset_2 (CallFunction|IKFootTrace "right_foot1_jntSocket" -2e+04))
      (Variables|Default|SetIKRightFootOffset _foottraceoffset_2))
    (:then_2
      (CallFunction|RotatingLeftMain)
      (CallFunction|RotatingRightMain)
      (CallFunction|StrafingRight)
      (CallFunction|StrafingLeft)
      (CallFunction|TowerMoving))
    (:then_3
      (Development|PrintString (Utilities|String|ToString(Integer) (Variables|Default|GetSteps_number)) true true "(R=0.000000,G=0.660000,B=1.000000,A=1.000000)" 0.0))))

(fn ConstructionScript)

(fn IKFootTrace
  (params (SocketName :type Name) (Distance :type Float%20%28double-precision%29))
  (bind _mesh (Variables|Character|GetMesh))
  (bind _returnvalue (Transformation|GetSocketLocation _mesh SocketName))
  (bind (_outhit _returnvalue_2) (Collision|LineTraceByChannel (Math|Vector|MakeVector (.x _returnvalue) (.y _returnvalue) (.z (Transformation|GetActorLocation))) (Math|Vector|MakeVector (.x _returnvalue) (.y _returnvalue) Distance) "TraceTypeQuery1" false 0 "None" true "(R=1.000000,G=0.000000,B=0.000000,A=1.000000)" "(R=0.000000,G=1.000000,B=0.000000,A=1.000000)" 0.0))
  (if _returnvalue_2
    (return (.location _outhit) (.z (- (.location _outhit) (Transformation|GetWorldLocation (Variables|Character|GetMesh)))))
    (else
      (return "0, 0, 0" 0.0))))