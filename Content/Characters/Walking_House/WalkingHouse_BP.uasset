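; Walking house actor that constantly moves forward, carrying Floor-tagged static mesh actors it attaches to itself shortly after BeginPlay.
; Each tick, downward traces from both foot sockets compute IK offsets, while separate events play camera shakes at the feet and foot-sphere hits swap mesh materials.
; Overlap triggers toggle two elevators and a front door up or down through timeline lerps, using DoOnce against retriggering and a material parameter as indicator.
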(event OnComponentHit(SphereLeft)
  (params (HitComponent :type Primitive%20Component%20Object%20Reference) (OtherActor :type Actor%20Object%20Reference) (OtherComp :type Primitive%20Component%20Object%20Reference) (NormalImpulse :type Vector :default "0, 0, 0") (Hit :type Hit%20Result%20Structure%20%28by%20ref%29))
  (Rendering|Material|SetMaterial (Variables|Character|GetMesh) 2 "/Game/Characters/Walking_House/House_Mat.House_Mat"))

(event OnComponentHit(SphereRight)
  (params (HitComponent :type Primitive%20Component%20Object%20Reference) (OtherActor :type Actor%20Object%20Reference) (OtherComp :type Primitive%20Component%20Object%20Reference) (NormalImpulse :type Vector :default "0, 0, 0") (Hit :type Hit%20Result%20Structure%20%28by%20ref%29))
  (Rendering|Material|SetMaterial (Variables|Character|GetMesh) 1 0))

(event OnComponentBeginOverlap(Elevator_World_Collision)
  (params (OverlappedComponent :type Primitive%20Component%20Object%20Reference) (OtherActor :type Actor%20Object%20Reference) (OtherComp :type Primitive%20Component%20Object%20Reference) (OtherBodyIndex :type Integer) (bFromSweep :type Boolean) (SweepResult :type Hit%20Result%20Structure%20%28by%20ref%29))
  (bind _elevator_world (Variables|Default|GetElevator_World))
  (bind _relativelocation (Variables|/Script/Engine.SceneComponent|GetRelativeLocation _elevator_world))
  (Utilities|FlowControl|Sequence
    (:then_0
      (Utilities|FlowControl|DoOnce false :!label _label
        (:Completed
          (if (Variables|Default|Getleft_right_World_Elevator)
            (Variables|Default|Setleft_right_World_Elevator false)
            (Variables|Default|Setleft_Right__World_Elevator_Variable_0 3026.0)
            (else
              (Variables|Default|Setleft_right_World_Elevator true)
              (Variables|Default|Setleft_Right__World_Elevator_Variable_0 -3026.0)))
          (Variables|Default|Setrotation_box_World_Elevator (.z _relativelocation))
          (bind _newtrack_0 (Timeline|Timeline_2 PlayFromStart)
            (:Update
              (Transformation|SetRelativeLocation _elevator_world (Math|Vector|MakeVector (.x _relativelocation) (.y _relativelocation) (Math|Float|Lerp (Variables|Default|Getrotation_box_World_Elevator) (+ (Variables|Default|Getrotation_box_World_Elevator) (Variables|Default|Getleft_Right__World_Elevator_Variable_0)) _newtrack_0)) false false))
            (:Finished
              (Rendering|Material|SetScalarParameterValueonMaterials (Variables|Default|GetElevator_Sphere) "Color" 0.0)
              (goto _label Reset))))))
    (:then_1
      (Rendering|Material|SetScalarParameterValueonMaterials (Variables|Default|GetElevator_Sphere) "Color" 1.0))))

(event OnComponentBeginOverlap(Front_Door)
  (params (OverlappedComponent :type Primitive%20Component%20Object%20Reference) (OtherActor :type Actor%20Object%20Reference) (OtherComp :type Primitive%20Component%20Object%20Reference) (OtherBodyIndex :type Integer) (bFromSweep :type Boolean) (SweepResult :type Hit%20Result%20Structure%20%28by%20ref%29))
  (bind _front_door_mesh (Variables|Default|GetFront_Door_Mesh))
  (bind _relativelocation (Variables|/Script/Engine.SceneComponent|GetRelativeLocation _front_door_mesh))
  (Utilities|FlowControl|Sequence
    (:then_0
      (Utilities|FlowControl|DoOnce false :!label _label
        (:Completed
          (if (Variables|Default|Getleft_right)
            (Variables|Default|Setleft_right false)
            (Variables|Default|Setleft_Right_Variable -7e+02)
            (else
              (Variables|Default|Setleft_right true)
              (Variables|Default|Setleft_Right_Variable 7e+02)))
          (Variables|Default|Setrotation_box (.z _relativelocation))
          (bind _newtrack_0 (Timeline|Timeline_1 PlayFromStart)
            (:Update
              (Transformation|SetRelativeLocation (Variables|Default|GetFront_Door_Mesh) (Math|Vector|MakeVector (.x _relativelocation) (.y _relativelocation) (Math|Float|Lerp (Variables|Default|Getrotation_box) (+ (Variables|Default|Getrotation_box) (Variables|Default|Getleft_Right_Variable)) _newtrack_0)) false false))
            (:Finished
              (Rendering|Material|SetScalarParameterValueonMaterials (Variables|Default|GetFront_Door_Sphere) "Color" 0.0)
              (goto _label Reset))))))
    (:then_1
      (Rendering|Material|SetScalarParameterValueonMaterials (Variables|Default|GetFront_Door_Sphere) "Color" 1.0))))

(event OnComponentBeginOverlap(Elevator_down)
  (params (OverlappedComponent :type Primitive%20Component%20Object%20Reference) (OtherActor :type Actor%20Object%20Reference) (OtherComp :type Primitive%20Component%20Object%20Reference) (OtherBodyIndex :type Integer) (bFromSweep :type Boolean) (SweepResult :type Hit%20Result%20Structure%20%28by%20ref%29))
  (bind _elevator_mesh (Variables|Default|GetElevator_Mesh))
  (bind _relativelocation (Variables|/Script/Engine.SceneComponent|GetRelativeLocation _elevator_mesh))
  (Utilities|FlowControl|Sequence
    (:then_0
      (Utilities|FlowControl|DoOnce false :!label _label
        (:Completed
          (if (Variables|Default|Getleft_right_inner)
            (Variables|Default|Setleft_right_inner false)
            (Variables|Default|Setleft_Right_Inner_Variable 1231.0)
            (else
              (Variables|Default|Setleft_right_inner true)
              (Variables|Default|Setleft_Right_Inner_Variable -1231.0)))
          (Variables|Default|Setrotation_box_inner (.z _relativelocation))
          (bind _newtrack_0 (Timeline|Timeline_0 PlayFromStart)
            (:Update
              (Transformation|SetRelativeLocation _elevator_mesh (Math|Vector|MakeVector (.x _relativelocation) (.y _relativelocation) (Math|Float|Lerp (Variables|Default|Getrotation_box_inner) (+ (Variables|Default|Getrotation_box_inner) (Variables|Default|Getleft_Right_Inner_Variable)) _newtrack_0)) false false))
            (:Finished
              (Rendering|Material|SetScalarParameterValueonMaterials (Variables|Default|GetElevator_Sphere) "Color" 0.0)
              (goto _label Reset))))))
    (:then_1
      (Rendering|Material|SetScalarParameterValueonMaterials (Variables|Default|GetElevator_Sphere) "Color" 1.0))))

(event Custom|Cam_Shake_R
  (Camera|PlayWorldCameraShake "/Game/Characters/Walking_House/Walking_House_Walking_Shake.Walking_House_Walking_Shake_C" (Transformation|GetSocketLocation (Variables|Character|GetMesh) "right_foot1_jntSocket") 0.0 1e+03))

(event Custom|Cam_Shale_L
  (Camera|PlayWorldCameraShake "/Game/Characters/Walking_House/Walking_House_Walking_Shake.Walking_House_Walking_Shake_C" (Transformation|GetSocketLocation (Variables|Character|GetMesh) "left_foot1_jntSocket") 0.0 1e+03))

(event EventBeginPlay
  (Utilities|FlowControl|Delay 0.2)
  (bind _outactors (Actor|GetAllActorsOfClass "/Script/Engine.StaticMeshActor"))
  (for _array_element _outactors
    (if (Components|ComponentHasTag (Variables|/Script/Engine.StaticMeshActor|GetStaticMeshComponent _array_element) "Floor")
      (Transformation|AttachActorToActor _array_element self "None" "KeepWorld" "KeepWorld" "KeepWorld" true))))

(event EventTick
  (params (DeltaSeconds :type Float%20%28single-precision%29))
  (Transformation|AddActorLocalOffset (* (Transformation|GetActorForwardVector) 10) true false)
  (bind _foottraceoffset (CallFunction|IKFootTrace "left_foot1_jntSocket" -2e+04))
  (Variables|Default|SetIKLeftFootOffset _foottraceoffset)
  (bind _foottraceoffset_2 (CallFunction|IKFootTrace "right_foot1_jntSocket" -2e+04))
  (Variables|Default|SetIKRightFootOffset _foottraceoffset_2))

(fn ConstructionScript)

(fn IKFootTrace
  (params (SocketName :type Name) (Distance :type Float%20%28double-precision%29))
  (bind _mesh (Variables|Character|GetMesh))
  (bind _returnvalue (Transformation|GetSocketLocation _mesh SocketName))
  (bind (_outhit _returnvalue_2) (Collision|LineTraceByChannel (Math|Vector|MakeVector (.x _returnvalue) (.y _returnvalue) (.z (Transformation|GetActorLocation))) (Math|Vector|MakeVector (.x _returnvalue) (.y _returnvalue) Distance) "TraceTypeQuery1" false 0 "None" true "(R=1.000000,G=0.000000,B=0.000000,A=1.000000)" "(R=0.000000,G=1.000000,B=0.000000,A=1.000000)" 0.0))
  (if _returnvalue_2
    (return (.location _outhit) (.z (- (.location _outhit) (Transformation|GetWorldLocation (Variables|Character|GetMesh)))))
    (else
      (return "0, 0, 0" 0.0))))