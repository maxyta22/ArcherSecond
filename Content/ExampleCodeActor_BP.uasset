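; Example actor Blueprint that exercises functions and variables exposed to Blueprint, apparently from a C++ parent class.
; BeginPlay passes the result of a pure function into a callable one.
; The native event override skips its unwired parent call, runs an input/output function using the actor's location, and prints the outputs.
; Implementable events are empty stubs, and the int-returning override returns zero.
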(event EventBeginPlay
  (Class|ExampleCodeActor|ExampleBlueprintCallableFunction (Class|ExampleCodeActor|ExampleBlueprintPureFunction)))

(event Collision|EventActorBeginOverlap
  (params (OtherActor :type Actor%20Object%20Reference)))

(event EventTick
  (params (DeltaSeconds :type Float%20%28single-precision%29)))

(event EventExampleNativeEventFunction
  (bind (_outint _outbool _outvector) (Class|ExampleCodeActor|ExampleInputOtputFunction 6 "0, 0, 0" (Transformation|GetActorLocation)))
  (Development|PrintString (Utilities|String|ToString(Integer) _outint))
  (Development|PrintString (Utilities|String|ToString(Boolean) _outbool))
  (Development|PrintString (Utilities|String|ToString(Vector) _outvector)))

(event EventExampleImplementableFunction
  (params (value :type Integer)))

(event EventExampleImplementableEventFunction
  (params (value :type Integer)))

(fn ConstructionScript)

(fn ExampleImplementableEventReturnIntFunction
  (params (value :type Integer))
  (return 0))