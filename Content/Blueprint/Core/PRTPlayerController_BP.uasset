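; PRTPlayerController_BP is a player controller that handles the pause menu.
; BeginPlay creates a MainMenu_UI widget, and possessing a pawn sets game-only input.
; The PauseMenu input toggles that widget: showing it pauses the game, shows the cursor and focuses it with game-and-UI input, while hiding it reverses this.
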(event EventBeginPlay
  (bind _returnvalue (UserInterface|CreateWidget "/Game/Blueprint/UI/MainMenu_UI.MainMenu_UI_C"))
  (Variables|Default|SetMainMenu _returnvalue))

(event EventPossess
  (params (PossessedPawn :type Pawn%20Object%20Reference))
  (|CallParentFunction PossessedPawn)
  (Input|SetInputModeGameOnly self))

(event Input|ActionEvents|InputActionPauseMenu
  (params (Key :type Key%20Structure :default "None"))
  (bind _self self)
  (bind _mainmenu (Variables|Default|GetMainMenu))
  ;[0.1411 0 1] Pause
  (:Pressed
    (if (not (UserInterface|Viewport|IsinViewport (Variables|Default|GetMainMenu)))
      (Game|SetGamePaused true)
      (UserInterface|Viewport|AddtoViewport _mainmenu 0)
      (Variables|/Script/Engine.PlayerController|SetbShowMouseCursor _self true)
      (Input|SetInputModeGameandUI _self (Variables|Default|GetMainMenu) "DoNotLock" true)
      (else
        (Game|SetGamePaused false)
        (Widget|RemovefromParent _mainmenu)
        (Variables|/Script/Engine.PlayerController|SetbShowMouseCursor _self false)
        (Input|SetInputModeGameOnly _self)))))

(fn ConstructionScript)