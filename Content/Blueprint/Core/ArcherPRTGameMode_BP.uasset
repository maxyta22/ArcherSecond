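; Game mode for the archer game that handles level streaming, world restarts and saving or loading the player.
; On BeginPlay it freezes the player while loading stream levels sequentially, then either initializes and saves default inventory or loads, per the GameInstance NewGame flag.
; Save and load copy player transform, resources and ammo through a PlayerSaveObject in one slot, iterating over enums.
; RestartWorld sets that flag and reopens the cave level.
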(event Custom|SaveGame
  (bind _playerref (Variables|Default|GetPlayerRef))
  (bind _playerref_2 (Variables|Default|GetPlayerRef))
  (bind _playerref_3 (Variables|Default|GetPlayerRef))
  (bind _inventorycomponent (Variables|/Script/ArcherPRT.PlayerCharacter|GetInventoryComponent _playerref_2))
  (bind _inventorycomponent_2 (Variables|/Script/ArcherPRT.PlayerCharacter|GetInventoryComponent _playerref_3))
  (Development|PrintString "SAVE GAME" true true "(R=1.000000,G=0.996119,B=0.000000,A=1.000000)" 5.0)
  (bind _returnvalue (SaveGame|DoesSaveGameExist "ArcherSave"))
  (if _returnvalue
    (bind _returnvalue_2 (SaveGame|LoadGamefromSlot "ArcherSave"))
    (bind _asplayer_save_object (Utilities|Casting|CastToPlayerSaveObject _returnvalue_2))
    (Variables|Default|SetCurrentSaveObject _asplayer_save_object)
    (else
      (bind _returnvalue_3 (SaveGame|CreateSaveGameObject "/Game/Blueprint/SaveObjects/PlayerSaveObject.PlayerSaveObject_C"))
      (Variables|Default|SetCurrentSaveObject _returnvalue_3)))
  (Utilities|FlowControl|Sequence
    (:then_0
      ;[0.03529 0 1 1 60] Save Player Position
      (Variables|/Game/Blueprint/SaveObjects/PlayerSaveObject.PlayerSaveObject_C|SetSavePlayerLocation (Variables|Default|GetCurrentSaveObject) (Transformation|GetActorLocation _playerref))
      (Variables|/Game/Blueprint/SaveObjects/PlayerSaveObject.PlayerSaveObject_C|SetSavePlayerRotation (Variables|Default|GetCurrentSaveObject) (Transformation|GetActorRotation _playerref)))
    (:then_1
      ;[0.03529 0 1 1 60] Save Player Inventory
      (Utilities|Map|Clear (Variables|/Game/Blueprint/SaveObjects/PlayerSaveObject.PlayerSaveObject_C|GetResources (Variables|Default|GetCurrentSaveObject)))
      (bind _enumvalue (|ForEachEResourcesType)
        (:LoopBody
          (Utilities|Map|Add (Variables|/Game/Blueprint/SaveObjects/PlayerSaveObject.PlayerSaveObject_C|GetResources (Variables|Default|GetCurrentSaveObject)) _enumvalue (Class|InventoryComponent|GetValueResourses _inventorycomponent_2 _enumvalue))
          (Utilities|Map|Add (Variables|/Game/Blueprint/SaveObjects/PlayerSaveObject.PlayerSaveObject_C|GetMaxResources (Variables|Default|GetCurrentSaveObject)) _enumvalue (Class|InventoryComponent|GetMaxResourses _inventorycomponent_2 _enumvalue)))
        (:then
          (Utilities|Map|Clear (Variables|/Game/Blueprint/SaveObjects/PlayerSaveObject.PlayerSaveObject_C|GetAmmo (Variables|Default|GetCurrentSaveObject)))
          (bind _enumvalue_2 (|ForEachEAmmoType)
            (:LoopBody
              (Utilities|Map|Add (Variables|/Game/Blueprint/SaveObjects/PlayerSaveObject.PlayerSaveObject_C|GetAmmo (Variables|Default|GetCurrentSaveObject)) _enumvalue_2 (Class|InventoryComponent|GetValueAmmo _inventorycomponent _enumvalue_2))
              (Utilities|Map|Add (Variables|/Game/Blueprint/SaveObjects/PlayerSaveObject.PlayerSaveObject_C|GetMaxAmmo (Variables|Default|GetCurrentSaveObject)) _enumvalue_2 (Class|InventoryComponent|GetMaxAmmo _inventorycomponent _enumvalue_2)))))))
    (:then_2
      (SaveGame|SaveGametoSlot (Variables|Default|GetCurrentSaveObject) "ArcherSave"))))

(event Custom|RestartWorld
  (params (NewGame :type Boolean))
  (Variables|/Game/Blueprint/Core/ArcherPRTGameInstance_BP.ArcherPRTGameInstance_BP_C|SetNewGame (.AsArcher%20PRTGame%20Instance%20BP (Utilities|Casting|CastToArcherPRTGameInstance_BP (Game|GetGameInstance))) NewGame)
  (Game|OpenLevel(byName) "Cave_05_visual"))

(event Custom|LoadGame
  (bind _playerref (Variables|Default|GetPlayerRef))
  (bind _playerref_2 (Variables|Default|GetPlayerRef))
  (bind _inventorycomponent (Variables|/Script/ArcherPRT.PlayerCharacter|GetInventoryComponent _playerref))
  (bind _inventorycomponent_2 (Variables|/Script/ArcherPRT.PlayerCharacter|GetInventoryComponent _playerref_2))
  (Development|PrintString "LOAD GAME" true true "(R=1.000000,G=0.996119,B=0.000000,A=1.000000)" 5.0)
  (bind _returnvalue (SaveGame|DoesSaveGameExist "ArcherSave"))
  (if _returnvalue
    (bind _returnvalue_2 (SaveGame|LoadGamefromSlot "ArcherSave"))
    (bind _asplayer_save_object (Utilities|Casting|CastToPlayerSaveObject _returnvalue_2))
    (Variables|Default|SetCurrentSaveObject _asplayer_save_object)
    (Utilities|FlowControl|Sequence
      (:then_0
        ;[0 1 0.9842 1 60] Load Player Position
        (Transformation|SetActorLocationAndRotation (Variables|Default|GetPlayerRef) (Variables|/Game/Blueprint/SaveObjects/PlayerSaveObject.PlayerSaveObject_C|GetSavePlayerLocation (Variables|Default|GetCurrentSaveObject)) (Variables|/Game/Blueprint/SaveObjects/PlayerSaveObject.PlayerSaveObject_C|GetSavePlayerRotation (Variables|Default|GetCurrentSaveObject)) false true))
      (:then_1
        ;[0 1 0.9842 1 60] Load Player Inventory
        (bind _enumvalue (|ForEachEResourcesType)
          (:LoopBody
            (Class|InventoryComponent|AddResources _inventorycomponent _enumvalue (.Value (Utilities|Map|Find (Variables|/Game/Blueprint/SaveObjects/PlayerSaveObject.PlayerSaveObject_C|GetResources (Variables|Default|GetCurrentSaveObject)) _enumvalue)))
            (Class|InventoryComponent|SetMaxResourses _inventorycomponent _enumvalue (.Value (Utilities|Map|Find (Variables|/Game/Blueprint/SaveObjects/PlayerSaveObject.PlayerSaveObject_C|GetMaxResources (Variables|Default|GetCurrentSaveObject)) _enumvalue))))
          (:then
            (bind _enumvalue_2 (|ForEachEAmmoType)
              (:LoopBody
                (Class|InventoryComponent|SetAmmo _inventorycomponent_2 _enumvalue_2 (.Value (Utilities|Map|Find (Variables|/Game/Blueprint/SaveObjects/PlayerSaveObject.PlayerSaveObject_C|GetAmmo (Variables|Default|GetCurrentSaveObject)) _enumvalue_2)))
                (Class|InventoryComponent|SetMaxAmmo _inventorycomponent_2 _enumvalue_2 (.Value (Utilities|Map|Find (Variables|/Game/Blueprint/SaveObjects/PlayerSaveObject.PlayerSaveObject_C|GetMaxAmmo (Variables|Default|GetCurrentSaveObject)) _enumvalue_2)))))))))
    (else
      (CallFunction|SetDefaultInventoryContents))))

(event EventBeginPlay
  (|CallParentFunction)
  (Utilities|FlowControl|Sequence
    (:then_0
      (bind _asplayer_character_bp (Utilities|Casting|CastToPlayerCharacter_BP (Game|GetPlayerCharacter 0)))
      (Variables|Default|SetPlayerRef _asplayer_character_bp)
      (Utilities|LoadFullStreamLevels)
      (if (Variables|/Game/Blueprint/Core/ArcherPRTGameInstance_BP.ArcherPRTGameInstance_BP_C|GetNewGame (.AsArcher%20PRTGame%20Instance%20BP (Utilities|Casting|CastToArcherPRTGameInstance_BP (Game|GetGameInstance))))
        (CallFunction|SetDefaultInventoryContents)
        (CallFunction|SaveGame)
        (else
          (CallFunction|LoadGame))))))

(fn ConstructionScript)

(fn SetDefaultInventoryContents
  (bind _playerref (Variables|Default|GetPlayerRef))
  (bind _playerref_2 (Variables|Default|GetPlayerRef))
  (bind _playerref_3 (Variables|Default|GetPlayerRef))
  (bind _playerref_4 (Variables|Default|GetPlayerRef))
  (bind _inventorycomponent (Variables|/Script/ArcherPRT.PlayerCharacter|GetInventoryComponent _playerref))
  (bind _inventorycomponent_2 (Variables|/Script/ArcherPRT.PlayerCharacter|GetInventoryComponent _playerref_2))
  (bind _inventorycomponent_3 (Variables|/Script/ArcherPRT.PlayerCharacter|GetInventoryComponent _playerref_3))
  (bind _inventorycomponent_4 (Variables|/Script/ArcherPRT.PlayerCharacter|GetInventoryComponent _playerref_4))
  (bind _maxresources (Variables|/Script/ArcherPRT.InventoryComponent|GetMaxResources _inventorycomponent_3))
  (bind _resources (Variables|/Script/ArcherPRT.InventoryComponent|GetResources _inventorycomponent_3))
  (bind _maxammo (Variables|/Script/ArcherPRT.InventoryComponent|GetMaxAmmo _inventorycomponent_2))
  (bind _ammo (Variables|/Script/ArcherPRT.InventoryComponent|GetAmmo _inventorycomponent_2))
  (bind (_maxwood _maxrock _maxgrass _maxmetal _maxfood _maxbattery _maxlamp _maxmine) (Utilities|Struct|BreakMaxResoursesData _maxresources))
  (bind (_valuewood _valuerock _valuegrass _valuemetal _valuefood _valuebattery _valuelamp _valuemine) (Utilities|Struct|BreakResoursesData _resources))
  (bind (_maxwoodarrow _maxrockarrow _maxmetalarrow) (Utilities|Struct|BreakMaxAmmoData _maxammo))
  (bind (_valuewoodarrow _valuerockarrow _valuemetalarrow) (Utilities|Struct|BreakAmmoData _ammo))
  (Utilities|FlowControl|Sequence
    (:then_0
      (bind _enumvalue (|ForEachEResourcesType)
        (:LoopBody
          (Class|InventoryComponent|SetMaxResourses _inventorycomponent_4 _enumvalue (Utilities|Select :Index _enumvalue :None 0 :Wood _maxwood :Rock _maxrock :Grass _maxgrass :Metal _maxmetal :Food _maxfood :Battery _maxbattery :Lamp _maxlamp :Mine _maxmine))
          (Class|InventoryComponent|AddResources _inventorycomponent_4 _enumvalue (Utilities|Select :Index _enumvalue :None 0 :Wood _valuewood :Rock _valuerock :Grass _valuegrass :Metal _valuemetal :Food _valuefood :Battery _valuebattery :Lamp _valuelamp :Mine _valuemine)))))
    (:then_1
      (bind _enumvalue_2 (|ForEachEAmmoType)
        (:LoopBody
          (Class|InventoryComponent|SetMaxAmmo _inventorycomponent _enumvalue_2 (Utilities|Select :Index _enumvalue_2 :None 0 :WoodArrow _maxwoodarrow :RockArrow _maxrockarrow :MetalArrow _maxmetalarrow))
          (Class|InventoryComponent|SetAmmo _inventorycomponent _enumvalue_2 (Utilities|Select :Index _enumvalue_2 :None 0 :WoodArrow _valuewoodarrow :RockArrow _valuerockarrow :MetalArrow _valuemetalarrow)))))))