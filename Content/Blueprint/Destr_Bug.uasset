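; Destr_Bug is a destructible Geometry Collection actor that breaks apart on its own shortly after play begins.
; After a delay, BeginPlay enables physics-only collision and simulation, then applies a radial external cluster strain field at the collection's location to fracture it.
; An X-axis velocity-change impulse follows immediately.
; A radial linear-force field and a delayed self-destroy are present but unconnected, so they never run.
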(event EventBeginPlay
  (Utilities|FlowControl|Delay 3.0)
  (Collision|SetCollisionEnabled (Variables|Default|GetGeometryCollection) "PhysicsOnly")
  (Physics|SetSimulatePhysics (Variables|Default|GetGeometryCollection) true)
  (Class|FieldSystemComponent|ApplyPhysicsField (Variables|Default|GetFieldSystem) true "Field_ExternalClusterStrain" 0 (Field|SetRadialFalloff (Variables|Default|GetRadialFalloff) 1e+05 0.0 1.0 0.0 5e+01 (Transformation|GetWorldLocation (Variables|Default|GetGeometryCollection)) "Field_FallOff_None"))
  (Physics|AddImpulse (Variables|Default|GetGeometryCollection) "400.000000,0.000000,0.000000" "None" true))

(event EventTick
  (params (DeltaSeconds :type Float%20%28single-precision%29)))

(fn ConstructionScript)