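; RandomizeCorpses_BP is a set-dressing Blueprint that shows a corpse in one of four poses with a random scattering of bugs on it.
; Its Construction Script reveals the mesh selected by CorpsePose and builds a bug component array for each pose.
; A loop bounded by the clamped Bugs count reveals random entries from the matching array, removing each pick to avoid repeats.
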(fn ConstructionScript
  (Variables|Default|SetBugsSet_01 (Utilities|Array|MakeArray (Variables|Default|GetBug_01) (Variables|Default|GetBug_02) (Variables|Default|GetBug_03) (Variables|Default|GetBug_04) (Variables|Default|GetBug_05) (Variables|Default|GetBug_06) (Variables|Default|GetBug_07) (Variables|Default|GetBug_08) (Variables|Default|GetBug_09) (Variables|Default|GetBug_10)))
  (Variables|Default|SetBugsSet_02 (Utilities|Array|MakeArray (Variables|Default|GetPose_02_Bug_01) (Variables|Default|GetPose_02_Bug_02) (Variables|Default|GetPose_02_Bug_03) (Variables|Default|GetPose_02_Bug_04) (Variables|Default|GetPose_02_Bug_05) (Variables|Default|GetPose_02_Bug_06) (Variables|Default|GetPose_02_Bug_07) (Variables|Default|GetPose_02_Bug_08) (Variables|Default|GetPose_02_Bug_09) (Variables|Default|GetPose_02_Bug_10)))
  (Variables|Default|SetBugsSet_03 (Utilities|Array|MakeArray (Variables|Default|GetPose_03_Bug_01) (Variables|Default|GetPose_03_Bug_02) (Variables|Default|GetPose_03_Bug_03) (Variables|Default|GetPose_03_Bug_04) (Variables|Default|GetPose_03_Bug_05) (Variables|Default|GetPose_03_Bug_06) (Variables|Default|GetPose_03_Bug_07) (Variables|Default|GetPose_03_Bug_08) (Variables|Default|GetPose_03_Bug_09) (Variables|Default|GetPose_03_Bug_10)))
  (Variables|Default|SetBugsSet_04 (Utilities|Array|MakeArray (Variables|Default|Getpose_04_bug_01) (Variables|Default|Getpose_04_bug_02) (Variables|Default|Getpose_04_bug_03) (Variables|Default|Getpose_04_bug_04) (Variables|Default|Getpose_04_bug_05) (Variables|Default|Getpose_04_bug_06) (Variables|Default|Getpose_04_bug_07) (Variables|Default|Getpose_04_bug_08) (Variables|Default|Getpose_04_bug_09) (Variables|Default|Getpose_04_bug_10)))
  (Rendering|SetVisibility (Utilities|Select :Index (Math|Integer|Clamp(Integer) (Variables|Default|GetCorpsePose) 0 3) :Option%200 (Variables|Default|GetCorpse_01) :Option%201 (Variables|Default|GetCorpse_02) :Option%202 (Variables|Default|GetCorpse_03) :Option%203 (Variables|Default|GetCorpse_04)) true false)
  (for _index (range 0 (Math|Integer|Clamp(Integer) (Variables|Default|GetBugs) 0 9))
    (bind _output_get (LocalVariables|SetL_MeshIteration (.OutItem (Utilities|Array|Random (Utilities|Select :Index (Variables|Default|GetCorpsePose) :Option%200 (Variables|Default|GetBugsSet_01) :Option%201 (Variables|Default|GetBugsSet_02) :Option%202 (Variables|Default|GetBugsSet_03) :Option%203 (Variables|Default|GetBugsSet_04))))))
    (Rendering|SetVisibility _output_get true false)
    (Utilities|Array|RemoveItem (Utilities|Select :Index (Variables|Default|GetCorpsePose) :Option%200 (Variables|Default|GetBugsSet_01) :Option%201 (Variables|Default|GetBugsSet_02) :Option%202 (Variables|Default|GetBugsSet_03) :Option%203 (Variables|Default|GetBugsSet_04)) (LocalVariables|GetL_MeshIteration))))