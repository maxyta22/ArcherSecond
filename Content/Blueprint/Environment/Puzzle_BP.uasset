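; Puzzle_BP is an environment puzzle actor built around two child actor buttons, with only placeholder responses in place.
; On BeginPlay it casts each child actor to ButtonBase_BP and binds a separate custom event to it through BindEventToUseButton.
; Each event only prints a debug string identifying which button was activated, with no puzzle state or solve logic.
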(event Custom|ActivateOneButton
  (Development|PrintString "ACTIVATE1"))

(event Custom|ActivateTwoButton
  (Development|PrintString "ACTIVATE2"))

(event EventBeginPlay
  (EventDispatchers|BindEventtoUseButton (.AsButton%20Base%20BP (Utilities|Casting|CastToButtonBase_BP (Variables|/Script/Engine.ChildActorComponent|GetChildActor (Variables|Default|GetChildActor)))) (delegate Custom|ActivateOneButton))
  (EventDispatchers|BindEventtoUseButton (.AsButton%20Base%20BP (Utilities|Casting|CastToButtonBase_BP (Variables|/Script/Engine.ChildActorComponent|GetChildActor (Variables|Default|GetChildActor1)))) (delegate Custom|ActivateTwoButton)))

(fn ConstructionScript)