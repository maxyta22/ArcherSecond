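; Puzzle actor that hosts three button child actors and one interact object child actor, currently with placeholder responses only.
; On BeginPlay it casts each child to ButtonBase_BP or InteractObjectBase_BP and binds its own custom events to their use callbacks.
; Each button event prints its own debug message and the interact object prints a colored success message, with no puzzle state or ordering checks.
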(event Custom|ActivateOneButton
  (Development|PrintString "ACTIVATE1"))

(event Custom|ActivateTwoButton
  (Development|PrintString "ACTIVATE2"))

(event Custom|Flash
  (Development|PrintString "Success" true true "(R=0.367609,G=0.000000,B=1.000000,A=1.000000)"))

(event Custom|CustomEvent_0
  (Development|PrintString "ACTIVATE3"))

(event EventBeginPlay
  (EventDispatchers|BindEventtoUseButton (.AsButton%20Base%20BP (Utilities|Casting|CastToButtonBase_BP (Variables|/Script/Engine.ChildActorComponent|GetChildActor (Variables|Default|GetChildActor)))) (delegate Custom|ActivateOneButton))
  (EventDispatchers|BindEventtoUseButton (.AsButton%20Base%20BP (Utilities|Casting|CastToButtonBase_BP (Variables|/Script/Engine.ChildActorComponent|GetChildActor (Variables|Default|GetChildActor1)))) (delegate Custom|ActivateTwoButton))
  (EventDispatchers|BindEventtoUseButton (.AsButton%20Base%20BP (Utilities|Casting|CastToButtonBase_BP (Variables|/Script/Engine.ChildActorComponent|GetChildActor (Variables|Default|GetChildActor2)))) (delegate Custom|CustomEvent_0))
  (EventDispatchers|BindEventtoUseInteractObject (.AsInteract%20Object%20Base%20BP (Utilities|Casting|CastToInteractObjectBase_BP (Variables|/Script/Engine.ChildActorComponent|GetChildActor (Variables|Default|GetChildActor3)))) (delegate Custom|Flash)))

(fn ConstructionScript)