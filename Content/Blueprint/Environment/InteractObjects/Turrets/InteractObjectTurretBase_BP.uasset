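; Base interactable turret that tracks AI characters and fires projectiles at them.
; A detection sphere, sized from DetectRadius at construction, locks onto the first AI character to enter and releases it only when that target leaves, without rescanning those already inside.
; Tick turns the turret at constant speed on yaw only and fires once nearly aligned.
; A DoOnce and delay gate projectile spawns from the muzzle by SpeedAttackRate.
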(event OnComponentBeginOverlap(SphereDetect)
  (params (OverlappedComponent :type Primitive%20Component%20Object%20Reference) (OtherActor :type Actor%20Object%20Reference) (OtherComp :type Primitive%20Component%20Object%20Reference) (OtherBodyIndex :type Integer) (bFromSweep :type Boolean) (SweepResult :type Hit%20Result%20Structure%20%28by%20ref%29))
  (bind _asaicharacter_base_bp (Utilities|Casting|CastToAICharacterBase_BP OtherActor))
  (Utilities|FlowControl|DoOnce false
    (:Completed
      (Variables|Default|SetTargetEnemy _asaicharacter_base_bp))))

(event OnComponentEndOverlap(SphereDetect)
  (params (OverlappedComponent :type Primitive%20Component%20Object%20Reference) (OtherActor :type Actor%20Object%20Reference) (OtherComp :type Primitive%20Component%20Object%20Reference) (OtherBodyIndex :type Integer))
  (if (== OtherActor (Variables|Default|GetTargetEnemy))
    (Variables|Default|SetTargetEnemy 0)
    (Utilities|FlowControl|DoOnce false) ; enters at Reset
  ))

(event Custom|MakeShot
  (bind _muzzle (Variables|Default|GetMuzzle))
  (Utilities|FlowControl|DoOnce false :!label _label
    (:Completed
      (Game|SpawnActorfromClass "/Game/Blueprint/Projectile/ProjectileForTurret_BP.ProjectileForTurret_BP_C" (Math|Transform|MakeTransform (Transformation|GetWorldLocation _muzzle) (Transformation|GetWorldRotation _muzzle) "1.000000,1.000000,1.000000") "AlwaysSpawn" 0 0)
      (Utilities|FlowControl|Delay (Variables|Default|GetSpeedAttackRate))
      (goto _label Reset))))

(event EventTick
  (params (DeltaSeconds :type Float%20%28single-precision%29))
  (bind _returnvalue (Transformation|GetActorRotation))
  (bind (_roll _pitch) (Math|Rotator|BreakRotator _returnvalue))
  (|CallParentFunction DeltaSeconds)
  (Utilities|IsValid (Variables|Default|GetTargetEnemy)
    (:Is%20Valid
      (Utilities|FlowControl|Sequence
        (:then_0
          (Transformation|SetActorRotation (Class|KismetMathLibrary|RInterptoConstant _returnvalue (Math|Rotator|MakeRotator _roll _pitch (.Yaw (Math|Rotator|BreakRotator (Math|Rotator|FindLookatRotation (Transformation|GetActorLocation) (Transformation|GetActorLocation (Variables|Default|GetTargetEnemy)))))) (Utilities|Time|GetWorldDeltaSeconds) 3e+01)))
        (:then_1
          (if (Math|Float|NearlyEqual(Float) (.Yaw (Math|Rotator|BreakRotator (Math|Rotator|FindLookatRotation (Transformation|GetActorLocation) (Transformation|GetActorLocation (Variables|Default|GetTargetEnemy))))) (.Yaw (Math|Rotator|BreakRotator (Transformation|GetActorRotation))) 2.0)
            (CallFunction|MakeShot)))))))

(fn ConstructionScript
  (|CallParentFunction)
  (Components|Sphere|SetSphereRadius (Variables|Default|GetSphereDetect) (Variables|Default|GetDetectRadius) true))