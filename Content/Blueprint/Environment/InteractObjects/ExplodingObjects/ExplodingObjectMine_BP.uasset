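; Interactable mine, a child exploding object that the player can collect as a Mine resource.
; On interaction it adds one Mine to the player's InventoryComponent and destroys itself.
; On explosion it swaps the mesh material, then runs the parent explosion logic.
; Its "Mine" info widget uses a short retriggerable delay to stay visible only while ShowInfo keeps being called.
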(event EventPerformExplosion
  (Rendering|Material|SetMaterial (Variables|Default|GetStaticMeshComponent) 0 "/Game/ExternalContent/Cave/cave_test_01_Mesh/New_Meshes/Mine_Mat_Inst.Mine_Mat_Inst")
  (|CallParentFunction))

(event EventShowInfo
  (Rendering|SetVisibility (Variables|Default|GetWidget) true false)
  (Utilities|FlowControl|RetriggerableDelay 0.01)
  (Class|InteractObjectBase|HideInfo))

(event EventHideInfo
  (Rendering|SetVisibility (Variables|Default|GetWidget) false false))

(event EventBeginPlay
  (bind _aswidget_info_ui (Utilities|Casting|CastToWidgetInfo_UI (UserInterface|GetWidget (Variables|Default|GetWidget))))
  (Rendering|Components|TextRender|SetText (Variables|/Game/Blueprint/UI/WidgetInfo_UI.WidgetInfo_UI_C|GetName _aswidget_info_ui) "Mine"))

(event EventAfterWasTryUseInteractObject
  (bind _asplayer_character_bp (Utilities|Casting|CastToPlayerCharacter_BP (Game|GetPlayerCharacter 0)))
  (Class|InventoryComponent|AddResources (Variables|/Script/ArcherPRT.PlayerCharacter|GetInventoryComponent _asplayer_character_bp) "Mine" 1)
  (Actor|DestroyActor))

(fn ConstructionScript
  (|CallParentFunction))