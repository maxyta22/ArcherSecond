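; Base Chaos destructible actor that breaks when hit by a charged pneumatic glove or pneumatic gun, with optional explosion.
; A one-shot, delayed trigger swaps the static mesh for the destructible mesh, applies strain field and impulse, then later destroys the actor.
; The explosion uses async-loaded VFX and a sphere overlap to damage AI, player and damageable actors.
; Overlapped destructibles are triggered too, creating chain reactions.
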(event Custom|PerformExplosion
  (bind _returnvalue (Game|GetPlayerCharacter 0))
  (bind _returnvalue_2 (Transformation|GetActorLocation))
  ;[0.1022 0 1 1 60] Explosion
  (Utilities|FlowControl|Sequence
    (:then_0
      (bind _explosionvfx (Variables|Default|GetExplosionVFX)
        (:then
          (Effects|SpawnEmitteratLocation _explosionvfx _returnvalue_2 "0, 0, 0" "2.000000,2.000000,2.000000"))
        (:else
          _))
      (Audio|PlaySoundatLocation (Variables|DestructSettings|GetSoundExplosion) _returnvalue_2 "0, 0, 0" 1.0 1.0 0.0 0 0 0 0))
    (:then_1
      (bind _outactors (Collision|SphereOverlapActors (Transformation|GetActorLocation) (Variables|Default|GetExplosionRadius) (Utilities|Array|MakeArray "ObjectTypeQuery3" "ObjectTypeQuery2" "ObjectTypeQuery8") 0))
      (for _array_element _outactors
        (bind _asaicharacter (Utilities|Casting|CastToAICharacter _array_element)
          (:then
            (Class|GameCharacter|ImplementTakeDamage _asaicharacter (Utilities|Struct|MakeDamageData (* (Transformation|GetActorForwardVector) -1) "(FaceIndex=0,Time=1.000000,Distance=0.000000,Location=(X=0.000000,Y=0.000000,Z=0.000000),ImpactPoint=(X=0.000000,Y=0.000000,Z=0.000000),Normal=(X=0.000000,Y=0.000000,Z=0.000000),ImpactNormal=(X=0.000000,Y=0.000000,Z=0.000000),TraceStart=(X=0.000000,Y=0.000000,Z=0.000000),TraceEnd=(X=0.000000,Y=0.000000,Z=0.000000),PenetrationDepth=0.000000,MyItem=-1,Item=0,ElementIndex=0,bBlockingHit=False,bStartPenetrating=False,PhysMaterial=None,HitObjectHandle=(Actor=None),Component=None,BoneName=\"\",MyBoneName=\"\")" (Game|GetInstigatorController _returnvalue) _returnvalue "None" false true false "/Game/Blueprint/Abilities/GameplayEffects/Environment/DamageFromBarrelForEnemies_GE.DamageFromBarrelForEnemies_GE_C" 0)))
          (:CastFailed
            (bind _asplayer_character (Utilities|Casting|CastToPlayerCharacter _array_element)
              (:then
                (Class|GameCharacter|ImplementTakeDamage _asplayer_character (Utilities|Struct|MakeDamageData (* (Transformation|GetActorForwardVector _asplayer_character) -1) "(FaceIndex=0,Time=1.000000,Distance=0.000000,Location=(X=0.000000,Y=0.000000,Z=0.000000),ImpactPoint=(X=0.000000,Y=0.000000,Z=0.000000),Normal=(X=0.000000,Y=0.000000,Z=0.000000),ImpactNormal=(X=0.000000,Y=0.000000,Z=0.000000),TraceStart=(X=0.000000,Y=0.000000,Z=0.000000),TraceEnd=(X=0.000000,Y=0.000000,Z=0.000000),PenetrationDepth=0.000000,MyItem=-1,Item=0,ElementIndex=0,bBlockingHit=False,bStartPenetrating=False,PhysMaterial=None,HitObjectHandle=(Actor=None),Component=None,BoneName=\"\",MyBoneName=\"\")" (Game|GetInstigatorController _asplayer_character) self "None" false true false "/Game/Blueprint/Abilities/GameplayEffects/Environment/DamageFromBarrel_GE.DamageFromBarrel_GE_C" 0)))
              (:CastFailed
                (bind _asdestructable_object_base_bp (Utilities|Casting|CastToDestructableObjectBase_BP _array_element)
                  (:then
                    (CallFunction|TryPerformDestroyObject _asdestructable_object_base_bp "0, 0, 0"))
                  (:CastFailed
                    (if (Utilities|DoesObjectImplementInterface _array_element "/Script/ArcherPRT.TakeDamageInterface")
                      (Class|TakeDamageInterface|ITakeDamage(Message) _array_element (Utilities|Struct|MakeDamageData "0.000000,0.000000,0.000000" "(FaceIndex=0,Time=1.000000,Distance=0.000000,Location=(X=0.000000,Y=0.000000,Z=0.000000),ImpactPoint=(X=0.000000,Y=0.000000,Z=0.000000),Normal=(X=0.000000,Y=0.000000,Z=0.000000),ImpactNormal=(X=0.000000,Y=0.000000,Z=0.000000),TraceStart=(X=0.000000,Y=0.000000,Z=0.000000),TraceEnd=(X=0.000000,Y=0.000000,Z=0.000000),PenetrationDepth=0.000000,MyItem=-1,Item=0,ElementIndex=0,bBlockingHit=False,bStartPenetrating=False,PhysMaterial=None,HitObjectHandle=(Actor=None),Component=None,BoneName=\"\",MyBoneName=\"\")" 0 0 "None" false true false "/Game/Blueprint/Abilities/GameplayEffects/Environment/DamageFromBarrel_GE.DamageFromBarrel_GE_C" 0)))))))))))
    (:then_2
      (if (Variables|Default|GetDrawDebug)
        (Rendering|Debug|DrawDebugSphere (Transformation|GetActorLocation) (Variables|Default|GetExplosionRadius) 12 "(R=0.388978,G=1.000000,B=0.000000,A=1.000000)" 3.0 5.0)))))

(event Custom|TryPerformDestroyObject
  (params (Impulse :type Vector))
  (Variables|Internal|SetImpulse Impulse)
  (Utilities|FlowControl|DoOnce false
    (:Completed
      (Utilities|FlowControl|Delay (Variables|DestructSettings|GetTimeBeforeExplosion))
      (Utilities|FlowControl|Sequence
        (:then_0
          (CallFunction|PerformDestroy))
        (:then_1
          (if (Variables|DestructSettings|GetMakeExplosion)
            (CallFunction|PerformExplosion)))
        (:then_2
          (Utilities|FlowControl|Delay (Variables|Default|GetSelf_Destroy_Timer))
          (Actor|DestroyActor))))))

(event Custom|PerformDestroy
  (bind _staticmesh (Variables|Default|GetStaticMesh))
  (bind _destructablemesh (Variables|Default|GetDestructableMesh))
  (bind _destructablemesh_2 (Variables|Default|GetDestructableMesh))
  ;[0 0.3888 1 1 60] Destruct
  (Rendering|SetVisibility _staticmesh false false)
  (Collision|SetCollisionEnabled _staticmesh "NoCollision")
  (Rendering|SetVisibility _destructablemesh true false)
  (Collision|SetCollisionEnabled _destructablemesh "QueryAndPhysics")
  (Utilities|FlowControl|Sequence
    (:then_0
      (Audio|PlaySoundatLocation (Variables|DestructSettings|GetDestructSound) (Transformation|GetActorLocation) "0, 0, 0" 1.0 1.0 0.0 0 0 0 0)
      (Niagara|SpawnSystematLocation (Variables|DestructSettings|GetDestructVFX) (Transformation|GetActorLocation) (Transformation|GetActorRotation)))
    (:then_1
      (Class|FieldSystemComponent|ApplyPhysicsField (Variables|Default|GetFieldSystem) true "Field_ExternalClusterStrain" 0 (Field|SetRadialFalloff (Variables|Default|GetRadialFalloff) 1e+02 0.0 1.0 0.0 (Variables|DestructSettings|GetDestructRadius) (Transformation|GetWorldLocation (Variables|Default|GetDestructableMesh)) "Field_FallOff_None"))
      (if (Variables|DestructSettings|GetRadialImpulse)
        (Physics|AddRadialImpulse _destructablemesh_2 (Transformation|GetWorldLocation _destructablemesh_2) (Variables|DestructSettings|GetDestructRadius) (Math|Conversions|ToFloat(Integer) (Variables|DestructSettings|GetPowerImpulse)) "RIF_Constant" false)
        (else
          (Physics|AddImpulse _destructablemesh_2 (* (Variables|Internal|GetImpulse) (Variables|DestructSettings|GetPowerImpulse)) "None" true))))
    (:then_2
      (Audio|PlaySoundatLocation (Variables|DestructSettings|GetSoundExplosion) (Transformation|GetActorLocation) "0, 0, 0" 1.0 1.0 0.0 0 0 0 0))))

(event EventBeginPlay
  (bind _softexplosionpath (Variables|Default|GetSoftExplosionPath))
  ;[0 0.7423 1 1 60] Begin Play
  (|CallParentFunction)
  (Utilities|FlowControl|Sequence
    (:then_0
      (Rendering|SetVisibility (Variables|Default|GetDestructableMesh) false false)
      (Rendering|SetVisibility (Variables|Default|GetStaticMesh) true false))
    (:then_1
      (if (Utilities|IsValidSoftObjectReference _softexplosionpath)
        (bind _object (Utilities|AsyncLoadAsset _softexplosionpath)
          (:Completed
            (bind _asparticle_system (Utilities|Casting|CastToParticleSystem _object))
            (Variables|Default|SetExplosionVFX _asparticle_system)))))))

(event EventAfterWasTryUseInteractObject)

(event EventITakeDamage
  (params (DamageData :type Damage%20Data%20Structure))
  (bind (_damagedirection _damagepoint _damageinstigator _damagecauser _damageweapontype _damagecharged) (Utilities|Struct|BreakDamageData DamageData))
  (bind (_bblockinghit _binitialoverlap _time _distance _location _impactpoint _normal _impactnormal _physmat _hitactor _hitcomponent _hitbonename _bonename _hititem _elementindex _faceindex _tracestart _traceend) (Collision|BreakHitResult _damagepoint))
  ;[0.2788 0 1 1 60] Interact from weapon
  (switch Utilities|FlowControl|Switch|SwitchonEWeaponType _damageweapontype
    (:PneumaticGlove
      (if _damagecharged
        (CallFunction|TryPerformDestroyObject (Math|Vector|GetUnitDirection(Vector) _tracestart _traceend))))
    (:PneumaticGun
      (CallFunction|TryPerformDestroyObject (Transformation|GetActorForwardVector _damagecauser)))))

(event EventAfterWasSuccessUseInteractObject)

(fn ConstructionScript)