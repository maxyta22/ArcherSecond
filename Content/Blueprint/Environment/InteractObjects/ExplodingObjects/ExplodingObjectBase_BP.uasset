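; Base Blueprint for an exploding environment object that detonates once, after a delay, when an AI character or archer projectile overlaps its hit box.
; The blast spawns effects and sound, damages AI characters in a sphere, triggers bug explosions and chain-detonates nearby exploding objects.
; It swaps the static mesh for a Geometry Collection, fractures it with a strain field, pushes it along any projectile's direction, then destroys itself.
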(event OnComponentBeginOverlap(BoxHitCollider)
  (params (OverlappedComponent :type Primitive%20Component%20Object%20Reference) (OtherActor :type Actor%20Object%20Reference) (OtherComp :type Primitive%20Component%20Object%20Reference) (OtherBodyIndex :type Integer) (bFromSweep :type Boolean) (SweepResult :type Hit%20Result%20Structure%20%28by%20ref%29))
  (bind (_bblockinghit _binitialoverlap _time _distance _location _impactpoint _normal _impactnormal _physmat _hitactor _hitcomponent _hitbonename _bonename _hititem _elementindex _faceindex _tracestart _traceend) (Collision|BreakHitResult SweepResult))
  (Utilities|Casting|CastToAICharacter OtherActor
    (:then
      (CallFunction|PerformExplosion))
    (:CastFailed
      (Utilities|Casting|CastToArcherPRTProjectile OtherActor)
      (Variables|Default|SetImpulseDirection (Math|Vector|GetUnitDirection(Vector) _tracestart _traceend))
      (CallFunction|PerformExplosion))))

(event Custom|PerformExplosion
  (bind _returnvalue (Transformation|GetActorLocation))
  (bind _geometrycollection (Variables|Default|GetGeometryCollection))
  ;[0.1785 0 1 1 60] Perform Explosion
  (Utilities|FlowControl|DoOnce false
    (:Completed
      (Utilities|FlowControl|Delay (Variables|Default|GetTimeBeforeExplosion))
      (Utilities|FlowControl|Sequence
        (:then_0
          (Effects|SpawnEmitteratLocation "/Game/StarterContent/Particles/P_Explosion.P_Explosion" _returnvalue "0, 0, 0" "2.000000,2.000000,2.000000")
          (Audio|PlaySoundatLocation "/Game/Characters/Walking_House/sounds/Explosion01.Explosion01" _returnvalue "0, 0, 0" 1.0 1.0 0.0 0 0 0 0))
        (:then_1
          (bind _outactors (Collision|SphereOverlapActors (Transformation|GetActorLocation) (Variables|Default|GetExplosionRadius) (Utilities|Array|MakeArray "ObjectTypeQuery3" "ObjectTypeQuery2") 0))
          (for _array_element _outactors
            (bind _asaicharacter_bug_base_bp (Utilities|Casting|CastToAICharacterBugBase_BP _array_element)
              (:then
                (Default|PerformBugExplosion _asaicharacter_bug_base_bp 0.0)
                (Game|Damage|ApplyDamage _asaicharacter_bug_base_bp (Variables|Default|GetDamage) 0 (Game|GetPlayerCharacter 0))
                (Class|AICharacter|PerformonHitReaction _asaicharacter_bug_base_bp (Utilities|Struct|MakeDamageData "0.000000,0.000000,0.000000" "(FaceIndex=0,Time=1.000000,Distance=0.000000,Location=(X=0.000000,Y=0.000000,Z=0.000000),ImpactPoint=(X=0.000000,Y=0.000000,Z=0.000000),Normal=(X=0.000000,Y=0.000000,Z=0.000000),ImpactNormal=(X=0.000000,Y=0.000000,Z=0.000000),TraceStart=(X=0.000000,Y=0.000000,Z=0.000000),TraceEnd=(X=0.000000,Y=0.000000,Z=0.000000),PenetrationDepth=0.000000,MyItem=-1,Item=0,ElementIndex=0,bBlockingHit=False,bStartPenetrating=False,PhysMaterial=None,HitObjectHandle=(Actor=None),Component=None,BoneName=\"\",MyBoneName=\"\")" 0 (Game|GetPlayerCharacter 0))))
              (:CastFailed
                (bind _asaicharacter (Utilities|Casting|CastToAICharacter _array_element)
                  (:then
                    (Game|Damage|ApplyDamage _asaicharacter (Variables|Default|GetDamage) 0 0))
                  (:CastFailed
                    (bind _asexploding_object_base_bp (Utilities|Casting|CastToExplodingObjectBase_BP _array_element))
                    (CallFunction|PerformExplosion _asexploding_object_base_bp)))))))
        (:then_2
          (if (Variables|Default|GetDrawDebug)
            (Rendering|Debug|DrawDebugSphere (Transformation|GetActorLocation) (Variables|Default|GetExplosionRadius) 12 "(R=0.388978,G=1.000000,B=0.000000,A=1.000000)" 3.0 5.0)))
        (:then_3
          (Utilities|IsValid (Variables|Default|GetGeometryCollection)
            (:Is%20Valid
              (Rendering|SetVisibility (Variables|Default|GetStaticMeshComponent) false false)
              (Rendering|SetVisibility (Variables|Default|GetGeometryCollection) true false)
              (Collision|SetCollisionEnabled (Variables|Default|GetBoxHitCollider) "NoCollision")
              (Collision|SetCollisionEnabled _geometrycollection "PhysicsOnly")
              (Physics|SetSimulatePhysics _geometrycollection true)
              (Class|FieldSystemComponent|ApplyPhysicsField (Variables|Default|GetFieldSystem) true "Field_ExternalClusterStrain" 0 (Field|SetRadialFalloff (Variables|Default|GetRadialFalloff) 5e+01 0.0 1.0 0.0 1e+02 (Transformation|GetWorldLocation (Variables|Default|GetGeometryCollection)) "Field_FallOff_None"))
              (Physics|AddImpulse (Variables|Default|GetGeometryCollection) (* (Variables|Default|GetImpulseDirection) 400) "None" true))))
        (:then_4
          (Utilities|FlowControl|Delay 5.0)
          (Actor|DestroyActor))))))

(event EventBeginPlay
  (|CallParentFunction)
  (Rendering|SetVisibility (Variables|Default|GetGeometryCollection) false false))

(fn ConstructionScript)