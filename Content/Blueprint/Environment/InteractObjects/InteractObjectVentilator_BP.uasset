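; Interactable ventilator that a successful use toggles on and off, acting as a hazard for AI bug characters.
; While active, Tick spins the static mesh by a fixed world-rotation step each frame, not scaled by delta time.
; Bug characters that begin overlapping the box collision while it is active are told to explode; those already inside when it switches on are not checked.
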(event OnComponentBeginOverlap(BoxGabaritCollision)
  (params (OverlappedComponent :type Primitive%20Component%20Object%20Reference) (OtherActor :type Actor%20Object%20Reference) (OtherComp :type Primitive%20Component%20Object%20Reference) (OtherBodyIndex :type Integer) (bFromSweep :type Boolean) (SweepResult :type Hit%20Result%20Structure%20%28by%20ref%29))
  (if (Variables|Default|GetActive)
    (bind _asaicharacter_bug_base_bp (Utilities|Casting|CastToAICharacterBugBase_BP OtherActor))
    (Default|PerformBugExplosion _asaicharacter_bug_base_bp)))

(event EventTick
  (params (DeltaSeconds :type Float%20%28single-precision%29))
  (|CallParentFunction DeltaSeconds)
  (if (Variables|Default|GetActive)
    (Transformation|AddWorldRotation (Variables|Default|GetStaticMeshComponent) "0.000000,30.000000,0.000000" false false)))

(event EventAfterWasSuccessUseInteractObject
  (Variables|Default|SetActive (not (Variables|Default|GetActive))))

(fn ConstructionScript
  (|CallParentFunction))