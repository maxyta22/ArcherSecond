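; An interactive propeller hazard actor that damages actors overlapping its Box collision through the Gameplay Ability System.
; On overlap it sends a Damage.Propeller gameplay event to the actor and fires the PlayerHitFromPropeller gameplay cue on it.
; It then applies DamageFromPropeller_GE from its own ability system component to the victim's.
; A DoOnce, reset after a one-second delay, throttles hits globally rather than per overlapping actor.
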(event OnComponentBeginOverlap(Box)
  (params (OverlappedComponent :type Primitive%20Component%20Object%20Reference) (OtherActor :type Actor%20Object%20Reference) (OtherComp :type Primitive%20Component%20Object%20Reference) (OtherBodyIndex :type Integer) (bFromSweep :type Boolean) (SweepResult :type Hit%20Result%20Structure%20%28by%20ref%29))
  (bind _returnvalue (Ability|TargetData|AbilityTargetDatafromActor OtherActor))
  (bind _self self)
  (bind _self_2 self)
  (bind _abilitysystem (Variables|Default|GetAbilitySystem))
  (bind _returnvalue_2 (GameplayEffects|MakeEffectContext _abilitysystem))
  (bind _gameplayeventdata (Utilities|Struct|MakeGameplayEventData "(TagName=\"Damage.Propeller\")" _self_2 OtherActor 0 0 _returnvalue_2 "(GameplayTags=)" "(GameplayTags=)" 1.0 _returnvalue))
  (bind (_eventtag _instigator _target _optionalobject _optionalobject2 _contexthandle) (Utilities|Struct|BreakGameplayEventData _gameplayeventdata))
  (Utilities|FlowControl|DoOnce false :!label _label
    (:Completed
      (Utilities|FlowControl|Sequence
        (:then_0
          (Ability|SendGameplayEventtoActor OtherActor "(TagName=\"Damage.Propeller\")" _gameplayeventdata)
          (GameplayCue|ExecuteGameplayCueOnActor(Burst) _target "(TagName=\"GameplayCue.PlayerHitFromPropeller\")" (Ability|GameplayCue|MakeGameplayCueParameters :EffectContext _contexthandle :Instigator _self :EffectCauser _self :SourceObject (Variables|Default|GetAbilitySystem)))
          (GameplayEffects|ApplyGameplayEffectToTarget (Ability|GetAbilitySystemComponent self) "/Game/Blueprint/Abilities/GameplayEffects/DamageFromPropeller_GE.DamageFromPropeller_GE_C" (Ability|GetAbilitySystemComponent _target) 1.0 _contexthandle))
        (:then_1
          (Utilities|FlowControl|Delay 1.0)
          (goto _label Reset))))))

(fn ConstructionScript)