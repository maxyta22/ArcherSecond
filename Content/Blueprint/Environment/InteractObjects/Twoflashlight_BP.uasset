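; Interactable floodlight that toggles on and off each time it is used.
; A FlipFlop after the parent interaction swaps lamp and glass materials, sets SpotLight intensity and updates ActiveLight.
; Switching on plays a neon start sound, then an idle sound after a delay; switching off only assigns a sound without playing or stopping it.
; It fetches the Cave_5_Platforming_02 actor, but the LigthsCount check on it is disconnected.
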(event EventAfterWasTryUseInteractObject
  (bind _staticmeshcomponent (Variables|Default|GetStaticMeshComponent))
  (bind _spotlight (Variables|Default|GetSpotLight))
  (bind _button_sound (Variables|Default|GetButton_sound))
  (|CallParentFunction)
  (bind _returnvalue (Actor|GetActorOfClass "/Game/Blueprint/Environment/New_Puzzles/Cave_5_Platforming_02.Cave_5_Platforming_02_C"))
  (Utilities|FlowControl|FlipFlop
    (:A
      (Rendering|Material|SetMaterial _staticmeshcomponent 0 "/Game/Underground_Bunker/Materials/Instances/MI_FloodLight_on_01.MI_FloodLight_on_01")
      (Rendering|Material|SetMaterial _staticmeshcomponent 1 "/Game/Underground_Bunker/Materials/Glass/MI_Glass_illuminated_Cool_01.MI_Glass_illuminated_Cool_01")
      (Variables|Default|Setactive_light true)
      (Rendering|Components|Light|SetIntensity _spotlight 5.0)
      (Audio|Components|Audio|SetSound _button_sound "/Game/ExternalContent/sounds/Buttons_Lights/Neon_light_on_Start.Neon_light_on_Start")
      (Audio|Components|Audio|Play _button_sound 0.0)
      (Utilities|FlowControl|Delay 1.4)
      (Audio|Components|Audio|SetSound _button_sound "/Game/ExternalContent/sounds/Buttons_Lights/Neon_Idle_Que.Neon_Idle_Que")
      (Audio|Components|Audio|Play _button_sound 0.0))
    (:B
      (Rendering|Material|SetMaterial _staticmeshcomponent 0 "/Game/Underground_Bunker/Materials/Instances/MI_FloodLight_off_01.MI_FloodLight_off_01")
      (Rendering|Material|SetMaterial _staticmeshcomponent 1 "/Game/Underground_Bunker/Materials/Glass/MI_Glass_illuminated_Warm_01l.MI_Glass_illuminated_Warm_01l")
      (Variables|Default|Setactive_light false)
      (Rendering|Components|Light|SetIntensity _spotlight 0.0)
      (Audio|Components|Audio|SetSound _button_sound "/Game/ExternalContent/sounds/Buttons_Lights/Neon_light_on_Start_Que.Neon_light_on_Start_Que"))))

(fn ConstructionScript
  (|CallParentFunction))