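; Interactable pickup for the Pneumatic Gun that gives the player this weapon.
; On BeginPlay it sets the name text on its info widget to the gun's name.
; After an interaction attempt it adds its default range weapon to the player character's weapon component and switches the player to it, building on parent class behavior.
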(event EventAfterWasTryUseInteractObject
  (|CallParentFunction)
  (bind _asplayer_character_bp (Utilities|Casting|CastToPlayerCharacter_BP (Game|GetPlayerCharacter 0)))
  (Utilities|Array|Add (Variables|/Script/ArcherPRT.WeaponComponent|GetAvailableWeapons (Variables|/Script/ArcherPRT.GameCharacter|GetWeaponComponent _asplayer_character_bp)) "/Game/Blueprint/Weapon/DefaultRangeWeapon.DefaultRangeWeapon_C")
  (Default|SwitchWeapon _asplayer_character_bp "/Game/Blueprint/Weapon/DefaultRangeWeapon.DefaultRangeWeapon_C"))

(event EventBeginPlay
  (|CallParentFunction)
  (bind _aswidget_info_ui (Utilities|Casting|CastToWidgetInfo_UI (UserInterface|GetWidget (Variables|Default|GetWidget))))
  (Variables|/Script/UMG.TextBlock|SetText (Variables|/Game/Blueprint/UI/WidgetInfo_UI.WidgetInfo_UI_C|GetName _aswidget_info_ui) "Pneumatic Gun"))

(fn ConstructionScript
  (|CallParentFunction))