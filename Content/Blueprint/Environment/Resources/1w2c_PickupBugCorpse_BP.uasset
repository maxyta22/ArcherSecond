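; Bug corpse resource pickup Blueprint that labels itself and its contents through an info widget.
; On BeginPlay it sets the WidgetInfo_UI name to "Bug Corpse" and fills the widget's text array.
; It then loops over the ResourcesList map, writing each resource enum and amount into a matching list line.
; The construction script only calls its parent, and the file contains no pickup logic.
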(event EventBeginPlay
  (Utilities|FlowControl|Sequence
    (:then_0
      (bind _aswidget_info_ui (Utilities|Casting|CastToWidgetInfo_UI (UserInterface|GetWidget (Variables|Default|GetWidget))))
      (Rendering|Components|TextRender|SetText (Variables|/Game/Blueprint/UI/WidgetInfo_UI.WidgetInfo_UI_C|GetName _aswidget_info_ui) "Bug Corpse"))
    (:then_1
      (bind _aswidget_info_ui_2 (Utilities|Casting|CastToWidgetInfo_UI (UserInterface|GetWidget (Variables|Default|GetWidget))))
      (Default|FillTextArray _aswidget_info_ui_2)
      (bind _keys (Utilities|Map|Keys (Variables|Default|GetResourcesList)))
      (for (_array_element _array_index) _keys
        (bind _aswidget_info_ui_3 (Utilities|Casting|CastToWidgetInfo_UI (UserInterface|GetWidget (Variables|Default|GetWidget))))
        (Rendering|Components|TextRender|SetText (Utilities|Array|Get(acopy) (Variables|/Game/Blueprint/UI/WidgetInfo_UI.WidgetInfo_UI_C|GetListText _aswidget_info_ui_3) _array_index) (Utilities|Text|ToText(String) (Utilities|String|Append (Utilities|String|EnumtoString _array_element) "  -  " (Utilities|String|ToString(Integer) (.Value (Utilities|Map|Find (Variables|Default|GetResourcesList) _array_element))))))))))

(fn ConstructionScript
  (|CallParentFunction))