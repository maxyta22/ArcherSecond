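; Base Blueprint for an interactable environment button that shows a name label and fires when used.
; On BeginPlay it writes NameButton into the WidgetInfo_UI hosted by its widget component.
; ShowInfo and HideInfo toggle that widget's visibility, and AfterWasTryUseInteractObject forwards the interaction to CallUseButton.
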(event EventAfterWasTryUseInteractObject
  (Default|CallUseButton))

(event EventShowInfo
  (Rendering|SetVisibility (Variables|Default|GetWidget) true false))

(event EventHideInfo
  (Rendering|SetVisibility (Variables|Default|GetWidget) false false))

(event EventBeginPlay
  (bind _aswidget_info_ui (Utilities|Casting|CastToWidgetInfo_UI (UserInterface|GetWidget (Variables|Default|GetWidget))))
  (Rendering|Components|TextRender|SetText (Variables|/Game/Blueprint/UI/WidgetInfo_UI.WidgetInfo_UI_C|GetName _aswidget_info_ui) (Utilities|Text|ToText(String) (Variables|Default|GetNameButton))))

(fn ConstructionScript)