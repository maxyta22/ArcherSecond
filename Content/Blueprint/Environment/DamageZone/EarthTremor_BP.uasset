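; Earth tremor damage zone that runs a requested number of waves and sends a finish gameplay event to BossBug when done.
; Each wave plays a timeline, rate-scaled by TimeWave, that drives the idle VFX velocity and restarts itself until the count is reached.
; The timeline's Damage event track fires the damage VFX and applies damage to GameCharacter actors overlapping the Box.
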(event Custom|MakeDamage
  ;[0.3192 0 1 1 60] Damage
  (Utilities|FlowControl|Sequence
    (:then_0
      (Components|Activation|Activate (Variables|Default|GetDamageVFX) true))
    (:then_1
      (for _array_element (Collision|GetOverlappingActors (Variables|Default|GetBox) "/Script/ArcherPRT.GameCharacter" :!class /Script/Engine.PrimitiveComponent)
        (bind _asgame_character (Utilities|Casting|CastToGameCharacter _array_element))
        (Game|Damage|ApplyDamage _asgame_character (Variables|Default|GetDamage) 0 _array_element)))))

(event Custom|StartEarthTremor
  (params (WaveCount :type Integer))
  ;[0 1 0.9531 1 60] Actavate/Deactivate
  (Variables|Default|SetNeedWaveCount WaveCount)
  (Variables|Internal|SetWaveCount 0)
  (CallFunction|ActivateEarthTremor))

(event Custom|ActivateEarthTremor
  (bind _idlevfx (Variables|Default|GetIdleVFX))
  ;[0 1 0.9531 1 60] Actavate/Deactivate
  (Components|Activation|Activate (Variables|Default|GetIdleVFX) true)
  (Components|Timeline|SetPlayRate (Variables|Default|GetEarthTremorTimeline) (/ 1.0 (Variables|Default|GetTimeWave)))
  (bind _min_vel (Timeline|EarthTremorTimeline PlayFromStart)
    (:Update
      (Effects|Components|ParticleSystem|SetFloatParameter _idlevfx "Max_Velocity" _min_vel)
      (Effects|Components|ParticleSystem|SetFloatParameter _idlevfx "Min_Velocity" _min_vel))
    (:Finished
      (bind _result (Math|Integer|IncrementInt (Variables|Internal|GetWaveCount))
        (:%20%20
          (if (>= _result (Variables|Default|GetNeedWaveCount))
            (Components|Activation|Deactivate (Variables|Default|GetIdleVFX))
            (Ability|SendGameplayEventtoActor (Variables|Default|GetBossBug) "(TagName=\"Gameplay.FinishEarthTremor\")")
            (else
              (CallFunction|ActivateEarthTremor))))))
    (:Damage
      (CallFunction|MakeDamage))))

(fn ConstructionScript)