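; AICharacterBugHideRange_BP is a ranged bug AI character that extends its parent's main attack.
; On attack, it runs the parent logic, then plays an Emissive timeline that drives glow on/off and power parameters on the mesh materials.
; It also grants and immediately activates a one-shot Gameplay Ability, LockAIBehaviorTeleportForRangeBug_GA, through its Ability System Component.
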(event EventPerformMainAttack
  (bind _mesh (Variables|Character|GetMesh))
  (|CallParentFunction)
  (Utilities|FlowControl|Sequence
    (:then_0
      (bind (_direction _on_off _emissive_value) (Timeline|Emissive PlayFromStart)
        (:Update
          (Rendering|Material|SetScalarParameterValueonMaterials _mesh "Emissive_On" _on_off)
          (Rendering|Material|SetScalarParameterValueonMaterials _mesh "Emissive_Power" _emissive_value))))
    (:then_1
      (Class|AbilitySystemComponent|GiveAbilityandActivateOnce (Ability|GetAbilitySystemComponent self) "/Game/Blueprint/Abilities/AI/LockAIBehaviorTeleportForRangeBug_GA.LockAIBehaviorTeleportForRangeBug_GA_C" 0 -1))))

(fn ConstructionScript
  (|CallParentFunction))