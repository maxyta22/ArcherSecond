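; Gun bug enemy AI variant, named as a practice version, that runs with horde mode enabled.
; BeginPlay calls the parent logic, then sets the HordeMode flag; everything else relies on the parent class.
; The AfteronDeath event stops the idle and bug sound components, waits briefly, then destroys the actor.
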(event EventBeginPlay
  (|CallParentFunction)
  (Variables|Default|Sethorde_Mode true))

(event Collision|EventActorBeginOverlap
  (params (OtherActor :type Actor%20Object%20Reference)))

(event EventTick
  (params (DeltaSeconds :type Float%20%28single-precision%29))
  (|CallParentFunction DeltaSeconds) ; This node is disabled and will not be called.\nDrag off pins to build functionality.
)

(event EventAfteronDeath
  (Audio|Components|Audio|Stop (Variables|Default|GetMonster_Idle_2_Cue))
  (Utilities|FlowControl|Delay 2.0)
  (Actor|DestroyActor))

(fn ConstructionScript
  (|CallParentFunction))