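; AICharacterBugRange_BP is the ranged bug enemy AI character, attacking by shooting projectiles.
; Its main attack plays the shoot montage while an Emissive timeline drives emissive on and power parameters on the mesh materials.
; A separate MakeShot event spawns an EnemyProjectileBase_BP at ShotPoint, rotated toward the enemy held by its AI controller.
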(event EventPerformMainAttack
  (bind _mesh (Variables|Character|GetMesh))
  (Animation|PlayAnimMontage "/Game/ExternalContent/New_Enemy/Bug_enemy/Bug_Enemy_Test/Animations/Bug_Enemy_Shoot_Montage.Bug_Enemy_Shoot_Montage" 1.0 "None")
  (bind (_direction _on_off _emissive_value) (Timeline|Emissive PlayFromStart)
    (:Update
      (Rendering|Material|SetScalarParameterValueonMaterials _mesh "Emissive_On" _on_off)
      (Rendering|Material|SetScalarParameterValueonMaterials _mesh "Emissive_Power" _emissive_value))))

(event EventMakeShot
  (bind _shotpoint (Variables|Default|GetShotPoint))
  (bind _returnvalue (Transformation|GetWorldLocation _shotpoint))
  (Game|SpawnActorfromClass "/Game/Blueprint/Projectile/EnemyProjectileBase_BP.EnemyProjectileBase_BP_C" (Math|Transform|MakeTransform _returnvalue (Math|Rotator|FindLookatRotation _returnvalue (Transformation|GetActorLocation (Class|PRTAIController|GetEnemy (Class|AICharacter|GetAIControllerRef)))) "1.000000,1.000000,1.000000") "AlwaysSpawn" 0 0))

(fn ConstructionScript
  (|CallParentFunction))