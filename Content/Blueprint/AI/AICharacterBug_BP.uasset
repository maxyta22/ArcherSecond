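; AI bug character that latches onto AICharacterBodyForBugs_BP hosts.
; A looping timer searches nearby pawns for a host with a free socket, then PerformAttach snaps mesh and actor onto it and reserves that socket.
; While attached, hits are forwarded to the host; at near-zero health the bug frees its socket, detaches and launches as a physics body.
; A timeline-driven jump to the host's head is present but unwired.
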(event Custom|Rise
  (bind _mesh (Variables|Character|GetMesh))
  (bind _returnvalue (Transformation|GetWorldLocation _mesh))
  ;[1 0 0.5232 1 60] Rise
  (Transformation|SetActorLocation (Math|Vector|MakeVector (.x _returnvalue) (.y _returnvalue) (.z (Transformation|GetActorLocation))) false false))

(event Custom|FindBodyForAttach
  (bind _outactors (Collision|SphereOverlapActors (Transformation|GetActorLocation) 2e+03 (Utilities|Array|MakeArray "ObjectTypeQuery3") "/Game/Blueprint/AI/AICharacterBodyForBugs_BP.AICharacterBodyForBugs_BP_C"))
  (for _array_element _outactors
    (bind _asaicharacter_body_for_bugs_bp (Utilities|Casting|CastToAICharacterBodyForBugs_BP _array_element))
    (Variables|Default|SetCurrentAttachBody _asaicharacter_body_for_bugs_bp))
  (Utilities|IsValid (Variables|Default|GetCurrentAttachBody)
    (:Is%20Valid
      (bind (_hasavaliablesocket _avaliablesocket) (Default|FindAvaliableSocketforBug (Variables|Default|GetCurrentAttachBody)))
      (if _hasavaliablesocket
        (CallFunction|PerformAttach (Variables|Default|GetCurrentAttachBody) false _avaliablesocket)
        (Utilities|Time|ClearandInvalidateTimerbyHandle (Variables|Default|GetFindBodyForAttachTimer))))))

(event EventTick
  (params (DeltaSeconds :type Float%20%28single-precision%29))
  (bind _mesh (Variables|Character|GetMesh))
  (bind _returnvalue (Transformation|GetWorldLocation _mesh))
  (|CallParentFunction DeltaSeconds)
  (Transformation|SetWorldLocation (Variables|Default|GetTextRender) (Math|Vector|MakeVector (.x _returnvalue) (.y _returnvalue) (+ (.z _returnvalue) 5e+01)) false false))

(event EventBeginPlay
  (|CallParentFunction)
  (bind _returnvalue (Utilities|Time|SetTimerbyEvent (EventDispatchers|CreateEvent :!event Custom|FindBodyForAttach) 3.0 true))
  (Variables|Default|SetFindBodyForAttachTimer _returnvalue))

(event EventPerformonHitReaction
  (params (HitDirection :type Vector :default "0, 0, 0") (HitComponent :type Primitive%20Component%20Object%20Reference) (WeaponType :type EWeaponType%20Enum :default "None") (Charged :type Boolean))
  (bind _mesh (Variables|Character|GetMesh))
  ;[0 0.05011 1 1 60] HitReaction
  (if (< (Class|StatsComponent|GetHealth (Variables|Default|GetStatsComponent)) 0.1)
    (Utilities|IsValid (Variables|Default|GetCurrentAttachBody)
      (:Is%20Valid
        (Default|MakeAvaliableSocket (Variables|Default|GetCurrentAttachBody) (Variables|Default|GetCurrentAttachSocket))
        (Variables|Default|SetCurrentAttachBody 0)
        (Components|SkinnedMesh|SetLeaderPoseComponent _mesh 0 true false)
        (Transformation|SetWorldLocation _mesh (Transformation|GetWorldLocation HitComponent) false false)
        (Transformation|DetachFromActor "KeepWorld" "KeepWorld" "KeepRelative")
        (Collision|SetCollisionEnabled _mesh "PhysicsOnly")
        (Class|PrimitiveComponent|SetAllMassScale _mesh 5e+01)
        (Physics|SetSimulatePhysics _mesh true)
        (Physics|AddImpulse _mesh (* HitDirection 2000) "None" true)))
    (else
      (Utilities|IsValid (Variables|Default|GetCurrentAttachBody)
        (:Is%20Valid
          (Class|AICharacter|PerformonHitReaction (Variables|Default|GetCurrentAttachBody) HitDirection HitComponent WeaponType Charged))))))

(fn ConstructionScript
  (|CallParentFunction))

(fn PerformAttach
  (params (BodyForAttach :type AI%20Character%20Body%20for%20Bugs%20BP%20Object%20Reference) (UseAttachBodyForLeaderPose :type Boolean) (SocketName :type Name))
  (Utilities|IsValid BodyForAttach
    (:Is%20Valid
      (Utilities|FlowControl|Sequence
        (:then_0
          (if UseAttachBodyForLeaderPose
            (Components|SkinnedMesh|SetLeaderPoseComponent (Variables|Character|GetMesh) (Variables|/Script/Engine.Character|GetMesh BodyForAttach) true false)
            (else
              (Transformation|AttachComponentToComponent (Variables|Character|GetMesh) (Variables|/Script/Engine.Character|GetMesh BodyForAttach) SocketName "SnapToTarget" "SnapToTarget" "KeepRelative" true))))
        (:then_1
          (Collision|SetCollisionEnabled (Variables|Default|GetCapsuleComponent) "NoCollision"))
        (:then_2
          (Transformation|SetActorLocationAndRotation (Transformation|GetActorLocation BodyForAttach) (Transformation|GetActorRotation BodyForAttach))
          (Transformation|AttachActorToActor BodyForAttach "None" "SnapToTarget" "SnapToTarget" "KeepRelative" true))
        (:then_3
          (Default|MakeUnavaliableSocket BodyForAttach SocketName)
          (Variables|Default|SetCurrentAttachSocket SocketName))
        (:then_4
          (Variables|Default|SetAttached true))))))