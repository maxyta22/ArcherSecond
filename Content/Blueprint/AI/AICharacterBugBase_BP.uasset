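; Base AI bug enemy that can latch onto a nearby host body, follow a spline or explode in a suicide attack.
; Attach, detach, explosion and hit reactions trigger one-shot Gameplay Abilities, while PerformAttach handles mesh/actor attachment and socket occupancy.
; Hits on attached bugs pass to the host, and death frees the socket and detaches.
; The notify-driven blast damages nearby characters and chain-detonates other bugs after a short delay.
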(event Custom|DetachFromBody
  (params (Direction :type Vector))
  ;[0 0.1032 1 1 60] Detach From Body
  (Variables|Default|SetDetachDirection Direction)
  (Class|AbilitySystemComponent|GiveAbilityandActivateOnce (Ability|GetAbilitySystemComponent self) "/Game/Blueprint/Abilities/PerformDetachBug_GA.PerformDetachBug_GA_C" 0 -1))

(event Custom|Rise
  (bind _mesh (Variables|Character|GetMesh))
  (bind _returnvalue (Transformation|GetWorldLocation _mesh))
  ;[1 0 0.5232 1 60] Rise
  (Transformation|SetActorLocation (Math|Vector|MakeVector (.x _returnvalue) (.y _returnvalue) (.z (Transformation|GetActorLocation))) false false))

(event Custom|FindBodyForAttach
  ;[0.8307 0 1 1 60] Attach on Body
  (bind _outactors (Collision|SphereOverlapActors (Transformation|GetActorLocation) 1e+02 (Utilities|Array|MakeArray "ObjectTypeQuery3") "/Game/Blueprint/AI/AICharacterBodyForBugs_BP.AICharacterBodyForBugs_BP_C"))
  (bind _array_element (Utilities|Array|ForEachLoopwithBreak _outactors :!label _label)
    (:LoopBody
      (bind _asaicharacter_body_for_bugs_bp (Utilities|Casting|CastToAICharacterBodyForBugs_BP _array_element))
      (Variables|Default|SetCurrentAttachBody _asaicharacter_body_for_bugs_bp)
      (goto _label Break))
    (:Completed
      (Utilities|IsValid (Variables|Default|GetCurrentAttachBody)
        (:Is%20Valid
          (Utilities|Time|ClearandInvalidateTimerbyHandle (Variables|Default|GetFindBodyForAttachTimer))
          (Class|AbilitySystemComponent|GiveAbilityandActivateOnce (Ability|GetAbilitySystemComponent self) "/Game/Blueprint/Abilities/AI/LockAIBehaviorBugAttach_GA.LockAIBehaviorBugAttach_GA_C" 0 -1))))))

(event Custom|PerformBugExplosion
  (params (Deffered :type Float%20%28double-precision%29))
  ;[0 0.04714 1 1 60] Perform Bug Explosion
  (Utilities|FlowControl|Delay Deffered)
  (Utilities|FlowControl|DoOnce false
    (:Completed
      (Class|AbilitySystemComponent|GiveAbilityandActivateOnce (Ability|GetAbilitySystemComponent self) "/Game/Blueprint/Abilities/PerformBugExplosion_GA.PerformBugExplosion_GA_C" 0 -1))))

(event EventPerformCuicide
  ;[0.03853 0 1 1 60] Perform Cuicide (Call by Notify)
  (CallFunction|PerformBugExplosion 0.0)
  (bind _outactors (Collision|SphereOverlapActors (Transformation|GetWorldLocation (Variables|Character|GetMesh)) (Variables|Behavior|GetBugExplosionRadius) (Utilities|Array|MakeArray "ObjectTypeQuery3") "/Script/ArcherPRT.GameCharacter"))
  (for _array_element _outactors
    (bind _asaicharacter_bug_base_bp (Utilities|Casting|CastToAICharacterBugBase_BP _array_element)
      (:then
        (CallFunction|PerformBugExplosion _asaicharacter_bug_base_bp 0.2))
      (:CastFailed
        (Game|Damage|ApplyDamage _array_element (Variables|Behavior|GetBugExplosionDamage) 0 self)))))

(event EventAfterEnemyFound)

(event EventForcePerformWakeUp)

(event EventBeginPlay
  (bind _movebyspline (Variables|Default|GetMoveBySpline))
  (|CallParentFunction)
  (Utilities|FlowControl|Delay 0.2)
  (Utilities|FlowControl|Sequence
    (:then_0
      (if (Variables|Behavior|GetCanJumpOnCorpse)
        (CallFunction|FindBodyforAttach)))
    (:then_1
      (Utilities|IsValid (Variables|Default|GetCurrentSpline)
        (:Is%20Valid
          (Components|Timeline|SetPlayRate _movebyspline 0.025)
          (Components|Timeline|SetLooping _movebyspline true)
          (Components|Timeline|PlayfromStart _movebyspline)
          (Variables|/Script/Engine.CharacterMovementComponent|SetGravityScale (Variables|Character|GetCharacterMovement) 0.0))))
    (:then_2
      (Variables|/Script/AIModule.AIController|SetDefaultNavigationFilterClass (AI|GetAIController self) "/Game/ExternalContent/Nav_mesh_stuff/Nav_Query_Filters/Nav_Query_Filter_01.Nav_Query_Filter_01_C"))))

(event EventPerformonHitReaction
  (params (HitDirection :type Vector :default "0, 0, 0") (HitResult :type Hit%20Result%20Structure) (Causer :type Actor%20Object%20Reference) (WeaponType :type EWeaponType%20Enum :default "None") (Charged :type Boolean) (ForceHeavyHitReactions :type Boolean))
  (bind _bug_sounds (Variables|Default|GetBug_Sounds))
  ;[0 0.05011 1 1 60] HitReaction
  (Utilities|FlowControl|Sequence
    (:then_0
      (if (Variables|Default|GetAttached)
        (if (Class|StatsComponent|IsDead (Variables|Default|GetStatsComponent))
          (Utilities|IsValid (Variables|Default|GetCurrentAttachBody)
            (:Is%20Valid
              (Default|MakeAvaliableSocket (Variables|Default|GetCurrentAttachBody) (Variables|Default|GetCurrentAttachSocket))
              (if (Default|CheckAllAvaliableSockets (Variables|Default|GetCurrentAttachBody))
                _
                (else
                  (Class|AICharacter|PerformonHitReaction (Variables|Default|GetCurrentAttachBody) HitDirection HitResult Causer WeaponType Charged true)))
              (Variables|Default|SetCurrentAttachBody 0))
            (:Is%20Not%20Valid
              _))
          (CallFunction|DetachfromBody HitDirection)
          (else
            (Utilities|IsValid (Variables|Default|GetCurrentAttachBody)
              (:Is%20Valid
                (Class|AICharacter|PerformonHitReaction (Variables|Default|GetCurrentAttachBody) HitDirection HitResult Causer WeaponType Charged false)))))
        (elif (Class|StatsComponent|IsDead (Variables|Default|GetStatsComponent))
          (CallFunction|DetachfromBody HitDirection)
          (else
            (Class|AbilitySystemComponent|GiveAbilityandActivateOnce (Ability|GetAbilitySystemComponent self) "/Game/Blueprint/Abilities/AI/LockAIBehaviorHitReactionForBugs_GA.LockAIBehaviorHitReactionForBugs_GA_C" 0 -1)))))
    (:then_1
      (Audio|Components|Audio|SetSound _bug_sounds "/Game/ExternalContent/New_Enemy/Bug_enemy/Bug_Enemy_Test/Bug_enemy_sounds/Bug_Get_Hit_Cue.Bug_Get_Hit_Cue")
      (Audio|Components|Audio|Play _bug_sounds 0.0))))

(event EventAfteronDeath
  (|CallParentFunction)
  (CallFunction|DetachfromBody "0, 0, 0"))

(fn ConstructionScript
  (|CallParentFunction))

(fn PerformAttach
  (params (BodyForAttach :type AI%20Character%20Body%20for%20Bugs%20BP%20Object%20Reference) (SocketName :type Name))
  (Utilities|IsValid BodyForAttach
    (:Is%20Valid
      (Utilities|FlowControl|Sequence
        (:then_0
          (Transformation|AttachComponentToComponent (Variables|Character|GetMesh) (Variables|/Script/Engine.Character|GetMesh BodyForAttach) SocketName "SnapToTarget" "SnapToTarget" "KeepRelative" true))
        (:then_1
          (Collision|SetCollisionEnabled (Variables|Default|GetCapsuleComponent) "NoCollision"))
        (:then_2
          (Transformation|SetActorLocationAndRotation (Transformation|GetActorLocation BodyForAttach) (Transformation|GetActorRotation BodyForAttach))
          (Transformation|AttachActorToActor BodyForAttach "None" "SnapToTarget" "SnapToTarget" "KeepRelative" true))
        (:then_3
          (Default|MakeUnavaliableSocket BodyForAttach SocketName)
          (Variables|Default|SetCurrentAttachSocket SocketName))
        (:then_4
          (Variables|Default|SetAttached true))))))