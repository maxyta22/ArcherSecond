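; Zombie AI character variant made of up to ten bugs, each with its own collider, that acts as one enemy.
; On BeginPlay, all bug meshes follow the main mesh's pose, and a clamped count of them, always the first plus random others, become visible weak points.
; A hit reaction detaches the struck bug and launches it with physics.
; When no active bugs remain, the character deals itself massive damage.
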(event Custom|BugDeath
  (params (HitDirection :type Vector) (Collider :type Primitive%20Component%20Object%20Reference))
  (bind _self self)
  (bind _allbugcolliders (Variables|Default|GetAllBugColliders))
  (bind _bug_10_bind (Variables|Default|GetBug_10_BIND))
  (bind _bug_05_bind (Variables|Default|GetBug_05_BIND))
  (bind _activatedbugs (Variables|Default|GetActivatedBugs))
  (bind _bug_02_bind (Variables|Default|GetBug_02_BIND))
  (bind _bug_01_bind (Variables|Default|GetBug_01_BIND))
  (bind _bug_03_bind (Variables|Default|GetBug_03_BIND))
  (bind _bug_04_bind (Variables|Default|GetBug_04_BIND))
  (bind _bug_06_bind (Variables|Default|GetBug_06_BIND))
  (bind _bug_07_bind (Variables|Default|GetBug_07_BIND))
  (bind _bug_08_bind (Variables|Default|GetBug_08_BIND))
  (bind _bug_09_bind (Variables|Default|GetBug_09_BIND))
  (bind _returnvalue (Utilities|Array|FindItem _allbugcolliders Collider))
  (bind _returnvalue_2 (Utilities|Select :Index _returnvalue :Option%200 _bug_01_bind :Option%201 _bug_02_bind :Option%202 _bug_03_bind :Option%203 _bug_04_bind :Option%204 _bug_05_bind :Option%205 _bug_06_bind :Option%206 _bug_07_bind :Option%207 _bug_08_bind :Option%208 _bug_09_bind :Option%209 _bug_10_bind))
  (Utilities|Array|Clear (Variables|/Script/Engine.ActorComponent|GetComponentTags Collider))
  (Collision|SetCollisionEnabled Collider "NoCollision")
  (Transformation|SetWorldLocation _returnvalue_2 (Transformation|GetWorldLocation Collider) false false)
  (Components|SkinnedMesh|SetLeaderPoseComponent _returnvalue_2 0 true false)
  (Collision|SetCollisionEnabled _returnvalue_2 "PhysicsOnly")
  (Class|PrimitiveComponent|SetAllMassScale _returnvalue_2 5e+01)
  (Physics|SetSimulatePhysics _returnvalue_2 true)
  (Physics|AddImpulse _returnvalue_2 (* HitDirection 2000) "None" true)
  (Utilities|Array|RemoveItem _activatedbugs _returnvalue_2)
  (if (Utilities|Array|IsEmpty _activatedbugs)
    (Utilities|FlowControl|DelayUntilNextTick)
    (Game|Damage|ApplyDamage _self 1e+04 0 _self)))

(event EventBeginPlay
  (|CallParentFunction)
  (CallFunction|ConstructBugs)
  (Variables|Default|SetSleeping_Pose_Int (Math|Random|RandomInteger 3)))

(event EventPerformonHitReaction
  (params (HitDirection :type Vector :default "0, 0, 0") (HitComponent :type Primitive%20Component%20Object%20Reference))
  (|CallParentFunction HitDirection 0)
  (CallFunction|BugDeath HitDirection HitComponent))

(fn ConstructionScript
  (|CallParentFunction))

(fn ConstructBugs
  (Variables|Default|SetAllBugColliders (Utilities|Array|MakeArray (Variables|Default|GetBug_01_Collider) (Variables|Default|GetBug_02_Collider) (Variables|Default|GetBug_03_Collider) (Variables|Default|GetBug_04_Collider) (Variables|Default|GetBug_05_Collider) (Variables|Default|GetBug_06_Collider) (Variables|Default|GetBug_07_Collider) (Variables|Default|GetBug_08_Collider) (Variables|Default|GetBug_09_Collider) (Variables|Default|GetBug_10_Collider)))
  (bind _output_get (Variables|Default|SetAllBugs (Utilities|Array|MakeArray (Variables|Default|GetBug_01_BIND) (Variables|Default|GetBug_02_BIND) (Variables|Default|GetBug_03_BIND) (Variables|Default|GetBug_04_BIND) (Variables|Default|GetBug_05_BIND) (Variables|Default|GetBug_06_BIND) (Variables|Default|GetBug_07_BIND) (Variables|Default|GetBug_08_BIND) (Variables|Default|GetBug_09_BIND) (Variables|Default|GetBug_10_BIND))))
  (Components|SkinnedMesh|SetLeaderPoseComponent _output_get (Variables|Character|GetMesh) true false)
  (for _index (range 1 (Math|Integer|Clamp(Integer) (Variables|Default|GetValueSpawnBugs) 1 10))
    (if (== _index 1)
      (bind _output_get_2 (Variables|Default|SetCurrentBug (Variables|Default|GetBug_01_BIND)))
      (Utilities|Array|Add (Variables|Default|GetActivatedBugs) _output_get_2)
      (else
        (bind _output_get_3 (Variables|Default|SetCurrentBug (.OutItem (Utilities|Array|Random (Variables|Default|GetAllBugs))) :!label _label))
        (if (not (Utilities|Array|ContainsItem (Variables|Default|GetActivatedBugs) _output_get_3))
          _
          (else
            (goto _label)))))
    (Utilities|Array|Add (Variables|Default|GetActivatedBugs) (Variables|Default|GetCurrentBug))
    (Rendering|SetVisibility (Variables|Default|GetCurrentBug) true false)
    (Variables|/Script/Engine.ActorComponent|SetComponentTags (Utilities|Array|Get(acopy) (Variables|Default|GetAllBugColliders) (Utilities|Array|FindItem (Variables|Default|GetAllBugs) (Variables|Default|GetCurrentBug))) (Utilities|Array|MakeArray "WeakPoint"))
    (Collision|SetCollisionEnabled (Utilities|Array|Get(acopy) (Variables|Default|GetAllBugColliders) (Utilities|Array|FindItem (Variables|Default|GetAllBugs) (Variables|Default|GetCurrentBug))) "QueryOnly")))