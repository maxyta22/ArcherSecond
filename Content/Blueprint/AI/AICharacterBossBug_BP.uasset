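; AI character Blueprint for a bug boss that overrides its parent's combat events to run boss-specific Gameplay Abilities.
; Main attack, hit reaction and stagger reaction each grant and activate their ability once through the Ability System Component.
; Hit reaction also prints current health from the StatsComponent.
; The enemy-found and forced wake-up events are empty, and construction only calls the parent.
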(event EventAfterEnemyFound)

(event EventPerformonHitReaction
  (params (HitDirection :type Vector :default "0, 0, 0") (HitResult :type Hit%20Result%20Structure) (Causer :type Actor%20Object%20Reference) (WeaponType :type EWeaponType%20Enum :default "None") (Charged :type Boolean) (ForceHeavyHitReactions :type Boolean))
  (Development|PrintString (Utilities|String|ToString(Float) (Class|StatsComponent|GetHealth (Variables|Default|GetStatsComponent))))
  (Class|AbilitySystemComponent|GiveAbilityandActivateOnce (Ability|GetAbilitySystemComponent self) "/Game/Blueprint/Abilities/AI/HitReactionForBossBug_GA.HitReactionForBossBug_GA_C" 0 -1))

(event EventPerformMainAttack
  (Class|AbilitySystemComponent|GiveAbilityandActivateOnce (Ability|GetAbilitySystemComponent self) "/Game/Blueprint/Abilities/AI/AttackForBossBug_GA.AttackForBossBug_GA_C" 0 -1))

(event EventForcePerformWakeUp)

(event EventPerformonStaggerReaction
  (Class|AbilitySystemComponent|GiveAbilityandActivateOnce (Ability|GetAbilitySystemComponent self) "/Game/Blueprint/Abilities/AI/StaggerReactionForBossBug_GA.StaggerReactionForBossBug_GA_C" 0 -1))

(fn ConstructionScript
  (|CallParentFunction))