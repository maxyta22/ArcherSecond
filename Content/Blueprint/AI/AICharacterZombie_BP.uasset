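; Zombie AI character Blueprint that extends its parent with a bug mesh riding on the body and a random sleeping pose index chosen at BeginPlay.
; The construction script slaves Bug01 to the character mesh through master pose.
; On hit reaction, after the parent logic, BugDeath unlinks Bug01, moves it to its collider and launches it as a physics body along the hit direction.
; Logic to reveal random unique bugs is present but disconnected.
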(event Custom|BugDeath
  (params (HitDirection :type Vector))
  (bind _bug_01_bind (Variables|Default|GetBug_01_BIND))
  (Class|SkinnedMeshComponent|SetMasterPoseComponent _bug_01_bind 0 true)
  (Transformation|SetWorldLocation _bug_01_bind (Transformation|GetWorldLocation (Variables|Default|GetBug_01Collider)) false false)
  (Collision|SetCollisionEnabled _bug_01_bind "PhysicsOnly")
  (Class|PrimitiveComponent|SetAllMassScale _bug_01_bind 5e+01)
  (Physics|SetSimulatePhysics _bug_01_bind true)
  (Physics|AddImpulse _bug_01_bind (* HitDirection 2000) "None" true))

(event EventBeginPlay
  (|CallParentFunction)
  (Variables|Default|SetSleeping_Pose_Int (Math|Random|RandomInteger 3)))

(event EventPerformonHitReaction
  (params (HitDirection :type Vector :default "0, 0, 0"))
  (|CallParentFunction HitDirection)
  (CallFunction|BugDeath HitDirection))

(fn ConstructionScript
  (|CallParentFunction)
  (Class|SkinnedMeshComponent|SetMasterPoseComponent (Variables|Default|GetBug_01_BIND) (Variables|Character|GetMesh) true))