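; AI character body for a scripted bug wake-up scene, starting in a sleeping pose with its sockets set up.
; When an enemy is found or wake-up is forced, the BugScene mesh plays a wake-up montage while a GAS lock-behavior ability and sounds fire.
; Timed delays then hide that mesh, set visibility on the AICharacterBugScene_BP actor, and briefly suspend looking at the player.
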(event EventBeginPlay
  (|CallParentFunction)
  (Variables|Default|SetSleeping_Pose_Int 2)
  (CallFunction|SetupAvaliableSockets))

(event Collision|EventActorBeginOverlap
  (params (OtherActor :type Actor%20Object%20Reference)))

(event EventTick
  (params (DeltaSeconds :type Float%20%28single-precision%29))
  (|CallParentFunction DeltaSeconds) ; This node is disabled and will not be called.\nDrag off pins to build functionality.
)

(event EventForcePerformWakeUp
  (bind _bug_scene (Variables|Default|GetBug_Scene))
  (Utilities|FlowControl|Sequence
    (:then_0
      (Animation|Montage|PlayMontage _bug_scene "/Game/ExternalContent/New_Enemy/Bug_enemy/Bug_Enemy_Test/Animations/Bug_Enemy_Wake_Up_Scene_01_Montage.Bug_Enemy_Wake_Up_Scene_01_Montage"))
    (:then_1
      (Utilities|FlowControl|Delay 3.0)
      (Rendering|SetVisibility _bug_scene false false)
      (bind _returnvalue (Actor|GetActorOfClass "/Game/Blueprint/AI/Scene_Bug_Jump/AICharacterBugScene_BP.AICharacterBugScene_BP_C"))
      (Default|SetVisibility _returnvalue))
    (:then_2
      (Class|AbilitySystemComponent|GiveAbilityandActivateOnce (Ability|GetAbilitySystemComponent self) "/Game/Blueprint/Abilities/AI/LockAIBehaviorWakeUp_GA.LockAIBehaviorWakeUp_GA_C" 0 -1)
      (Audio|SpawnSound2D 0 1.0 1.0 0.0 0)
      (Components|Activation|Activate (Variables|Default|GetMonster_Idle_2_Cue) true))
    (:then_3
      (Variables|Default|SetShould_Look_At_Player false)
      (Utilities|FlowControl|Delay 3.0)
      (Variables|Default|SetShould_Look_At_Player true))))

(event EventAfterEnemyFound
  (bind _bug_scene (Variables|Default|GetBug_Scene))
  (Utilities|FlowControl|Delay 0.005)
  (Utilities|FlowControl|Sequence
    (:then_0
      (Animation|Montage|PlayMontage _bug_scene "/Game/ExternalContent/New_Enemy/Bug_enemy/Bug_Enemy_Test/Animations/Bug_Enemy_Wake_Up_Scene_01_Montage.Bug_Enemy_Wake_Up_Scene_01_Montage"))
    (:then_1
      (Utilities|FlowControl|Delay 3.0)
      (Rendering|SetVisibility _bug_scene false false)
      (bind _returnvalue (Actor|GetActorOfClass "/Game/Blueprint/AI/Scene_Bug_Jump/AICharacterBugScene_BP.AICharacterBugScene_BP_C"))
      (Default|SetVisibility _returnvalue))
    (:then_2
      (Class|AbilitySystemComponent|GiveAbilityandActivateOnce (Ability|GetAbilitySystemComponent self) "/Game/Blueprint/Abilities/AI/LockAIBehaviorWakeUp_GA.LockAIBehaviorWakeUp_GA_C" 0 -1)
      (Audio|SpawnSound2D 0 1.0 1.0 0.0 0)
      (Components|Activation|Activate (Variables|Default|GetMonster_Idle_2_Cue) true))
    (:then_3
      (Variables|Default|SetShould_Look_At_Player false)
      (Utilities|FlowControl|Delay 3.0)
      (Variables|Default|SetShould_Look_At_Player true))))

(fn ConstructionScript
  (|CallParentFunction))