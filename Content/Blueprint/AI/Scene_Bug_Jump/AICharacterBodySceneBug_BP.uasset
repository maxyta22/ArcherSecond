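; AI character body that starts in a sleeping pose and carries attachment sockets for bugs.
; Wake-up plays a montage on a scene bug mesh, runs a behavior-locking ability and later destroys that mesh; hits set the enemy and trigger a reaction ability.
; BeginPlay picks the first socket plus random others.
; Occupying a socket sets the BugRevived blackboard key; once all are free again, the body clears it and kills itself with damage.
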(event EventBeginPlay
  (|CallParentFunction)
  (Variables|Default|SetSleeping_Pose_Int 2)
  (CallFunction|SetupAvaliableSockets))

(event EventPerformonHitReaction
  (params (DamageData :type Damage%20Data%20Structure))
  (bind (_damagedirection _damagepoint _damageinstigator _damagecauser _damageweapontype _damagecharged) (Utilities|Struct|BreakDamageData DamageData))
  (bind _asprtaicontroller (Utilities|Casting|CastToPRTAIController (Pawn|GetController)))
  (Class|PRTAIController|SetEnemy _asprtaicontroller 0)
  (Variables|Default|SetLastHitStruct (Utilities|Struct|MakeLastHitStruct _damagedirection (.HitComponent (Collision|BreakHitResult _damagepoint)) _damageweapontype _damagecharged))
  (Class|AbilitySystemComponent|GiveAbilityandActivateOnce (Ability|GetAbilitySystemComponent self) "/Game/Blueprint/Abilities/AI/LockAIBehaviorHitReaction_GA.LockAIBehaviorHitReaction_GA_C" 0 -1))

(event EventForcePerformWakeUp
  (bind _bug_scene (Variables|Default|GetBug_Scene))
  (Utilities|FlowControl|Sequence
    (:then_0
      (Animation|Montage|PlayMontage _bug_scene "/Game/ExternalContent/New_Enemy/Bug_enemy/Bug_Enemy_Test/Animations/Bug_Enemy_Wake_Up_Scene_01_Montage.Bug_Enemy_Wake_Up_Scene_01_Montage"))
    (:then_1
      (Variables|Default|SetShould_Look_At_Player false)
      (Utilities|FlowControl|Delay 3.0)
      (Variables|Default|SetShould_Look_At_Player true))
    (:then_2
      (Class|AbilitySystemComponent|GiveAbilityandActivateOnce (Ability|GetAbilitySystemComponent self) "/Game/Blueprint/Abilities/AI/LockAIBehaviorWakeUp_GA.LockAIBehaviorWakeUp_GA_C" 0 -1)
      (Audio|SpawnSound2D 0 1.0 1.0 0.0 0)
      (Components|Activation|Activate (Variables|Default|GetMonster_Idle_2_Cue) true))
    (:then_3
      (Utilities|FlowControl|Delay 3.0)
      (Components|DestroyComponent _bug_scene))))

(event EventAfterEnemyFound
  (bind _bug_scene (Variables|Default|GetBug_Scene))
  (Utilities|FlowControl|Delay 0.005)
  (Utilities|FlowControl|Sequence
    (:then_0
      (Animation|Montage|PlayMontage _bug_scene "/Game/ExternalContent/New_Enemy/Bug_enemy/Bug_Enemy_Test/Animations/Bug_Enemy_Wake_Up_Scene_01_Montage.Bug_Enemy_Wake_Up_Scene_01_Montage"))
    (:then_1
      (Variables|Default|SetShould_Look_At_Player false)
      (Utilities|FlowControl|Delay 3.0)
      (Variables|Default|SetShould_Look_At_Player true))
    (:then_2
      (Class|AbilitySystemComponent|GiveAbilityandActivateOnce (Ability|GetAbilitySystemComponent self) "/Game/Blueprint/Abilities/AI/LockAIBehaviorWakeUp_GA.LockAIBehaviorWakeUp_GA_C" 0 -1)
      (Audio|SpawnSound2D 0 1.0 1.0 0.0 0)
      (Components|Activation|Activate (Variables|Default|GetMonster_Idle_2_Cue) true))
    (:then_3
      (Utilities|FlowControl|Delay 3.0)
      (Components|DestroyComponent _bug_scene))))

(fn ConstructionScript
  (|CallParentFunction))

(fn FindAvaliableSocketforBug
  (bind _currentavaliablessocketsforbugs (Variables|Default|GetCurrentAvaliablesSocketsForBugs))
  (if (Utilities|Array|IsNotEmpty _currentavaliablessocketsforbugs)
    (return true (Utilities|Array|Get(acopy) _currentavaliablessocketsforbugs))
    (else
      (return false "None"))))

(fn MakeUnavaliableSocket
  (params (UnavaliableSocket :type Name))
  (bind _currentavaliablessocketsforbugs (Variables|Default|GetCurrentAvaliablesSocketsForBugs))
  (if (Utilities|Array|ContainsItem _currentavaliablessocketsforbugs UnavaliableSocket)
    (Utilities|Array|RemoveItem _currentavaliablessocketsforbugs UnavaliableSocket)
    (AI|Components|Blackboard|SetValueasBool (AI|GetBlackboard 0) (Utilities|Name|MakeLiteralName "BugRevived") true)))

(fn MakeAvaliableSocket
  (params (AvaliableSocket :type Name))
  (Utilities|Array|AddUnique (Variables|Default|GetCurrentAvaliablesSocketsForBugs) AvaliableSocket)
  (CallFunction|CheckDeath))

(fn CheckAllAvaliableSockets
  (return (== (Utilities|Array|Length (Variables|Internal|GetAvaliablesSocketsForCheckDeath)) (Utilities|Array|Length (Variables|Default|GetCurrentAvaliablesSocketsForBugs)))))

(fn CheckDeath
  (bind _self self)
  (if (CallFunction|CheckAllAvaliableSockets)
    (AI|Components|Blackboard|SetValueasBool (AI|GetBlackboard 0) (Utilities|Name|MakeLiteralName "BugRevived") false)
    (Game|Damage|ApplyDamage _self 1e+04 0 _self)))

(fn SetupAvaliableSockets
  (LocalVariables|SetL_SoketNames (Variables|Default|GetAllSocketNamesForBugs))
  (for _index (range 0 (Variables|Default|GetValueAvaliableSockets))
    (if (== _index 0)
      (Utilities|Array|AddUnique (Variables|Default|GetCurrentAvaliablesSocketsForBugs) (Utilities|Array|Get(acopy) (LocalVariables|GetL_SoketNames)))
      (Utilities|Array|RemoveItem (LocalVariables|GetL_SoketNames) (Utilities|Array|Get(acopy) (LocalVariables|GetL_SoketNames)))
      (else
        (bind _output_get (LocalVariables|SetL_CurrentSocket (.OutItem (Utilities|Array|Random (LocalVariables|GetL_SoketNames)))))
        (Utilities|Array|AddUnique (Variables|Default|GetCurrentAvaliablesSocketsForBugs) _output_get)
        (Utilities|Array|RemoveItem (LocalVariables|GetL_SoketNames) (LocalVariables|GetL_CurrentSocket)))))
  (Variables|Internal|SetAvaliablesSocketsForCheckDeath (Variables|Default|GetCurrentAvaliablesSocketsForBugs)))