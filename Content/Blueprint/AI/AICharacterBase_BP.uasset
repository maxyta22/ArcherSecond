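; Base AI enemy Blueprint that handles combat reactions, waking from sleep and death.
; Event hooks activate one-shot GAS "LockAIBehavior" abilities for attack, wake-up, death, chance-based evade on being aimed at and occasional hit reactions, otherwise playing a montage.
; Death also disables capsule collision and attaches an optional DropCorpse actor to the mesh.
; Tick shows health as text; SpawnDrop is empty and the timeline item-scatter logic is disconnected.
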(event Custom|PerformEvade
  ;[0 1 0.2142 1 69] Evade
  (if (Math|Random|RandomBoolwithWeight (Variables|Default|GetProbabilityEvade))
    (Class|AbilitySystemComponent|GiveAbilityandActivateOnce (Ability|GetAbilitySystemComponent self) "/Game/Blueprint/Abilities/AI/LockAIBehaviorEvade_GA.LockAIBehaviorEvade_GA_C" 0 -1)))

(event Custom|SpawnDrop
  ;[0 0.0676 1 1 60] Spawn Drop
)

(event Custom|ForcePerformWakeUp
  ;[0.8309 0 1 1 69] WakeUp
  (Class|AbilitySystemComponent|GiveAbilityandActivateOnce (Ability|GetAbilitySystemComponent self) "/Game/Blueprint/Abilities/AI/LockAIBehaviorWakeUp_GA.LockAIBehaviorWakeUp_GA_C" 0 -1)
  (Audio|SpawnSound2D 0 1.0 1.0 0.0 0)
  (Components|Activation|Activate (Variables|Default|GetMonster_Idle_2_Cue) true)
  (Variables|Default|SetShould_Look_At_Player true))

(event Custom|PerformCuicide
  ;[0 1 0.3298 1 60] Events (Need Transfer in c++ Code
)

(event Custom|PerformMainAttack
  ;[1 0.3532 0 1 60] Attack
  (Class|AbilitySystemComponent|GiveAbilityandActivateOnce (Ability|GetAbilitySystemComponent self) "/Game/Blueprint/Abilities/AI/LockAIBehaviorMainAttack_GA.LockAIBehaviorMainAttack_GA_C" 0 -1))

(event EventAfterReactiontoAiming
  ;[0 1 0.2142 1 69] Evade
  (CallFunction|PerformEvade))

(event EventTick
  (params (DeltaSeconds :type Float%20%28single-precision%29))
  (|CallParentFunction DeltaSeconds)
  ;[0.7783 1 0 1 30] Show HP
  (Rendering|Components|TextRender|SetText (Variables|Default|GetTextRender) (Utilities|Text|ToText(Float) (Class|StatsComponent|GetHealth (Variables|Default|GetStatsComponent)) "HalfToEven")))

(event EventAfterEnemyFound
  ;[0.8309 0 1 1 69] WakeUp
  (Utilities|FlowControl|Delay 0.005)
  (Class|AbilitySystemComponent|GiveAbilityandActivateOnce (Ability|GetAbilitySystemComponent self) "/Game/Blueprint/Abilities/AI/LockAIBehaviorWakeUp_GA.LockAIBehaviorWakeUp_GA_C" 0 -1)
  (Audio|SpawnSound2D 0 1.0 1.0 0.0 0)
  (Components|Activation|Activate (Variables|Default|GetMonster_Idle_2_Cue) true)
  (Variables|Default|SetShould_Look_At_Player true))

(event EventPerformonHitReaction
  (params (HitDirection :type Vector :default "0, 0, 0") (HitResult :type Hit%20Result%20Structure) (Causer :type Actor%20Object%20Reference) (WeaponType :type EWeaponType%20Enum :default "None") (Charged :type Boolean))
  ;[0 0.2695 1 1 60] Hit Reaction
  (if (Math|Random|RandomBoolwithWeight 0.2)
    (Class|AbilitySystemComponent|GiveAbilityandActivateOnce (Ability|GetAbilitySystemComponent self) "/Game/Blueprint/Abilities/AI/LockAIBehaviorHitReaction_GA.LockAIBehaviorHitReaction_GA_C" 0 -1)
    (else
      (Animation|PlayAnimMontage "/Game/ExternalContent/New_Enemy/Soldier_Enemy/anims/Soldier_get_add_hit_Montage.Soldier_get_add_hit_Montage" 1.0 "None"))))

(event EventBeginPlay
  (switch Utilities|FlowControl|Switch|SwitchonEAIStartCondition (Variables|Default|GetStartCondition)
    (:Sleep
      (Components|Activation|Deactivate (Variables|Default|GetMonster_Idle_2_Cue)))))

(event EventAfteronDeath
  (bind _dropcorpse (Variables|Default|GetDropCorpse))
  ;[0 0.2695 1 1 60] Death
  (Utilities|FlowControl|Sequence
    (:then_0
      (Default|CallOnDeath)
      (Collision|SetCollisionEnabled (Variables|Default|GetCapsuleComponent) "NoCollision")
      (CallFunction|SpawnDrop)
      (Class|AbilitySystemComponent|GiveAbilityandActivateOnce (Ability|GetAbilitySystemComponent self) "/Game/Blueprint/Abilities/AI/LockAIBehaviorDeath_GA.LockAIBehaviorDeath_GA_C" 0 -1))
    (:then_1
      (if (Utilities|IsValidClass _dropcorpse)
        (bind _returnvalue (Game|SpawnActorfromClass _dropcorpse (Math|Transform|MakeTransform "0, 0, 0" "0, 0, 0" "1.000000,1.000000,1.000000") "AlwaysSpawn" 0 0))
        (Class|PickupResourcesBase|SetContainer _returnvalue self)
        (Transformation|SetActorLocation _returnvalue (Class|SkeletalMeshComponent|GetSkeletalCenterOfMass (Variables|Character|GetMesh)) false false)
        (Transformation|AttachComponentToComponent _returnvalue (Variables|Character|GetMesh) "None" "SnapToTarget" "SnapToTarget" "KeepRelative" true)))))

(event EventAfteronHit
  (params (HitDirection :type Vector :default "0, 0, 0") (HitResult :type Hit%20Result%20Structure) (Causer :type Actor%20Object%20Reference) (WeaponType :type EWeaponType%20Enum :default "None") (Charged :type Boolean))
  ;[0 0.2695 1 1 60] Hit Reaction
  (Audio|SpawnSound2D "/Game/ExternalContent/Lizard/sounds/Lizard_Get_Hit_Cue.Lizard_Get_Hit_Cue" 1.0 1.0 0.0 0)
  (Effects|SpawnEmitteratLocation "/Game/ExternalContent/FXVillesBloodVFXPack/Particles/Cascade/Real/P_Blood_Burst_Omni.P_Blood_Burst_Omni" (Transformation|GetSocketLocation (Variables|Character|GetMesh) "Head_Socket")))

(fn ConstructionScript)