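; Stationary ranged bug AI character that defines its attack trigger, attack glow and sounds on top of a parent character.
; The main attack gives and activates a one-shot Gameplay Ability through the Ability System Component.
; A separate emissive attack event plays the ranged attack sound and runs a timeline that drives emissive material parameters on the mesh.
; Hit reactions call the parent logic, then play a hurt sound on the same audio component.
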(event Custom|EmissiveAttack
  (bind _mesh (Variables|Character|GetMesh))
  (bind _bug_sounds (Variables|Default|GetBug_Sounds))
  (Audio|Components|Audio|SetSound _bug_sounds "/Game/ExternalContent/New_Enemy/Bug_enemy/Bug_Enemy_Test/Bug_enemy_sounds/Insectoid_Ranged_Sound_Cue.Insectoid_Ranged_Sound_Cue")
  (Audio|Components|Audio|Play _bug_sounds 0.0)
  (bind (_direction _on_off _emissive_value) (Timeline|Emissive PlayFromStart)
    (:Update
      (Rendering|Material|SetScalarParameterValueonMaterials _mesh "Emissive_On" _on_off)
      (Rendering|Material|SetScalarParameterValueonMaterials _mesh "Emissive_Power" _emissive_value))))

(event EventPerformMainAttack
  (Class|AbilitySystemComponent|GiveAbilityandActivateOnce (Ability|GetAbilitySystemComponent self) "/Game/Blueprint/Abilities/AI/AttackForStancionaryRangeBug_GA.AttackForStancionaryRangeBug_GA_C" 0 -1))

(event EventPerformonHitReaction
  (params (DamageData :type Damage%20Data%20Structure))
  (bind _bug_sounds (Variables|Default|GetBug_Sounds))
  (|CallParentFunction DamageData)
  (Audio|Components|Audio|SetSound _bug_sounds "/Game/ExternalContent/New_Enemy/Bug_enemy/Bug_Enemy_Test/Bug_enemy_sounds/Bug_Get_Hit_Cue.Bug_Get_Hit_Cue")
  (Audio|Components|Audio|Play _bug_sounds 0.0))

(fn ConstructionScript
  (|CallParentFunction))