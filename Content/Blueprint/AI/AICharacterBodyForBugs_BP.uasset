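; AI character body that hosts bugs on mesh sockets, partly randomized at BeginPlay.
; Taking a socket sets the BugRevived blackboard key; once all sockets are free again, it clears the key and kills itself with damage.
; Hits set the controller's enemy and trigger a GAS hit-reaction ability; death switches to ragdoll after a delay.
; Physical animation drives the arms, and Tick feeds the angle to the player into BlendSpaceWalk.
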(event Custom|Physical_Animation
  (bind _physicalanimationdata (Utilities|Struct|MakePhysicalAnimationData false 1e+03 1e+02 1e+03 1e+02))
  (bind _left_arm (Variables|Default|Getleft_arm))
  (bind _physicalanimation (Variables|Default|GetPhysicalAnimation))
  (bind _mesh (Variables|Character|GetMesh))
  (bind _right_arm (Variables|Default|Getright_arm))
  (Class|PhysicalAnimationComponent|SetSkeletalMeshComponent _physicalanimation (Variables|Character|GetMesh))
  (Class|PhysicalAnimationComponent|ApplyPhysicalAnimationSettingsBelow _physicalanimation _left_arm _physicalanimationdata false)
  (Class|SkeletalMeshComponent|SetAllBodiesBelowSimulatePhysics _mesh _left_arm true false)
  (Class|PhysicalAnimationComponent|ApplyPhysicalAnimationSettingsBelow _physicalanimation _right_arm _physicalanimationdata false)
  (Class|SkeletalMeshComponent|SetAllBodiesBelowSimulatePhysics _mesh _right_arm true false))

(event Custom|Tick_String)

(event EventBeginPlay
  (|CallParentFunction)
  (Variables|Default|SetSleeping_Pose_Int (Math|Random|RandomInteger 3))
  (CallFunction|SetupAvaliableSockets)
  (CallFunction|PhysicalAnimation))

(event EventPerformonHitReaction
  (params (HitDirection :type Vector :default "0, 0, 0") (HitResult :type Hit%20Result%20Structure) (Causer :type Actor%20Object%20Reference) (WeaponType :type EWeaponType%20Enum :default "None") (Charged :type Boolean) (ForceHeavyHitReactions :type Boolean))
  (bind _asprtaicontroller (Utilities|Casting|CastToPRTAIController (Pawn|GetController)))
  (Class|PRTAIController|SetEnemy _asprtaicontroller Causer)
  (Variables|Default|SetLastHitStruct (Utilities|Struct|MakeLastHitStruct HitDirection (.HitComponent (Collision|BreakHitResult HitResult)) WeaponType Charged ForceHeavyHitReactions))
  (Class|AbilitySystemComponent|GiveAbilityandActivateOnce (Ability|GetAbilitySystemComponent self) "/Game/Blueprint/Abilities/AI/LockAIBehaviorHitReaction_GA.LockAIBehaviorHitReaction_GA_C" 0 -1))

(event EventTick
  (params (DeltaSeconds :type Float%20%28single-precision%29))
  (Utilities|FlowControl|Sequence
    (:then_0
      (bind _returnvalue (Class|MathUtils|FindAngleBetweenForwardVectorandTarget (Transformation|GetWorldLocation (Variables|Default|GetCapsuleComponent)) (Math|Vector|GetForwardVector (Variables|Character|GetMesh)) (Transformation|GetWorldLocation (Variables|/Script/Engine.Character|GetCapsuleComponent (Game|GetPlayerCharacter 0)))))
      (bind _output_get (Variables|Default|SetBlend_Space_Walk (Math|Interpolation|FInterpTo _returnvalue _returnvalue 0.0 0.1)))
      (Development|PrintString (Utilities|String|ToString(Float) _output_get) true true "(R=0.000000,G=0.660000,B=1.000000,A=1.000000)" 0.0))))

(event EventAfteronDeath
  (|CallParentFunction)
  (Class|PhysicalAnimationComponent|ApplyPhysicalAnimationSettingsBelow (Variables|Default|GetPhysicalAnimation) (Variables|Default|GetRoot_Bone) (Utilities|Struct|MakePhysicalAnimationData true 0.0) false)
  (Utilities|FlowControl|Delay 0.4)
  (Physics|SetSimulatePhysics (Variables|Character|GetMesh) true))

(fn ConstructionScript
  (|CallParentFunction))

(fn FindAvaliableSocketforBug
  (bind _currentavaliablessocketsforbugs (Variables|Default|GetCurrentAvaliablesSocketsForBugs))
  (if (Utilities|Array|IsNotEmpty _currentavaliablessocketsforbugs)
    (return true (Utilities|Array|Get(acopy) _currentavaliablessocketsforbugs))
    (else
      (return false "None"))))

(fn MakeUnavaliableSocket
  (params (UnavaliableSocket :type Name))
  (bind _currentavaliablessocketsforbugs (Variables|Default|GetCurrentAvaliablesSocketsForBugs))
  (if (Utilities|Array|ContainsItem _currentavaliablessocketsforbugs UnavaliableSocket)
    (Utilities|Array|RemoveItem _currentavaliablessocketsforbugs UnavaliableSocket)
    (AI|Components|Blackboard|SetValueasBool (AI|GetBlackboard 0) (Utilities|Name|MakeLiteralName "BugRevived") true)))

(fn MakeAvaliableSocket
  (params (AvaliableSocket :type Name))
  (Utilities|Array|AddUnique (Variables|Default|GetCurrentAvaliablesSocketsForBugs) AvaliableSocket)
  (CallFunction|CheckDeath))

(fn CheckAllAvaliableSockets
  (return (== (Utilities|Array|Length (Variables|Internal|GetAvaliablesSocketsForCheckDeath)) (Utilities|Array|Length (Variables|Default|GetCurrentAvaliablesSocketsForBugs)))))

(fn CheckDeath
  (bind _self self)
  (if (CallFunction|CheckAllAvaliableSockets)
    (AI|Components|Blackboard|SetValueasBool (AI|GetBlackboard 0) (Utilities|Name|MakeLiteralName "BugRevived") false)
    (Game|Damage|ApplyDamage _self 1e+04 0 _self)))

(fn SetupAvaliableSockets
  (LocalVariables|SetL_SoketNames (Variables|Default|GetAllSocketNamesForBugs))
  (for _index (range 0 (Variables|Behavior|GetValueAvaliableSockets))
    (if (== _index 0)
      (Utilities|Array|AddUnique (Variables|Default|GetCurrentAvaliablesSocketsForBugs) (Utilities|Array|Get(acopy) (LocalVariables|GetL_SoketNames)))
      (Utilities|Array|RemoveItem (LocalVariables|GetL_SoketNames) (Utilities|Array|Get(acopy) (LocalVariables|GetL_SoketNames)))
      (else
        (bind _output_get (LocalVariables|SetL_CurrentSocket (.OutItem (Utilities|Array|Random (LocalVariables|GetL_SoketNames)))))
        (Utilities|Array|AddUnique (Variables|Default|GetCurrentAvaliablesSocketsForBugs) _output_get)
        (Utilities|Array|RemoveItem (LocalVariables|GetL_SoketNames) (LocalVariables|GetL_CurrentSocket)))))
  (Variables|Internal|SetAvaliablesSocketsForCheckDeath (Variables|Default|GetCurrentAvaliablesSocketsForBugs)))