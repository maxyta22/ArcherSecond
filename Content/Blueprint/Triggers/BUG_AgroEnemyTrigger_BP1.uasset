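; Trigger actor that sets listed enemies on the player when the player character overlaps it.
; Every player overlap calls BugJump on the Bug_Jump_BP actor found in the level by class.
; A DoOnce then runs a single pass over AgroEnemiesList, making the player the enemy of each PRT AI controller without a valid one and force-waking its AI character.
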(event Collision|EventActorBeginOverlap
  (params (OtherActor :type Actor%20Object%20Reference))
  (bind _asplayer_character (Utilities|Casting|CastToPlayerCharacter OtherActor))
  (bind _returnvalue (Actor|GetActorOfClass "/Game/ExternalContent/New_Enemy/Bug_enemy/Bug_Enemy_Test/Bug_Jump_BP.Bug_Jump_BP_C"))
  (Default|BugJump _returnvalue)
  (Utilities|FlowControl|DoOnce false
    (:Completed
      (for _array_element (Variables|Default|GetAgroEnemiesList)
        (bind _asprtaicontroller (Utilities|Casting|CastToPRTAIController (AI|GetAIController _array_element)))
        (Utilities|IsValid (Class|PRTAIController|GetEnemy _asprtaicontroller)
          (:Is%20Not%20Valid
            (Class|PRTAIController|SetEnemy _asprtaicontroller _asplayer_character)
            (bind _asaicharacter_base_bp (Utilities|Casting|CastToAICharacterBase_BP _array_element))
            (Default|ForcePerformWakeUp _asaicharacter_base_bp)))))))

(fn ConstructionScript)