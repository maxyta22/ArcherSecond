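; AgroEnemyTrigger_BP is a trigger that aggros a list of AI enemies onto the player when the player walks into it.
; On the first overlap by an actor of exactly PlayerCharacter_BP class, a DoOnce lets it loop through AgroEnemiesList.
; Each enemy whose PRTAIController has no valid enemy gets the player as its enemy, then is forced awake through AICharacterBase_BP.
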(event Collision|EventActorBeginOverlap
  (params (OtherActor :type Actor%20Object%20Reference))
  (bind _asplayer_character (Utilities|Casting|CastToPlayerCharacter OtherActor))
  (if (== (Utilities|GetClass OtherActor) "/Game/Blueprint/Player/PlayerCharacter_BP.PlayerCharacter_BP_C")
    (Utilities|FlowControl|DoOnce false
      (:Completed
        (for _array_element (Variables|Default|GetAgroEnemiesList)
          (bind _asprtaicontroller (Utilities|Casting|CastToPRTAIController (AI|GetAIController _array_element)))
          (Utilities|IsValid (Class|PRTAIController|GetEnemy _asprtaicontroller)
            (:Is%20Not%20Valid
              (Class|PRTAIController|SetEnemy _asprtaicontroller _asplayer_character)
              (bind _asaicharacter_base_bp (Utilities|Casting|CastToAICharacterBase_BP _array_element))
              (Default|ForcePerformWakeUp _asaicharacter_base_bp))))))))

(fn ConstructionScript)