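; Enemy spawn point that, once activated, repeatedly spawns an enemy class at its own transform at an accelerating rate.
; Activation waits a random delay of up to a second, spawns immediately and starts the spawn timer.
; Each spawn plays a montage and sets the player as the AI controller's enemy.
; It then shrinks the interval and restarts the timer, with no lower clamp or stop condition.
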(event Custom|StartSpawnTimer
  (Utilities|Time|ClearandInvalidateTimerbyHandle (Variables|Default|GetSpawnTimer))
  (bind _returnvalue (Utilities|Time|SetTimerbyEvent (delegate Custom|SpawnEnemyIteration) (Variables|SpawnSettings|GetTimeSpawnInterval) true))
  (Variables|Default|SetSpawnTimer _returnvalue))

(event Custom|SpawnEnemyIteration
  (bind _returnvalue (Game|SpawnActorfromClass (Variables|SpawnSettings|GetSpawnedEnemy) (Math|Transform|MakeTransform (Transformation|GetActorLocation) (Transformation|GetActorRotation) "1.000000,1.000000,1.000000") "Undefined" 0 0))
  (Animation|PlayAnimMontage _returnvalue (Variables|Default|GetSpawnMonage) 1.0 "None")
  (Class|PRTAIController|SetEnemy (Class|AICharacter|GetAIControllerRef _returnvalue) (Game|GetPlayerCharacter 0))
  (Variables|SpawnSettings|SetTimeSpawnInterval (- (Variables|SpawnSettings|GetTimeSpawnInterval) (Variables|SpawnSettings|GetSpeedScaleSpawn)))
  (CallFunction|StartSpawnTimer))

(event Custom|ActivateSpawnTarget
  (Utilities|FlowControl|Delay (Math|Random|RandomFloatinRange 0.0 1.0))
  (CallFunction|SpawnEnemyIteration)
  (CallFunction|StartSpawnTimer))

(fn ConstructionScript)