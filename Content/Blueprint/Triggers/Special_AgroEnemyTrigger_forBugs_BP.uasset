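; Special one-shot trigger that aggros a list of bug enemies when the player character overlaps it.
; For each listed enemy whose AI controller has no valid enemy, it sets the player as the target and forces the enemy's wake-up.
; Each enemy woken this way also calls LightsOn on a Drop_Light_BP actor found by class lookup in the level.
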(event Collision|EventActorBeginOverlap
  (params (OtherActor :type Actor%20Object%20Reference))
  (bind _asplayer_character (Utilities|Casting|CastToPlayerCharacter OtherActor))
  (Utilities|FlowControl|DoOnce false
    (:Completed
      (for _array_element (Variables|Default|GetAgroEnemiesList)
        (bind _asprtaicontroller (Utilities|Casting|CastToPRTAIController (AI|GetAIController _array_element)))
        (Utilities|IsValid (Class|PRTAIController|GetEnemy _asprtaicontroller)
          (:Is%20Not%20Valid
            (Class|PRTAIController|SetEnemy _asprtaicontroller _asplayer_character)
            (bind _asaicharacter_base_bp (Utilities|Casting|CastToAICharacterBase_BP _array_element))
            (Default|ForcePerformWakeUp _asaicharacter_base_bp)
            (bind _returnvalue (Actor|GetActorOfClass "/Game/ExternalContent/Cave/cave_test_01_Mesh/Cave_Level_Design_Tests/Propellers_Room_Lights/Drop_Light_BP.Drop_Light_BP_C"))
            (Default|Lightson _returnvalue)))))))

(fn ConstructionScript)