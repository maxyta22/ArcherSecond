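; Checkpoint trigger actor that saves the game through ArcherPRTGameMode_BP when an actor of class PlayerCharacter_BP overlaps it.
; On BeginPlay it hides its sprite and binds to the game mode's LoadFullSteamLevels event.
; Saving stays gated by a CanSaveGame flag, which is set 0.2 seconds after that bound event fires.
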(event Custom|CanSaveGame
  (Utilities|FlowControl|Delay 0.2)
  (Variables|Default|SetbCanSaveGame true))

(event EventBeginPlay
  (Development|SetHiddeninGame (Variables|Default|GetSpriteComponent) true false)
  (EventDispatchers|BindEventtoLoadFullSteamLevels (.AsArcher%20PRTGame%20Mode%20BP (Utilities|Casting|CastToArcherPRTGameMode_BP (Game|GetGameMode))) (delegate Custom|CanSaveGame)))

(event Collision|EventActorBeginOverlap
  (params (OtherActor :type Actor%20Object%20Reference))
  (if (Variables|Default|GetbCanSaveGame)
    (if (== (Utilities|GetClass OtherActor) "/Game/Blueprint/Player/PlayerCharacter_BP.PlayerCharacter_BP_C")
      (bind _asarcher_prtgame_mode_bp (Utilities|Casting|CastToArcherPRTGameMode_BP (Game|GetGameMode)))
      (Default|SaveGame _asarcher_prtgame_mode_bp))))

(fn ConstructionScript)