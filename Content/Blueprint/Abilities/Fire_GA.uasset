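; Gameplay ability that runs the player's fire-button weapon charge, branching on the equipped weapon's type.
; Glove and gun chain charge into full-charge montages on blend out, with sounds; only the gun sets WeaponCharged.
; An empty gun plays a no-ammo montage, then calls FinishFire.
; A StopFire gameplay event ends the ability, which cleans up the wait task and calls FinishFire on the weapon component.
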(event Ability|EventActivateAbility
  (bind _asplayer_character_bp (Utilities|Casting|CastToPlayerCharacter_BP (Ability|GetAvatarActorfromActorInfo))
    (:then
      (Variables|Default|SetPlayerCharacterBP _asplayer_character_bp)
      (bind _asynctaskproxy (Ability|Tasks|WaitGameplayEvent "(TagName=\"Player.Attack.StopFire\")" 0)
        (:then
          (Variables|Default|SetAsync%20Task _asynctaskproxy)
          (switch Utilities|FlowControl|Switch|SwitchonEWeaponType (.WeaponType (Utilities|GetClassDefaults (Variables|/Script/ArcherPRT.WeaponComponent|GetCurrentEquipWeapon (Variables|/Script/ArcherPRT.GameCharacter|GetWeaponComponent (Variables|Default|GetPlayerCharacterBP)))))
            (:None
              (Ability|EndAbility))
            (:PneumaticGlove
              (Animation|Montage|PlayMontage (Variables|/Script/Engine.Character|GetMesh (Variables|Default|GetPlayerCharacterBP)) (.ChargeAnimation (Utilities|GetClassDefaults (Variables|/Script/ArcherPRT.WeaponComponent|GetCurrentEquipWeapon (Variables|/Script/ArcherPRT.GameCharacter|GetWeaponComponent (Variables|Default|GetPlayerCharacterBP)))))
                (:then
                  (Default|PlaySound (Variables|Default|GetPlayerCharacterBP) (Variables|/Game/Blueprint/Player/PlayerCharacter_BP.PlayerCharacter_BP_C|GetWeapon_Sound (Variables|Default|GetPlayerCharacterBP)) "/Game/ExternalContent/sounds/Nail_Gun/Glove_charging_que1.Glove_charging_que1"))
                (:OnBlendOut
                  (Animation|Montage|PlayMontage (Variables|/Script/Engine.Character|GetMesh (Variables|Default|GetPlayerCharacterBP)) (.FullChargedAnimation (Utilities|GetClassDefaults (Variables|/Script/ArcherPRT.WeaponComponent|GetCurrentEquipWeapon (Variables|/Script/ArcherPRT.GameCharacter|GetWeaponComponent (Variables|Default|GetPlayerCharacterBP)))))
                    (:then
                      (Default|PlaySound (Variables|Default|GetPlayerCharacterBP) (Variables|/Game/Blueprint/Player/PlayerCharacter_BP.PlayerCharacter_BP_C|GetWeapon_Sound (Variables|Default|GetPlayerCharacterBP)) "/Game/ExternalContent/sounds/Nail_Gun/Glove_charged_idle_que.Glove_charged_idle_que"))))))
            (:PneumaticGun
              (if (Class|WeaponComponent|HaveAmmo (Variables|/Script/ArcherPRT.GameCharacter|GetWeaponComponent (Variables|Default|GetPlayerCharacterBP)))
                (Animation|Montage|PlayMontage (Variables|/Script/Engine.Character|GetMesh (Variables|Default|GetPlayerCharacterBP)) (.ChargeAnimation (Utilities|GetClassDefaults (Variables|/Script/ArcherPRT.WeaponComponent|GetCurrentEquipWeapon (Variables|/Script/ArcherPRT.GameCharacter|GetWeaponComponent (Variables|Default|GetPlayerCharacterBP)))))
                  (:then
                    (Default|PlaySound (Variables|Default|GetPlayerCharacterBP) (Variables|/Game/Blueprint/Player/PlayerCharacter_BP.PlayerCharacter_BP_C|GetWeapon_Sound (Variables|Default|GetPlayerCharacterBP)) "/Game/ExternalContent/sounds/Nail_Gun/Gun_Start_Charging_que.Gun_Start_Charging_que"))
                  (:OnBlendOut
                    (Animation|Montage|PlayMontage (Variables|/Script/Engine.Character|GetMesh (Variables|Default|GetPlayerCharacterBP)) (.FullChargedAnimation (Utilities|GetClassDefaults (Variables|/Script/ArcherPRT.WeaponComponent|GetCurrentEquipWeapon (Variables|/Script/ArcherPRT.GameCharacter|GetWeaponComponent (Variables|Default|GetPlayerCharacterBP)))))
                      (:then
                        (Variables|/Script/ArcherPRT.WeaponComponent|SetbWeaponCharged (Variables|/Script/ArcherPRT.GameCharacter|GetWeaponComponent (Variables|Default|GetPlayerCharacterBP)) true)))))
                (else
                  (Animation|Montage|PlayMontage (Variables|/Script/Engine.Character|GetMesh (Variables|Default|GetPlayerCharacterBP)) (.EmptyAmmoAnimation (Utilities|GetClassDefaults (Variables|/Script/ArcherPRT.WeaponComponent|GetCurrentEquipWeapon (Variables|/Script/ArcherPRT.GameCharacter|GetWeaponComponent (Variables|Default|GetPlayerCharacterBP)))))
                    (:OnCompleted
                      _)
                    (:OnInterrupted
                      _))
                  (Class|WeaponComponent|FinishFire (Variables|/Script/ArcherPRT.GameCharacter|GetWeaponComponent (Variables|Default|GetPlayerCharacterBP)) false))))))
        (:EventReceived
          (Ability|EndAbility))))
    (:CastFailed
      (Ability|EndAbility))))

(event Ability|EventOnEndAbility
  (params (bWasCancelled :type Boolean))
  (bind _async_task (Variables|Default|GetAsync%20Task))
  (Utilities|FlowControl|Sequence
    (:then_0
      (Utilities|IsValid _async_task
        (:Is%20Valid
          (GameplayTasks|EndTask _async_task))))
    (:then_1
      (Class|WeaponComponent|FinishFire (Variables|/Script/ArcherPRT.GameCharacter|GetWeaponComponent (Variables|Default|GetPlayerCharacterBP)) false))))