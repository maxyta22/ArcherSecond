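; Player character Blueprint handling walk/run, climbing, gun/melee switching, damage feedback, HUD and quick save/restart keys.
; Tick drives movement state and footsteps, while the pausing wheel widget selects montage-driven weapon swaps.
; Climb overlaps switch to Flying with sliding audio and downward push, and Space launches off.
; Landing shakes scale with fall speed and hits launch the player backward, while dodge, aim-meter and walking-house logic sit partly disconnected.
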(event Custom|PerformCameraShake
  (params (Epicenter :type Vector))
  (Camera|PlayWorldCameraShake "/Game/Characters/Walking_House/Walking_House_Walking_Shake.Walking_House_Walking_Shake_C" Epicenter 1e+02 1.5e+04 3.0))

(event Custom|Player_Get_Hit
  (bind _charactermovement (Variables|Character|GetCharacterMovement))
  (bind _capsulecomponent (Variables|Default|GetCapsuleComponent))
  (bind _returnvalue (Math|Vector|GetForwardVector _capsulecomponent))
  (bind _returnvalue_2 (* _returnvalue -2e+03))
  ;[1 1 1] Игрок получает урон
  (bind _returnvalue_3 (Actor|GetActorOfClass "/Game/Blueprint/AI/AICharacterLizard_BP.AICharacterLizard_BP_C"))
  (Camera|PlayWorldCameraShake "/Game/Characters/MainChar/Get_Hit_CAmera_Shake.Get_Hit_CAmera_Shake_C" (Transformation|GetWorldLocation (Variables|Default|GetCapsuleComponent)) 1e+02 1e+03 3.0)
  (Character|LaunchCharacter (Math|Vector|MakeVector (.x _returnvalue_2) (.y _returnvalue_2) (* (.z (Math|Vector|GetUpVector (Variables|Default|GetCapsuleComponent))) -5e+02)) false false)
  (bind _newtrack_0 (Timeline|Get_Hit PlayFromStart)
    (:Update
      (Variables|/Script/Engine.MovementComponent|SetVelocity _charactermovement (Math|Vector|Lerp(Vector) (Variables|/Script/Engine.MovementComponent|GetVelocity _charactermovement) (/ (Variables|/Script/Engine.MovementComponent|GetVelocity _charactermovement) 1.1) _newtrack_0)))))

(event Custom|StopRunCameraShake
  ;[1 0 0.7705 1 60] Camera shake when player move
)

(event Custom|RunTick
  ;[1 0 0.7705 1 60] Camera shake when player move
  (if (Utilities|Enum|Equal(Enum) (Variables|Default|Getidle_walk_run) "NewEnumerator1")
    (goto _label Reset)
    (else
      (CallFunction|StopWalkCameraShake)
      (if (or (!= (Input|AxisValues|GetMoveForward) 0.0) (!= (Input|AxisValues|GetMoveRight) 0.0))
        (Utilities|FlowControl|DoOnce false :!label _label
          (:Completed
            (CallFunction|StartRunCameraShake)
            (goto _label_2 Reset)))
        (else
          (Utilities|FlowControl|DoOnce false :!label _label_2
            (:Completed
              (CallFunction|StopRunCameraShake)
              (goto _label Reset))))))))

(event Custom|CheckInput
  ;[1 0.9875 0 1 60] Check Walk/Run
  (if (not (Utilities|Enum|Equal(Enum) (Variables|Default|Getidle_walk_run) "NewEnumerator2"))
    (if (CallFunction|HasInput)
      (Variables|Default|Setidle_walk_run "NewEnumerator1")
      (else
        (Variables|Default|Setidle_walk_run "NewEnumerator0")))))

(event Custom|Walk_Run_sound
  (bind _footsteps_cue (Variables|Default|Getfootsteps_Cue))
  ;[1 1 1] Steps Sound
  (Utilities|FlowControl|Sequence
    (:then_0
      (if (CallFunction|HasInput)
        (Utilities|FlowControl|DoOnce false :!label _label
          (:Completed
            (Audio|Components|Audio|Play (Variables|Default|Getfootsteps_Cue) 0.0)))
        (else
          (Audio|Components|Audio|Stop (Variables|Default|Getfootsteps_Cue))
          (goto _label Reset))))
    (:then_1
      (if (Utilities|Enum|Equal(Enum) (Variables|Default|Getidle_walk_run) "NewEnumerator2")
        (Utilities|FlowControl|DoOnce false :!label _label_2
          (:Completed
            (Audio|Components|Audio|SetPitchMultiplier _footsteps_cue 2.0)
            (Audio|Components|Audio|Play (Variables|Default|Getfootsteps_Cue) 0.0)))
        (else
          (Audio|Components|Audio|SetPitchMultiplier _footsteps_cue 1.0)
          (goto _label_2 Reset))))))

(event Custom|Light_Inside
  ;[1 1 1] Lights
)

(event Custom|Light_Outside
  ;[1 1 1] Lights
)

(event Custom|Velocity_Check
  ;[1 1 1] Cam Shake Landing
  (Development|PrintString (Utilities|String|ToString(Float) (Math|Vector|VectorLength (Transformation|GetVelocity self))) true true "(R=0.000000,G=0.660000,B=1.000000,A=1.000000)" 0.0))

(event Custom|End_overlap
  (bind _falling_rocks_audio (Variables|Default|GetFalling_Rocks_Audio))
  (bind _charactermovement (Variables|Character|GetCharacterMovement))
  (Audio|Components|Audio|SetSound _falling_rocks_audio "/Game/ExternalContent/sounds/Player_Sounds/Slidind_Player_Cue.Slidind_Player_Cue")
  (Audio|Components|Audio|Stop _falling_rocks_audio)
  (if (not (and (Variables|Default|Getjump_climbing) (not (Variables|Default|Getis_climbing))))
    (Variables|Default|Setis_climbing false)
    (Variables|Default|Setjump_climbing false)
    (Variables|/Script/Engine.CharacterMovementComponent|SetMaxFlySpeed _charactermovement 0.0)
    (Variables|/Script/Engine.CharacterMovementComponent|SetBrakingDecelerationFlying _charactermovement 0.0)
    (Pawn|Components|CharacterMovement|SetMovementMode _charactermovement "MOVE_Walking" 0)))

(event Custom|Tick_Draw_path
  (bind _bow (Variables|Default|GetBow))
  (bind _mesh (Variables|Character|GetMesh))
  ;[1 0 0.2054 1 100] OLD
  ;;[0 0.1181 1 1 60] Draw Aim (Transfer in HUD*)
  (if (and (not (Class|CraftComponent|CraftinProgress (Variables|Default|GetCraftComponent))) (not (Class|BuildingComponent|BuildingModeActivated (Variables|Default|GetBuildingComponent))))
    (Utilities|FlowControl|Sequence
      (:then_0
        (if (Class|WeaponComponent|AiminginProgress (Variables|Default|GetWeaponComponent))
          (Utilities|FlowControl|Sequence
            (:then_0
              (bind _output_get (Variables|Default|SetAttack%20Pressed%20Meter (+ (Variables|Default|GetAttack%20Pressed%20Meter) 0.02)))
              (if (>= _output_get 1.0)
                (Variables|Default|SetAttack%20Pressed%20Meter 1.0)
                (Variables|Default|Setarrow_ready true)
                (else
                  (Variables|Default|Setarrow_ready false))))
            (:then_1
              (bind _output_get_2 (Variables|Default|Setattack_pressed_circle_scale (- (Variables|Default|Getattack_pressed_circle_scale) 0.02)))
              (if (<= _output_get_2 0.0)
                (Variables|Default|Setattack_pressed_circle_scale 0.0)))
            (:then_2
              (if (> (Variables|Default|GetAttack%20Pressed%20Meter) 0.97)
                (Variables|Default|SetDot_draw 1.0)))
            (:then_3
              (Utilities|FlowControl|DoOnce false
                (:Completed
                  (Audio|Components|Audio|SetSound _bow "/Game/ExternalContent/sounds/Player_Sounds/Bow_sounds/Loading_Bow_que.Loading_Bow_que")
                  (Audio|Components|Audio|Play _bow 0.0)))))
          (else
            (Variables|Default|SetAttack%20Pressed%20Meter 0.0)
            (Variables|Default|Setattack_pressed_circle_scale 1.0)
            (Variables|Default|SetDot_draw 0.0))))
      (:then_1
        (Variables|Default|Setarrow_trajectory_highnes (Math|Float|MapRangeClamped (Variables|Default|GetAttack%20Pressed%20Meter) 0.0 1.0 2.5e+03 0.0)))
      (:then_4
        (if (Class|WeaponComponent|AiminginProgress (Variables|Default|GetWeaponComponent))
          (Rendering|Material|SetScalarParameterValueonMaterials _mesh "Arrow_transparent" 1.0)
          (else
            (Rendering|Material|SetScalarParameterValueonMaterials _mesh "Arrow_transparent" 0.0)))))))

(event Custom|Start_overlap
  (bind _falling_rocks_audio (Variables|Default|GetFalling_Rocks_Audio))
  (bind _charactermovement (Variables|Character|GetCharacterMovement))
  (bind _charactermovement_2 (Variables|Character|GetCharacterMovement))
  (Audio|Components|Audio|SetSound _falling_rocks_audio "/Game/ExternalContent/sounds/Player_Sounds/Slidind_Player_Cue.Slidind_Player_Cue")
  (Audio|Components|Audio|Play _falling_rocks_audio 0.0)
  (Variables|Default|Setis_climbing true)
  (Variables|Default|Setjump_climbing false)
  (Utilities|FlowControl|Sequence
    (:then_0
      (Pawn|Components|CharacterMovement|SetMovementMode _charactermovement_2 "MOVE_Flying" 0)
      (Variables|/Script/Engine.CharacterMovementComponent|SetMaxFlySpeed _charactermovement_2 2e+02)
      (Variables|/Script/Engine.CharacterMovementComponent|SetBrakingDecelerationFlying _charactermovement_2 5e+02))
    (:then_1
      (bind _newtrack_0 (Timeline|Timeline_3 Play)
        (:Update
          (if (> (Math|Vector|VectorLength (Variables|/Script/Engine.MovementComponent|GetVelocity _charactermovement)) 2e+02)
            (Variables|/Script/Engine.MovementComponent|SetVelocity _charactermovement (Math|Vector|Lerp(Vector) (Variables|/Script/Engine.MovementComponent|GetVelocity _charactermovement) (/ (Variables|/Script/Engine.MovementComponent|GetVelocity _charactermovement) 2.0) _newtrack_0))))))))

(event Custom|Push_Down_Climbing
  (if (Variables|Default|Getis_climbing)
    (Physics|AddImpulse (Variables|/Script/Engine.Character|GetCharacterMovement (Game|GetPlayerCharacter 0)) (* (Math|Vector|GetUpVector (Variables|/Script/Engine.Character|GetCapsuleComponent (Game|GetPlayerCharacter 0))) -1e+01) true)))

(event Custom|Loading_Bow_Sound_Reset
  (bind _bow (Variables|Default|GetBow))
  ;[1 0 0.2054 1 100] OLD
  ;;[0 0.1181 1 1 60] Draw Aim (Transfer in HUD*)
  (Utilities|FlowControl|DoOnce false) ; enters at Reset
)

(event Custom|launch_tick
  (bind _charactermovement (Variables|Character|GetCharacterMovement))
  (bind _returnvalue (Pawn|Components|PawnMovement|GetLastInputVector _charactermovement))
  (bind _returnvalue_2 (* _returnvalue 1e+03))
  ;[0 0.8115 1 1 60] Dodge
  (if (Variables|Default|Getcan_launch)
    (Development|PrintString "launch")
    (Character|LaunchCharacter (Math|Vector|MakeVector (.x _returnvalue_2) (.y _returnvalue_2) (* (.z (Math|Vector|GetUpVector (Variables|Default|GetCapsuleComponent))) -5e+02)) false false)
    (bind _newtrack_0 (Timeline|dodge PlayFromStart)
      (:Update
        (Variables|/Script/Engine.MovementComponent|SetVelocity _charactermovement (Math|Vector|Lerp(Vector) (Variables|/Script/Engine.MovementComponent|GetVelocity _charactermovement) (/ (Variables|/Script/Engine.MovementComponent|GetVelocity _charactermovement) 1.1) _newtrack_0)))
      (:Finished
        (Variables|Default|Setcan_launch true)))))

(event Custom|CreateWidgets
  ;[0.6057 0 1 1 60] UI Widgets
  (Utilities|FlowControl|Sequence
    (:then_0
      (bind _returnvalue (UserInterface|CreateWidget "/Game/Blueprint/UI/Gameplay/MainHUD_UI.MainHUD_UI_C"))
      (bind _output_get (Variables|UMG|SetMainHudGamePlay _returnvalue))
      (Utilities|IsValid _output_get
        (:Is%20Valid
          (UserInterface|Viewport|AddtoViewport _output_get 0))))
    (:then_1
      (bind _returnvalue_2 (UserInterface|CreateWidget "/Game/Blueprint/UI/Gameplay/Wheel_UI.Wheel_UI_C"))
      (Variables|UMG|SetWheel_UI _returnvalue_2))))

(event Custom|SwitchWeapon
  (params (SelectIndex :type Integer))
  (bind _mesh (Variables|Character|GetMesh))
  (bind _weaponcomponent (Variables|Default|GetWeaponComponent))
  ;[0.5567 0 1 1 60] SwitchWeapon
  (if (!= SelectIndex (Variables|Default|GetLastSelectedWeaponIndex))
    (Variables|Default|SetLastSelectedWeaponIndex SelectIndex)
    (switch int SelectIndex
      (:0
        (Animation|Montage|PlayMontage _mesh "/Game/Characters/New_Player/New_Player_Animations/New_Player_Up_gun_Montage.New_Player_Up_gun_Montage"
          (:then
            (Variables|Default|SetGun_Equipped true)
            (Class|WeaponComponent|EquipWeapon _weaponcomponent "/Game/Blueprint/Weapon/DefaultRangeWeapon.DefaultRangeWeapon_C"))))
      (:2
        (Animation|Montage|PlayMontage _mesh "/Game/Characters/New_Player/New_Player_Animations/New_Player_Down_Gun_Montage.New_Player_Down_Gun_Montage"
          (:then
            (Variables|Default|SetGun_Equipped false)
            (Class|WeaponComponent|EquipWeapon _weaponcomponent "/Game/Blueprint/Weapon/DefaultMeleeWeapon.DefaultMeleeWeapon_C")))))))

(event Custom|StartWalkCameraShake
  ;[1 0 0.7705 1 60] Camera shake when player move
)

(event Custom|StopWalkCameraShake
  ;[1 0 0.7705 1 60] Camera shake when player move
)

(event Custom|VelocityWalkTick
  ;[1 0 0.7705 1 60] Camera shake when player move
  (if (Utilities|Enum|Equal(Enum) (Variables|Default|Getidle_walk_run) "NewEnumerator2")
    (goto _label Reset)
    (else
      (CallFunction|StopRunCameraShake)
      (if (or (!= (Input|AxisValues|GetMoveForward) 0.0) (!= (Input|AxisValues|GetMoveRight) 0.0))
        (Utilities|FlowControl|DoOnce false :!label _label
          (:Completed
            (CallFunction|StartWalkCameraShake)
            (goto _label_2 Reset)))
        (else
          (Utilities|FlowControl|DoOnce false :!label _label_2
            (:Completed
              (CallFunction|StopWalkCameraShake)
              (goto _label Reset))))))))

(event Custom|StartRunCameraShake
  ;[1 0 0.7705 1 60] Camera shake when player move
)

(event EventTick
  (params (DeltaSeconds :type Float%20%28single-precision%29))
  ;[0 0.2029 1 1 60] Tick
  (|CallParentFunction DeltaSeconds)
  (Utilities|FlowControl|Sequence
    (:then_4
      (CallFunction|CheckInput))
    (:then_5
      (CallFunction|VelocityWalkTick))
    (:then_6
      (CallFunction|RunTick))
    (:then_7
      (CallFunction|WalkRunSound))
    (:then_8
      (CallFunction|VelocityCheck))
    (:then_9
      (CallFunction|PushDownClimbing))))

(event EventBeginPlay
  ;[0 0.2029 1 1 60] BeginPlay
  (Utilities|FlowControl|Sequence
    (:then_0
      (CallFunction|CreateWidgets))
    (:then_1
      (Variables|/Script/Engine.CharacterMovementComponent|SetMaxWalkSpeed (Variables|Character|GetCharacterMovement) (Variables|Default|GetPlayer_Walking_Speed)))
    (:then_2
      (Audio|PlaySound2D "/Game/ExternalContent/sounds/ghostly_Woods_Sound_2_Cue.ghostly_Woods_Sound_2_Cue" 1.0 1.0 0.0 0 0))))

(event EventPressedAttackButon)

(event EventReleasedAttackButton)

(event EventAfterTakeDamage
  ;[1 0.3944 0 1 60] TakeDamage
  (Utilities|FlowControl|Sequence
    (:then_0
      (Default|ShowDamage (Variables|UMG|GetMainHudGamePlay)))
    (:then_1
      (CallFunction|PlayerGetHit))))

(event EventOnLanded
  (params (Hit :type Hit%20Result%20Structure%20%28by%20ref%29))
  (bind _self self)
  (bind _falling_rocks_audio (Variables|Default|GetFalling_Rocks_Audio))
  (bind _returnvalue (Transformation|GetVelocity _self))
  ;[1 1 1] Cam Shake Landing
  (|CallParentFunction Hit)
  (Utilities|FlowControl|Sequence
    (:then_0
      (Audio|Components|Audio|SetSound _falling_rocks_audio "/Game/ExternalContent/sounds/Player_Sounds/Landing_Impact_Que.Landing_Impact_Que")
      (Audio|Components|Audio|Play _falling_rocks_audio 0.0))
    (:then_1
      (if (< (.z (Transformation|GetVelocity self)) -1e+02)
        (if (< (.z _returnvalue) -5e+02)
          (if (>= (.z _returnvalue) -1.1e+03)
            (Camera|PlayWorldCameraShake "/Game/Characters/MainChar/Landing_Medium_CAmera_Shake2.Landing_Medium_CAmera_Shake2_C" (Transformation|GetWorldLocation (Variables|Default|GetCapsuleComponent)) 1e+02 1e+03)
            (else
              (Camera|PlayWorldCameraShake "/Game/Characters/MainChar/Landing_Hard_CAmera_Shake1.Landing_Hard_CAmera_Shake1_C" (Transformation|GetWorldLocation (Variables|Default|GetCapsuleComponent)) 1e+02 1e+03)))
          (else
            (Camera|PlayWorldCameraShake "/Game/Characters/MainChar/Landing_CAmera_Shake.Landing_CAmera_Shake_C" (Transformation|GetWorldLocation (Variables|Default|GetCapsuleComponent)) 1e+02 1e+03)))))))

(event EventAfterBeginCraft
  (bind _charactermovement (Variables|Character|GetCharacterMovement))
  ;[1 1 1] Crafting
  (Variables|/Script/Engine.CharacterMovementComponent|SetMaxWalkSpeed (Variables|Character|GetCharacterMovement) (Variables|Default|GetPlayer_Walking_Speed))
  (Components|Timeline|SetTimelineLength (Variables|Default|GetTimeline_0) (Variables|/Script/ArcherPRT.CraftComponent|GetTimeCraft (Variables|Default|GetCraftComponent)))
  (Timeline|Timeline_0 PlayFromStart
    (:Finished
      (if (Utilities|Enum|Equal(Enum) (Variables|Default|Getidle_walk_run) "NewEnumerator2")
        (Variables|/Script/Engine.CharacterMovementComponent|SetMaxWalkSpeed _charactermovement (Variables|Default|GetPlayer_Running_Speed))
        (else
          (Variables|/Script/Engine.CharacterMovementComponent|SetMaxWalkSpeed _charactermovement (Variables|Default|GetPlayer_Walking_Speed)))))))

(event EventAfteronDeath
  ;[0.1134 0 1 1 60] Death
  (bind _asprtplayer_controller_bp (Utilities|Casting|CastToPRTPlayerController_BP (Game|GetPlayerController 0)))
  (Default|CallMenu _asprtplayer_controller_bp))

(event Input|ActionEvents|InputActionShowWheel
  (params (Key :type Key%20Structure :default "None"))
  (bind _wheel_ui (Variables|UMG|GetWheel_UI))
  (:Pressed
    (Game|SetGamePaused true)
    (UserInterface|Viewport|AddtoViewport _wheel_ui 0))
  (:Released
    (Game|SetGamePaused false)
    (Widget|RemovefromParent _wheel_ui)
    (CallFunction|SwitchWeapon (Variables|/Game/Blueprint/UI/Gameplay/Wheel_UI.Wheel_UI_C|GetSelectIndex _wheel_ui))))

(event Input|KeyboardEvents|LeftShift
  (params (Key :type Key%20Structure :default "None"))
  (bind _charactermovement (Variables|Character|GetCharacterMovement))
  ;[1 0.9875 0 1 60] Check Walk/Run
  (:Pressed
    (if (or (Class|WeaponComponent|AiminginProgress (Variables|Default|GetWeaponComponent)) (Class|CraftComponent|CraftinProgress (Variables|Default|GetCraftComponent)))
      (Variables|/Script/Engine.CharacterMovementComponent|SetMaxWalkSpeed _charactermovement (Variables|Default|GetPlayer_Walking_Speed) :!label _label)
      (Variables|Default|Setidle_walk_run "NewEnumerator1")
      (else
        (Variables|/Script/Engine.CharacterMovementComponent|SetMaxWalkSpeed _charactermovement (Variables|Default|GetPlayer_Running_Speed))
        (Variables|Default|Setidle_walk_run "NewEnumerator2"))))
  (:Released
    (goto _label)))

(event Input|MouseEvents|LeftMouseButton
  (params (Key :type Key%20Structure :default "None"))
  ;[1 1 1] Walking_House_Setup
)

(event Input|KeyboardEvents|F9
  (params (Key :type Key%20Structure :default "None"))
  (:Pressed
    (bind _asarcher_prtgame_mode_bp (Utilities|Casting|CastToArcherPRTGameMode_BP (Game|GetGameMode)))
    (Default|RestartWorld _asarcher_prtgame_mode_bp false)))

(event Input|KeyboardEvents|SpaceBar
  (params (Key :type Key%20Structure :default "None"))
  (bind _capsulecomponent (Variables|Default|GetCapsuleComponent))
  (bind _charactermovement (Variables|Character|GetCharacterMovement))
  (:Pressed
    (if (Variables|Default|Getis_climbing)
      (Variables|Default|Setjump_climbing true)
      (Utilities|FlowControl|Sequence
        (:then_0
          (bind _newtrack_0 (Timeline|Timeline_3 Stop)
            (:Update
              (if (> (Math|Vector|VectorLength (Variables|/Script/Engine.MovementComponent|GetVelocity _charactermovement)) 2e+02)
                (Variables|/Script/Engine.MovementComponent|SetVelocity _charactermovement (Math|Vector|Lerp(Vector) (Variables|/Script/Engine.MovementComponent|GetVelocity _charactermovement) (/ (Variables|/Script/Engine.MovementComponent|GetVelocity _charactermovement) 2.0) _newtrack_0))))))
        (:then_1
          (Variables|/Script/Engine.PrimitiveComponent|SetbGenerateOverlapEvents (Variables|Default|GetClimbing_collision) false)
          (Variables|Default|Setis_climbing false)
          (Pawn|Components|CharacterMovement|SetMovementMode (Variables|Character|GetCharacterMovement) "MOVE_Walking" 0)
          (Character|LaunchCharacter (+ (* (Math|Vector|GetForwardVector _capsulecomponent) 2e+02) (* (Math|Vector|GetUpVector _capsulecomponent) 1.5e+02)) false true)
          (Utilities|FlowControl|Delay 0.7)
          (Variables|/Script/Engine.PrimitiveComponent|SetbGenerateOverlapEvents (Variables|Default|GetClimbing_collision) true))))))

(event Input|KeyboardEvents|R
  (params (Key :type Key%20Structure :default "None")))

(event Input|KeyboardEvents|H
  (params (Key :type Key%20Structure :default "None")))

(event Input|KeyboardEvents|LeftShift
  (params (Key :type Key%20Structure :default "None"))
  ;[0 0.8115 1 1 60] Dodge
)

(event Input|KeyboardEvents|J
  (params (Key :type Key%20Structure :default "None")))

(event Input|KeyboardEvents|K
  (params (Key :type Key%20Structure :default "None")))

(event Input|MouseEvents|RightMouseButton
  (params (Key :type Key%20Structure :default "None"))
  ;[1 1 1] Walking_House_Setup
)

(event Input|KeyboardEvents|E
  (params (Key :type Key%20Structure :default "None"))
  ;[1 1 1] Walking_House_Setup
)

(event Input|KeyboardEvents|F5
  (params (Key :type Key%20Structure :default "None"))
  (:Pressed
    (bind _asarcher_prtgame_mode_bp (Utilities|Casting|CastToArcherPRTGameMode_BP (Game|GetGameMode)))
    (Default|SaveGame _asarcher_prtgame_mode_bp)))

(event Input|KeyboardEvents|Q
  (params (Key :type Key%20Structure :default "None"))
  (:Pressed
    (Rendering|ToggleVisibility (Variables|Default|GetPostProcess) false)))

(fn ConstructionScript
  (Class|SkinnedMeshComponent|SetMasterPoseComponent (Variables|Default|GetGlove) (Variables|Character|GetMesh) false))

(fn OnRepHealth)

(fn HasInput
  (return (or (!= (Input|AxisValues|GetMoveForward) 0.0) (!= (Input|AxisValues|GetMoveRight) 0.0))))