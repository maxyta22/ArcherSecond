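; Player controller that handles screen fades and toggles the main menu widget as a pause menu.
; On begin play it creates the menu, then adds a fade widget to the viewport and fades out.
; Possession sets game-only input.
; The PauseMenu action toggles menu, pause, cursor and input mode, fading in on open through a DoOnce that resets on close, when it fades out.
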(event EventBeginPlay
  (bind _returnvalue (UserInterface|CreateWidget "/Game/Blueprint/UI/MainMenu_UI.MainMenu_UI_C"))
  (Variables|Default|SetMainMenu _returnvalue)
  (Utilities|FlowControl|Sequence
    (:then_0
      (bind _returnvalue_2 (UserInterface|CreateWidget "/Game/Characters/MainChar/interface/Fade_Widget.Fade_Widget_C" (Game|GetPlayerController 0)))
      (bind _asfade_widget (Utilities|Casting|CastToFade_Widget _returnvalue_2))
      (Variables|Default|SetFade%20Variable _asfade_widget)
      (UserInterface|Viewport|AddtoViewport _returnvalue_2 0))
    (:then_1
      (Default|FadeOutEvent (Variables|Default|GetFade%20Variable)))))

(event EventPossess
  (params (PossessedPawn :type Pawn%20Object%20Reference))
  (|CallParentFunction PossessedPawn)
  (Input|SetInputModeGameOnly self))

(event Input|ActionEvents|InputActionPauseMenu
  (params (Key :type Key%20Structure))
  (bind _self self)
  (bind _mainmenu (Variables|Default|GetMainMenu))
  (bind _fade_variable (Variables|Default|GetFade%20Variable))
  ;[0.1411 0 1] Pause
  (:Pressed
    (if (not (UserInterface|Viewport|IsinViewport (Variables|Default|GetMainMenu)))
      (Game|SetGamePaused true)
      (UserInterface|Viewport|AddtoViewport _mainmenu 0)
      (Variables|/Script/Engine.PlayerController|SetbShowMouseCursor _self true)
      (Input|SetInputModeGameandUI _self (Variables|Default|GetMainMenu) "DoNotLock" true)
      (Utilities|FlowControl|DoOnce false :!label _label
        (:Completed
          (Default|FadeinEvent _fade_variable)))
      (else
        (Game|SetGamePaused false)
        (Widget|RemovefromParent _mainmenu)
        (Variables|/Script/Engine.PlayerController|SetbShowMouseCursor _self false)
        (Input|SetInputModeGameOnly _self)
        (Default|FadeOutEvent _fade_variable)
        (goto _label Reset)))))

(fn ConstructionScript)