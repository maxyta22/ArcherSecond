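; Charged nail projectile Blueprint that leaves a particle trail and destroys itself on impact.
; Every tick it spawns a new charged bullet trail system at its static mesh's location, with auto-destroy off.
; A Hit event draws a debug sphere at the supplied location before destroying the actor, while a hit on the collision capsule destroys it directly.
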(event OnComponentHit(CapsuleCollisionForStatic)
  (params (HitComponent :type Primitive%20Component%20Object%20Reference) (OtherActor :type Actor%20Object%20Reference) (OtherComp :type Primitive%20Component%20Object%20Reference) (NormalImpulse :type Vector :default "0, 0, 0") (Hit :type Hit%20Result%20Structure%20%28by%20ref%29))
  (Actor|DestroyActor))

(event EventTick
  (params (DeltaSeconds :type Float%20%28single-precision%29))
  (|CallParentFunction DeltaSeconds)
  (Niagara|SpawnSystematLocation "/Game/Characters/New_Player/Gun/bullet_trail_Niagara/NE_Charged_Bullet_Trail.NE_Charged_Bullet_Trail" (Transformation|GetWorldLocation (Variables|Default|GetStaticMesh)) "0, 0, 0" "1.000000,1.000000,1.000000" false))

(event Collision|EventHit
  (params (MyComp :type Primitive%20Component%20Object%20Reference) (Other :type Actor%20Object%20Reference) (OtherComp :type Primitive%20Component%20Object%20Reference) (bSelfMoved :type Boolean) (HitLocation :type Vector :default "0, 0, 0") (HitNormal :type Vector :default "0, 0, 0") (NormalImpulse :type Vector :default "0, 0, 0") (Hit :type Hit%20Result%20Structure%20%28by%20ref%29))
  (Rendering|Debug|DrawDebugSphere HitLocation 1e+01 12 "(R=0.227949,G=1.000000,B=0.000000,A=1.000000)" 5.0 1.0)
  (Actor|DestroyActor))

(fn ConstructionScript
  (|CallParentFunction))